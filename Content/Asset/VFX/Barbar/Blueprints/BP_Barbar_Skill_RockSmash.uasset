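; Barbarian Rock Smash skill VFX actor that plays a ground impact with cracking decals when spawned.
; On BeginPlay it shares one dynamic crack material across three decals, triggers a weak world camera shake, and fires the lava impact particle, then the chain snakes after a short delay.
; A timeline then animates the material's Gradient parameter and activates the ultimate triangle impact particle when it finishes.
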(event EventBeginPlay
  ;[1 1 1] Material For Crack
  (bind _returnvalue (Rendering|Material|CreateDynamicMaterialInstance "/Game/Asset/VFX/Barbar/Materials/Decals/StandartDecals/MI_Decal_Crack_thick.MI_Decal_Crack_thick" "None" "None" :!class /Script/Engine.KismetMaterialLibrary))
  (bind _output_get (Variables|Default|SetDecal_Crack _returnvalue))
  (Rendering|Components|Decal|SetDecalMaterial (Variables|Default|GetDecal_Crack_01) _output_get)
  (Rendering|Components|Decal|SetDecalMaterial (Variables|Default|GetDecal_Crack_02) _output_get)
  (Rendering|Components|Decal|SetDecalMaterial (Variables|Default|GetDecal_Crack_03) _output_get)
  ;[1 1 1] cam shake
  (Camera|PlayWorldCameraShake "/Game/Asset/VFX/Barbar/Blueprints/CameraEffects/BP_CameraShake_Weak.BP_CameraShake_Weak_C" (Transformation|GetActorLocation self) 0.0 5e+02 0.0)
  (Components|Activation|Activate (Variables|Default|GetPS_Impact_Small_Lava) false)
  (Utilities|FlowControl|Delay 0.1)
  (Components|Activation|Activate (Variables|Default|GetPS_BarBar_Chain_Snakes) false)
  ;[1 1 1] Decal Anim
  (bind _gradient (Timeline|Timeline PlayFromStart)
    (:Update
      (Rendering|Material|SetScalarParameterValue (Variables|Default|GetDecal_Crack) "Gradient" _gradient :!class /Script/Engine.MaterialInstanceDynamic))
    (:Finished
      (Components|Activation|Activate (Variables|Default|GetPS_BarBar_Ultimate_Impact_Triangle) false))))

(fn ConstructionScript)