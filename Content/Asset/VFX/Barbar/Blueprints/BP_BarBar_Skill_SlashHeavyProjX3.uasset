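; Barbarian heavy slash skill VFX actor that fires three ground projectiles alongside animated crack decals.
; On BeginPlay it spawns three short-lived BP_BarBar_Projectile actors using a ground particle effect, with the side two offset along world Y and angled outward.
; One dynamic material shared by three decals has its Gradient driven by the CrackGradient timeline, which also triggers a weak world camera shake on every update.
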(event EventBeginPlay
  (bind _self self)
  (bind _self_2 self)
  (bind _self_3 self)
  (bind _returnvalue (Transformation|GetActorLocation _self))
  (bind _returnvalue_2 (Transformation|GetActorLocation _self_2))
  (bind _returnvalue_3 (Transformation|GetActorLocation _self_3))
  ;[1 1 1] Decal Material
  (bind _returnvalue_4 (Rendering|Material|CreateDynamicMaterialInstance "/Game/Asset/VFX/Barbar/Materials/Decals/StandartDecals/MI_Decal_Crack_thick_proj.MI_Decal_Crack_thick_proj" "None" "None" :!class /Script/Engine.KismetMaterialLibrary))
  (bind _output_get (Variables|Default|SetDecalCrackMat _returnvalue_4))
  (Rendering|Components|Decal|SetDecalMaterial (Variables|Default|GetDecal_Crack) _output_get)
  (Rendering|Components|Decal|SetDecalMaterial (Variables|Default|GetDecal_Crack1) _output_get)
  (Rendering|Components|Decal|SetDecalMaterial (Variables|Default|GetDecal_Crack2) _output_get)
  (Utilities|FlowControl|Sequence
    (:then_0
      ;[1 1 1] Projectiles
      (Game|SpawnActorfromClass "/Game/Asset/VFX/Barbar/Blueprints/Projectiles/BP_BarBar_Projectile.BP_BarBar_Projectile_C" (Math|Transform|MakeTransform (Math|Vector|MakeVector (.x _returnvalue_3) (.y _returnvalue_3) (.z _returnvalue_3)) "0, 0, 0" "1.000000,1.000000,1.000000") "Undefined" "OverrideRootScale" 0 1.5e+03 1.0 "/Game/Asset/VFX/Barbar/Particles/Projectiles/PS_Projectile_Ground.PS_Projectile_Ground" 0)
      (Game|SpawnActorfromClass "/Game/Asset/VFX/Barbar/Blueprints/Projectiles/BP_BarBar_Projectile.BP_BarBar_Projectile_C" (Math|Transform|MakeTransform (Math|Vector|MakeVector (.x _returnvalue_2) (+ (.y _returnvalue_2) 125.0) (.z _returnvalue_2)) "0.000000,10.000000,0.000000" "1.000000,1.000000,1.000000") "Undefined" "OverrideRootScale" 0 1.5e+03 1.0 "/Game/Asset/VFX/Barbar/Particles/Projectiles/PS_Projectile_Ground.PS_Projectile_Ground" 0)
      (Game|SpawnActorfromClass "/Game/Asset/VFX/Barbar/Blueprints/Projectiles/BP_BarBar_Projectile.BP_BarBar_Projectile_C" (Math|Transform|MakeTransform (Math|Vector|MakeVector (.x _returnvalue) (+ (.y _returnvalue) -125.0) (.z _returnvalue)) "0.000000,-10.000000,0.000000" "1.000000,1.000000,1.000000") "Undefined" "OverrideRootScale" 0 1.5e+03 1.0 "/Game/Asset/VFX/Barbar/Particles/Projectiles/PS_Projectile_Ground.PS_Projectile_Ground" 0))
    (:then_1
      ;[1 1 1] Decal Anim
      (bind _newtrack_0 (Timeline|CrackGradient PlayFromStart)
        (:Update
          (Rendering|Material|SetScalarParameterValue (Variables|Default|GetDecalCrackMat) "Gradient" _newtrack_0 :!class /Script/Engine.MaterialInstanceDynamic)
          ;[1 1 1] CamShake
          (Camera|PlayWorldCameraShake "/Game/Asset/VFX/Barbar/Blueprints/CameraEffects/BP_CameraShake_Weak.BP_CameraShake_Weak_C" (Transformation|GetActorLocation self) 0.0 3e+03 1.5))))))

(fn ConstructionScript)