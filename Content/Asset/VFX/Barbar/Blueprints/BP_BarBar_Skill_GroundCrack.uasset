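; Barbarian skill VFX actor that plays a ground crack: a decal, impact particles and a camera shake.
; On BeginPlay it puts a dynamic crack material on the decal and plays a weak world camera shake from its location.
; A timeline drives the material's Gradient parameter to animate the crack while four impact particle systems activate in quick, evenly staggered succession.
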(event EventBeginPlay
  ;[1 1 1] Decal Material
  (bind _returnvalue (Rendering|Material|CreateDynamicMaterialInstance "/Game/Asset/VFX/Barbar/Materials/Decals/StandartDecals/MI_Decal_Crack_thick.MI_Decal_Crack_thick" "None" "None" :!class /Script/Engine.KismetMaterialLibrary))
  (bind _output_get (Variables|Default|SetDecalCrackMat _returnvalue))
  (Rendering|Components|Decal|SetDecalMaterial (Variables|Default|GetDecal_Crack) _output_get)
  ;[1 1 1] Camera Shake
  (Camera|PlayWorldCameraShake "/Game/Asset/VFX/Barbar/Blueprints/CameraEffects/BP_CameraShake_Weak.BP_CameraShake_Weak_C" (Transformation|GetActorLocation self) 0.0 3.5e+03)
  (Utilities|FlowControl|Sequence
    (:then_0
      ;[1 1 1] Decal Anim
      (bind _newtrack_0 (Timeline|CrackGradient PlayFromStart)
        (:Update
          (Rendering|Material|SetScalarParameterValue (Variables|Default|GetDecalCrackMat) "Gradient" _newtrack_0 :!class /Script/Engine.MaterialInstanceDynamic))))
    (:then_1
      ;[1 1 1] Impact Timings
      (Utilities|FlowControl|Delay 0.08)
      (Components|Activation|Activate (Variables|Default|GetPS_Impact_GroundCrack) false))
    (:then_2
      (Utilities|FlowControl|Delay 0.16)
      (Components|Activation|Activate (Variables|Default|GetPS_Impact_GroundCrack1) false))
    (:then_3
      (Utilities|FlowControl|Delay 0.24)
      (Components|Activation|Activate (Variables|Default|GetPS_Impact_GroundCrack2) false))
    (:then_4
      (Utilities|FlowControl|Delay 0.32)
      (Components|Activation|Activate (Variables|Default|GetPS_Impact_GroundCrack3) false))))

(fn ConstructionScript)