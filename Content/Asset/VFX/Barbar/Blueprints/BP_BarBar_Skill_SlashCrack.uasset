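; Barbarian slash-crack skill VFX actor that leaves an animated crack decal and launches a slash projectile.
; On BeginPlay it creates a dynamic instance of the thin crack decal material and assigns it to its decal.
; It then spawns a fast, short-lived BP_BarBar_Projectile with a slash particle at its location.
; The CrackGradient timeline drives the material's Gradient parameter to animate the crack.
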(event EventBeginPlay
  ;[1 1 1] Decal Material
  (bind _returnvalue (Rendering|Material|CreateDynamicMaterialInstance "/Game/Asset/VFX/Barbar/Materials/Decals/StandartDecals/MI_Decal_Crack_thin.MI_Decal_Crack_thin" "None" "None" :!class /Script/Engine.KismetMaterialLibrary))
  (bind _output_get (Variables|Default|SetDecalCrackMat _returnvalue))
  (Rendering|Components|Decal|SetDecalMaterial (Variables|Default|GetDecal_Crack) _output_get)
  (Utilities|FlowControl|Sequence
    (:then_0
      ;[1 1 1] Projectile
      (Game|SpawnActorfromClass "/Game/Asset/VFX/Barbar/Blueprints/Projectiles/BP_BarBar_Projectile.BP_BarBar_Projectile_C" (Math|Transform|MakeTransform (Transformation|GetActorLocation self) "0, 0, 0" "1.000000,1.000000,1.000000") "Undefined" "OverrideRootScale" 0 2e+03 0.19 "/Game/Asset/VFX/Barbar/Particles/Projectiles/PS_Projectile_Slash.PS_Projectile_Slash" 0))
    (:then_1
      ;[1 1 1] Decal Animation
      (bind _newtrack_0 (Timeline|CrackGradient PlayFromStart)
        (:Update
          (Rendering|Material|SetScalarParameterValue (Variables|Default|GetDecalCrackMat) "Gradient" _newtrack_0 :!class /Script/Engine.MaterialInstanceDynamic))))))

(fn ConstructionScript)