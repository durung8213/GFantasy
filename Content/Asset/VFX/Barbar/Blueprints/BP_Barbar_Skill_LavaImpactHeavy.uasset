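; BP_Barbar_Skill_LavaImpactHeavy is a VFX actor for the heavy lava impact of a Barbar skill.
; On BeginPlay it plays a weak world camera shake at its location, then waits briefly before the main impact.
; The impact activates the explosion lava-puddle particle system, plays a strong camera shake and spawns a short-lived BP_RadialBlur actor for post-process radial blur.
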(event EventBeginPlay
  (Camera|PlayWorldCameraShake "/Game/Asset/VFX/Barbar/Blueprints/CameraEffects/BP_CameraShake_Weak.BP_CameraShake_Weak_C" (Transformation|GetActorLocation self) 0.0 3.5e+03)
  (Utilities|FlowControl|Delay 1.5)
  (Components|Activation|Activate (Variables|Default|GetPS_Impact_ExplosionHeavy_LavaPuddle) false)
  (Camera|PlayWorldCameraShake "/Game/Asset/VFX/Barbar/Blueprints/CameraEffects/BP_CameraShake_Strong.BP_CameraShake_Strong_C" (Transformation|GetActorLocation self) 0.0 3.5e+03)
  ;[1 1 1] PP Radial Blur
  (Game|SpawnActorfromClass "/Game/Asset/VFX/Barbar/Blueprints/CameraEffects/BP_RadialBlur.BP_RadialBlur_C" (Math|Transform|MakeTransform (Transformation|GetActorLocation self) "0, 0, 0" "1.000000,1.000000,1.000000") "Undefined" "OverrideRootScale" 0 0.25 0))

(fn ConstructionScript)