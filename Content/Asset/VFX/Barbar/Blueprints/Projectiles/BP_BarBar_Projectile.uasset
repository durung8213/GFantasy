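; BP_BarBar_Projectile is a VFX projectile for the Barbar effects that flies and shows a Niagara effect.
; The construction script copies Speed into the projectile movement's initial speed.
; On BeginPlay it assigns the Projectile system to its Niagara component, waits LifeTime, deactivates the effect, then destroys itself after a short grace delay.
; It has no collision or damage logic in its graphs.
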(event EventBeginPlay
  (Class|NiagaraComponent|SetAsset (Variables|Default|GetNiagara) (Variables|Default|GetProjectile) true)
  (Utilities|FlowControl|Delay (Variables|Default|GetLifeTime))
  (Components|Activation|Deactivate (Variables|Default|GetNiagara))
  (Utilities|FlowControl|Delay 2.0)
  (Actor|DestroyActor self))

(fn ConstructionScript
  (Variables|/Script/Engine.ProjectileMovementComponent|SetInitialSpeed (Variables|Default|GetProjectileMovement) (Variables|Default|GetSpeed)))