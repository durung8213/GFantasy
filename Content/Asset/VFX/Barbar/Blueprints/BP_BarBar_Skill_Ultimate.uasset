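; VFX actor for the BarBar ultimate skill, playing a timed ground-crack and chain sequence on BeginPlay.
; It shakes the camera, then animates a shared dynamic decal material's Gradient via a timeline while three chain-snake particle effects fire.
; When the cracks finish, an implosion leads into ground energy, chain shield and a longer shake.
; Delayed branches finish by disabling shield shadows, spawning a radial-blur actor and leaving a fading chain-shadow decal.
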(event EventBeginPlay
  (bind _decal_crack_02 (Variables|Default|GetDecal_Crack_02))
  ;[1 1 1] Cam Shake
  (Camera|PlayWorldCameraShake "/Game/Asset/VFX/Barbar/Blueprints/CameraEffects/BP_CameraShake_Weak.BP_CameraShake_Weak_C" (Transformation|GetActorLocation self) 0.0 5e+02 0.0)
  ;[1 1 1] Set Dynamic Material
  (bind _returnvalue (Rendering|Material|CreateDynamicMaterialInstance "/Game/Asset/VFX/Barbar/Materials/Decals/StandartDecals/MI_Decal_Crack_thick.MI_Decal_Crack_thick" "None" "None" :!class /Script/Engine.KismetMaterialLibrary))
  (bind _output_get (Variables|Default|SetDecalCrack _returnvalue))
  (Rendering|Components|Decal|SetDecalMaterial (Variables|Default|GetDecal_Crack_01) _output_get)
  (Rendering|Components|Decal|SetDecalMaterial _decal_crack_02 _output_get)
  (Rendering|Components|Decal|SetDecalMaterial _decal_crack_02 _output_get)
  ;[1 1 1] activate Snakes
  (Utilities|FlowControl|Delay 0.2)
  (Utilities|FlowControl|Sequence
    (:then_0
      ;[1 1 1] Crack Animation
      (bind _newtrack_0 (Timeline|DecalCrackGradient PlayFromStart)
        (:Update
          (Rendering|Material|SetScalarParameterValue (Variables|Default|GetDecalCrack) "Gradient" _newtrack_0 :!class /Script/Engine.MaterialInstanceDynamic))
        (:Finished
          (Components|Activation|Activate (Variables|Default|GetPS_Impact_Implode) false)
          (Utilities|FlowControl|Delay 0.2)
          ;[1 1 1] Ground Energy
          (Components|Activation|Activate (Variables|Default|GetPS_BarBar_Ground_energy) false)
          ;[1 1 1] Chain Shield
          (Components|Activation|Activate (Variables|Default|GetPS_BarBar_Ultimate_Chain_Shield) false)
          ;[1 1 1] Long Cam Shake
          (Camera|PlayWorldCameraShake "/Game/Asset/VFX/Barbar/Blueprints/CameraEffects/BP_CameraShake_Long_Mid.BP_CameraShake_Long_Mid_C" (Transformation|GetActorLocation self) 0.0 5e+02 0.0)
          (Utilities|FlowControl|Sequence
            (:then_0
              ;[1 1 1] Last Decal
              (Utilities|FlowControl|Delay 3.0)
              (CallFunction|SpawnDecal "/Game/Asset/VFX/Barbar/Materials/Decals/StandartDecals/MI_Decal_Chain_Shadows.MI_Decal_Chain_Shadows" "5.000000,1000.000000,1000.000000" 3.0 0.05 1.5 (Transformation|GetActorLocation self)))
            (:then_1
              ;[1 1 1] PP Radial Blur
              (Utilities|FlowControl|Delay 2.9)
              (Game|SpawnActorfromClass "/Game/Asset/VFX/Barbar/Blueprints/CameraEffects/BP_RadialBlur.BP_RadialBlur_C" (Math|Transform|MakeTransform (Transformation|GetActorLocation self) "0, 0, 0" "1.000000,1.000000,1.000000") "Undefined" "OverrideRootScale" 0 0.25 0))
            (:then_2
              (Utilities|FlowControl|Delay 2.85)
              (Rendering|SetCastShadow (Variables|Default|GetPS_BarBar_Ultimate_Chain_Shield) false))))))
    (:then_1
      (Components|Activation|Activate (Variables|Default|GetPS_BarBar_Chain_Snake_Single) false))
    (:then_2
      (Components|Activation|Activate (Variables|Default|GetPS_BarBar_Chain_Snake_Single1) false))
    (:then_3
      (Components|Activation|Activate (Variables|Default|GetPS_BarBar_Chain_Snake_Single2) false))))

(fn ConstructionScript)