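; BP_Key is a trigger actor that lets the player spawn a configurable Niagara effect, from the NiagaraMagicalSlashes VFX folder.
; Overlapping its Box with either BP_ThirdPersonCharacter or ThirdPersonCharacter enables input on the actor for player controller 0, and nothing here disables it again.
; Pressing E or V waits a configurable delay, then spawns the system at the Sphere's world location plus an offset, with configurable rotation and scale.
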(event OnComponentBeginOverlap(Box)
  (params (OverlappedComponent :type Primitive%20Component%20Object%20Reference) (OtherActor :type Actor%20Object%20Reference) (OtherComp :type Primitive%20Component%20Object%20Reference) (OtherBodyIndex :type Integer) (bFromSweep :type Boolean) (SweepResult :type Hit%20Result%20Structure%20%28by%20ref%29))
  (Utilities|Casting|CastToBP_ThirdPersonCharacter OtherActor
    (:then
      _)
    (:CastFailed
      (Utilities|Casting|CastToThirdPersonCharacter OtherActor)))
  (Input|EnableInput (Game|GetPlayerController 0)))

(event Input|KeyboardEvents|V
  (params (Key :type Key%20Structure :default "None"))
  (:Pressed
    (Utilities|FlowControl|Delay (Variables|Default|GetDelay))
    (Niagara|SpawnSystematLocation (Variables|Default|GetNiagara) (+ (Transformation|GetWorldLocation (Variables|Default|GetSphere)) (Variables|Default|GetLocation)) (Variables|Default|GetRotation) (Variables|Default|GetScale))))

(event Input|KeyboardEvents|E
  (params (Key :type Key%20Structure :default "None"))
  (:Pressed
    (Utilities|FlowControl|Delay (Variables|Default|GetDelay))
    (Niagara|SpawnSystematLocation (Variables|Default|GetNiagara) (+ (Transformation|GetWorldLocation (Variables|Default|GetSphere)) (Variables|Default|GetLocation)) (Variables|Default|GetRotation) (Variables|Default|GetScale))))

(fn ConstructionScript)