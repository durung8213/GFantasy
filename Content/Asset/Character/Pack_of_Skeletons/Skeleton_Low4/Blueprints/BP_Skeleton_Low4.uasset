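; BP_Skeleton_Low4 is a modular skeleton character from the Pack of Skeletons, built from separate armor, clothing, body and arbalest skeletal mesh parts.
; On BeginPlay, every part, including the head, helm, mask, quiver and crossbow pieces, sets the main Mesh as its leader pose component so all animate in sync.
; It has no other logic; Tick, overlap and construction script are empty.
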(event EventBeginPlay
  (Components|SkinnedMesh|SetLeaderPoseComponent (Variables|Default|GetSK_Skeleton_Low4_Toga) (Variables|Character|GetMesh) false false))

(event Collision|EventActorBeginOverlap
  (params (OtherActor :type Actor%20Object%20Reference)))

(event EventTick
  (params (DeltaSeconds :type Float%20%28single-precision%29)))

(fn ConstructionScript)