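; GAS player character Blueprint that adds a character customization mode with its own spring-arm camera.
; RPC and OffRPC toggle that camera and multicast character settings: owner-only visibility, hidden weapon, idle animation.
; Mouse input rotates, tilts and zooms the view, while Tick eases zoom and blends face-to-body camera height, corrected for viewport aspect.
; Hair color changes go through server and multicast events, creating dynamic materials for hair and visible bangs.
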(event Custom|GroundLoop
  (params (GroundPatternActive :type Boolean))
  (bind _asabp_ida_gasplayer (Utilities|Casting|CastToABP_IdaGASPlayer (Components|SkeletalMesh|GetAnimInstance (Variables|Character|GetMesh))))
  (Variables|/Game/Characters/Players/IdaFaberChar/ABP/ABP_IdaGASPlayer.ABP_IdaGASPlayer_C|SetGroundPatternActive _asabp_ida_gasplayer GroundPatternActive))

(event Custom|SendEventByTag
  (params (EventTag :type Gameplay%20Tag%20Structure))
  (Ability|SendGameplayEventtoActor self EventTag))

(event EventCustomizeCameraOff
  (CallFunction|CustomizeCameraSetting false))

(event EventBeginPlay
  (bind _asbp_gasworld_player_controller (Utilities|Casting|CastToBP_GASWorldPlayerController (Game|GetPlayerController 0)))
  (Variables|Default|SetWolrdPlayerControllerRef _asbp_gasworld_player_controller)
  (CallFunction|CustomizeCameraSetting false)
  (bind _keys (Utilities|Map|Keys (Variables|Default|GetMeshParts)))
  (for _array_element _keys
    (Rendering|SetReceivesDecals (.Value (Utilities|Map|Find (Variables|Default|GetMeshParts) _array_element)) false)))

(event Custom|OffRPC
  (CallFunction|OffCustomizeCamera)
  (CallFunction|MulticastCharacterOffSetting))

(event Custom|OffCustomizeCamera
  (CallFunction|CustomizeCameraSetting false)
  (Transformation|SetRelativeRotation (Variables|Character|GetMesh) (Math|Rotator|MakeRotator 0.0 0.0 -9e+01) false false))

(event Custom|OnCustomizeCamera
  (CallFunction|CameraPostionReset)
  (CallFunction|CustomizeCameraSetting true)
  (Transformation|SetRelativeRotation (Variables|Character|GetMesh) (Math|Rotator|MakeRotator 0.0 0.0 9e+01) false false))

(event Custom|MulticastHairColorChange
  (params (ColorParms :type Linear%20Color%20Structure) (HairMaterial :type Material%20Instance%20Object%20Reference))
  (bind _returnvalue (Class|GASPlayerCharacter|GetMeshPart "Bangs"))
  (bind _returnvalue_2 (Class|GASPlayerCharacter|GetMeshPart "Bangs"))
  (Variables|Customize|SetColor%20Parms ColorParms)
  (bind _output_get (Variables|Customize|SetHair%20Material HairMaterial))
  (if (== _output_get "/Game/Asset/Character/IdaFaber/Materials/Instances/Base/Wavy/MPMI_HAIR_Wavy_23.MPMI_HAIR_Wavy_23")
    (Utilities|FlowControl|Sequence
      (:then_0
        (bind _returnvalue_3 (Rendering|Material|CreateDynamicMaterialInstance (Class|GASPlayerCharacter|GetMeshPart "Hair") 0 (Variables|Customize|GetHair%20Material) "None" :!class /Script/Engine.PrimitiveComponent))
        (bind _output_get_2 (Variables|Customize|SetHairMID _returnvalue_3))
        (Utilities|Map|Add (Variables|Default|GetPartsMIDs) "Hair" _output_get_2)
        (Rendering|Material|SetVectorParameterValue (.Value (Utilities|Map|Find (Variables|Default|GetPartsMIDs) "Hair")) "CustomHairColor" (Variables|Customize|GetColor%20Parms) :!class /Script/Engine.MaterialInstanceDynamic))
      (:then_1
        (if (Variables|/Script/Engine.SceneComponent|GetbVisible _returnvalue_2)
          (bind _returnvalue_4 (Rendering|Material|CreateDynamicMaterialInstance _returnvalue_2 0 (Variables|Customize|GetHair%20Material) "None" :!class /Script/Engine.PrimitiveComponent))
          (bind _output_get_3 (Variables|Customize|SetBangsMID _returnvalue_4))
          (Utilities|Map|Add (Variables|Default|GetPartsMIDs) "Bangs" _output_get_3)
          (Rendering|Material|SetVectorParameterValue (.Value (Utilities|Map|Find (Variables|Default|GetPartsMIDs) "Bangs")) "CustomHairColor" (Variables|Customize|GetColor%20Parms) :!class /Script/Engine.MaterialInstanceDynamic))))
    (else
      (Utilities|FlowControl|Sequence
        (:then_0
          (bind _returnvalue_5 (Rendering|Material|CreateDynamicMaterialInstance (Class|GASPlayerCharacter|GetMeshPart "Hair") 0 (Variables|Customize|GetHair%20Material) "None" :!class /Script/Engine.PrimitiveComponent))
          (bind _output_get_4 (Variables|Customize|SetHairMID _returnvalue_5))
          (Utilities|Map|Add (Variables|Default|GetPartsMIDs) "Hair" _output_get_4))
        (:then_1
          (if (Variables|/Script/Engine.SceneComponent|GetbVisible _returnvalue)
            (bind _returnvalue_6 (Rendering|Material|CreateDynamicMaterialInstance _returnvalue 0 (Variables|Customize|GetHair%20Material) "None" :!class /Script/Engine.PrimitiveComponent))
            (bind _output_get_5 (Variables|Customize|SetBangsMID _returnvalue_6))
            (Utilities|Map|Add (Variables|Default|GetPartsMIDs) "Bangs" _output_get_5)))))))

(event Custom|Multicast_CharacterOffSetting
  (CallFunction|CustomizeCharacterSetting false))

(event Custom|RPC
  (CallFunction|OnCustomizeCamera)
  (CallFunction|MulticastCharacterSetting))

(event Custom|Multicast_CharacterSetting
  (CallFunction|CustomizeCharacterSetting true))

(event Custom|HairColorChange
  (params (ColorParms :type Linear%20Color%20Structure) (HairMaterial :type Material%20Instance%20Object%20Reference))
  (CallFunction|ServerHairColorChange ColorParms HairMaterial))

(event Custom|ServerHairColorChange
  (params (ColorParms :type Linear%20Color%20Structure) (HairMaterial :type Material%20Instance%20Object%20Reference))
  (CallFunction|MulticastHairColorChange ColorParms HairMaterial))

(event Input|EnhancedActionEvents|EnhancedInputActionIA_CustomizerLeftMouse
  (params (ActionValue :type Boolean) (ElapsedSeconds :type Float%20%28double-precision%29) (TriggeredSeconds :type Float%20%28double-precision%29) (InputAction :type Input%20Action%20Object%20Reference :default "/Game/Controller/PlayerController/Input/IA/Customizer/IA_CustomizerLeftMouse.IA_CustomizerLeftMouse"))
  (:Started
    (Variables|Customize|SetLMBClicked true))
  (:Completed
    (Variables|Customize|SetLMBClicked false)))

(event Input|EnhancedActionEvents|EnhancedInputActionIA_CustomizerRightMouse
  (params (ActionValue :type Boolean) (ElapsedSeconds :type Float%20%28double-precision%29) (TriggeredSeconds :type Float%20%28double-precision%29) (InputAction :type Input%20Action%20Object%20Reference :default "/Game/Controller/PlayerController/Input/IA/Customizer/IA_CustomizerRightMouse.IA_CustomizerRightMouse"))
  (:Started
    (Variables|Customize|SetRMBClicked true))
  (:Completed
    (Variables|Customize|SetRMBClicked false)))

(event Input|EnhancedActionEvents|EnhancedInputActionIA_CustomizerMouseWheel
  (params (ActionValue :type Float%20%28double-precision%29) (ElapsedSeconds :type Float%20%28double-precision%29) (TriggeredSeconds :type Float%20%28double-precision%29) (InputAction :type Input%20Action%20Object%20Reference :default "/Game/Controller/PlayerController/Input/IA/Customizer/IA_CustomizerMouseWheel.IA_CustomizerMouseWheel"))
  (bind _returnvalue (Viewport|GetViewportSize))
  (bind (_x _y) (Math|Vector2D|BreakVector2D _returnvalue))
  (bind _returnvalue_2 (/ _x _y))
  (bind _returnvalue_3 (Math|Float|MapRangeClamped _returnvalue_2 1.3 2.4 -2e+01 6e+01))
  (if (!= ActionValue 0.0)
    (Variables|Customize|SetDefaultCameraDistance (Math|Float|Clamp(Float) (- (Variables|/Script/Engine.SpringArmComponent|GetTargetArmLength (Variables|Default|GetCustomizeSpringArm)) (* ActionValue (Math|Curves|GetFloatValue (Variables|Customize|GetCameraZoom) (Variables|/Script/Engine.SpringArmComponent|GetTargetArmLength (Variables|Default|GetCustomizeSpringArm))))) (+ (Variables|Customize|GetMinCameraDistance) _returnvalue_3) (+ _returnvalue_3 (Variables|Customize|GetMaxCameraDistance))))))

(event Input|EnhancedActionEvents|EnhancedInputActionIA_CustomizerLookX
  (params (ActionValue :type Float%20%28double-precision%29) (ElapsedSeconds :type Float%20%28double-precision%29) (TriggeredSeconds :type Float%20%28double-precision%29) (InputAction :type Input%20Action%20Object%20Reference :default "/Game/Controller/PlayerController/Input/IA/Customizer/IA_CustomizerLookX.IA_CustomizerLookX"))
  (if (Variables|Customize|GetLMBClicked)
    (Pawn|Input|AddControllerYawInput (* ActionValue -2.0))))

(event Input|EnhancedActionEvents|EnhancedInputActionIA_CustomizerLookY
  (params (ActionValue :type Float%20%28double-precision%29) (ElapsedSeconds :type Float%20%28double-precision%29) (TriggeredSeconds :type Float%20%28double-precision%29) (InputAction :type Input%20Action%20Object%20Reference :default "/Game/Controller/PlayerController/Input/IA/Customizer/IA_CustomizerLookY.IA_CustomizerLookY"))
  (bind _customizespringarm (Variables|Default|GetCustomizeSpringArm))
  (bind _relativerotation (Variables|/Script/Engine.SceneComponent|GetRelativeRotation _customizespringarm))
  (if (Variables|Customize|GetRMBClicked)
    (Transformation|SetRelativeLocation (Variables|Default|GetCustomizeSpringArm) (Math|Vector|MakeVector 0.0 0.0 (Math|Float|Clamp(Float) (+ (* ActionValue 0.5) (.z (Variables|/Script/Engine.SceneComponent|GetRelativeLocation (Variables|Default|GetCustomizeSpringArm)))) 36.0 5e+01)) false false)
    (Transformation|SetRelativeRotation (Variables|Default|GetCustomizeSpringArm) (Math|Rotator|MakeRotator (.roll _relativerotation) (Math|Float|Clamp(Float) (- (.pitch _relativerotation) (* ActionValue 0.04)) -5.0 -4.0) (.yaw _relativerotation)) false false)))

(event EventTick
  (params (DeltaSeconds :type Float%20%28single-precision%29))
  (bind _returnvalue (Viewport|GetViewportSize))
  (bind (_x _y) (Math|Vector2D|BreakVector2D _returnvalue))
  (bind _returnvalue_2 (/ _x _y))
  (bind _returnvalue_3 (Math|Float|MapRangeClamped _returnvalue_2 1.3 2.4 -2e+01 6e+01))
  (if (Variables|/Game/BluePrints/PlayerController/BP_GASWorldPlayerController.BP_GASWorldPlayerController_C|GetOnCustomizing (Variables|Default|GetWolrdPlayerControllerRef))
    (Variables|Default|SetDelta%20Seconds DeltaSeconds)
    (bind _interpspeed (Timeline|Zoom Play)
      (:Update
        (Variables|/Script/Engine.SpringArmComponent|SetTargetArmLength (Variables|Default|GetCustomizeSpringArm) (Math|Interpolation|FInterpTo (Variables|/Script/Engine.SpringArmComponent|GetTargetArmLength (Variables|Default|GetCustomizeSpringArm)) (Variables|Customize|GetDefaultCameraDistance) (Variables|Default|GetDelta%20Seconds) _interpspeed))
        (Transformation|SetRelativeLocation (Variables|Default|GetCustomizeCamera) (Math|Vector|MakeVector 0.0 0.0 (Math|Float|Lerp (- (Variables|Customize|GetViewportHeightFaceLevel) (Math|Float|MapRangeClamped _returnvalue_2 1.3 2.4 -2.0 2.0)) (+ (Variables|Customize|GetViewportHeightBodyLevel) (Math|Float|MapRangeClamped _returnvalue_2 1.3 2.4 2e+01 -1e+01)) (Math|Float|MapRangeClamped (Variables|/Script/Engine.SpringArmComponent|GetTargetArmLength (Variables|Default|GetCustomizeSpringArm)) (+ (Variables|Customize|GetMinCameraDistance) _returnvalue_3) (+ _returnvalue_3 (Variables|Customize|GetMaxCameraDistance)) 0.0 1.0))) false false)))))

(fn ConstructionScript)

(fn GetInventoryComponent
  (return 0))

(fn GetEquipmentComponent
  (return 0))

(fn CustomizeCameraSetting
  (params (OnCustomize :type Boolean))
  (bind _returnvalue (not OnCustomize))
  (Utilities|FlowControl|Sequence
    (:then_0
      (Components|Activation|SetActive (Variables|Default|GetCustomizeSpringArm) OnCustomize false)
      (Components|Activation|SetActive (Variables|Default|GetCustomizeCamera) OnCustomize false))
    (:then_1
      (Components|Activation|SetActive (Variables|Default|GetFollowCamera) _returnvalue false)
      (Components|Activation|SetActive (Variables|Default|GetCameraBoom) _returnvalue false))))

(fn CustomizeCharacterSetting
  (params (OnCustomize :type Boolean))
  (bind _self self)
  (bind _mesh (Variables|Character|GetMesh))
  (bind _mesh_2 (Variables|Character|GetMesh))
  (bind _mesh_3 (Variables|Character|GetMesh))
  (bind _currentweapon (Variables|Default|GetCurrentWeapon _self))
  (Utilities|IsValid _currentweapon
    (:Is%20Valid
      (Rendering|SetVisibility (Variables|/Script/GFantasy.WeaponBase|GetWeaponMesh _currentweapon) (not OnCustomize) false))
    (:Is%20Not%20Valid
      _))
  (bind _values (Utilities|Map|Values (Variables|Default|GetMeshParts)))
  (for _array_element _values
    (Rendering|SetOnlyOwnerSee _array_element OnCustomize :!class /Script/Engine.PrimitiveComponent)
    (Collision|SetCollisionResponsetoChannel _array_element "ECC_GameTraceChannel2" "ECR_Ignore")
    (Collision|SetCollisionResponsetoChannel _array_element "ECC_Camera" "ECR_Ignore"))
  (Rendering|SetOnlyOwnerSee _mesh OnCustomize :!class /Script/Engine.PrimitiveComponent)
  (Collision|SetCollisionResponsetoChannel _mesh "ECC_GameTraceChannel2" "ECR_Ignore")
  (Collision|SetCollisionResponsetoChannel _mesh "ECC_Camera" "ECR_Ignore")
  (if OnCustomize
    (Components|Animation|SetAnimationMode _mesh_3 "AnimationSingleNode" true)
    (Components|Animation|PlayAnimation _mesh_3 "/Game/Characters/Players/Animation/Retarget/MF_Idle.MF_Idle" false)
    (else
      (Audio|Components|Audio|Stop _mesh_2)
      (Components|Animation|SetAnimationMode _mesh_2 "AnimationBlueprint" true)
      (Class|SkeletalMeshComponent|SetAnimClass _mesh_2 "/Game/Characters/Players/IdaFaberChar/ABP/ABP_IdaGASPlayer.ABP_IdaGASPlayer_C"))))

(fn CameraPostionReset
  (Pawn|SetControlRotation (Game|GetPlayerController 0) (Transformation|GetWorldRotation (Variables|Default|GetCameraPostionRef))))