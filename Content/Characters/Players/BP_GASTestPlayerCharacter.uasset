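; GAS test player character with a character-customizer camera mode, replicated hair material changes and a health bar fed by attribute callbacks.
; Customizing swaps follow camera for a close-up rig and flips the mesh; held mouse buttons gate turning and height/tilt.
; Wheel zoom interpolates arm length, blending camera height between face and body levels, compensated for viewport aspect ratio.
; Hair changes pass server-to-multicast, rebuilding hair and visible bangs MIDs, tinting only the Wavy_23 material.
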(event Custom|OnCustomizeCamera
  (Components|Activation|SetActive (Variables|Default|GetFollowCamera) false false)
  (Components|Activation|SetActive (Variables|Default|GetCamera) true false)
  (Components|Activation|SetActive (Variables|Default|GetCameraArm) true false)
  (Components|Activation|SetActive (Variables|Default|GetCameraBoom) false false)
  (Transformation|SetRelativeRotation (Variables|Character|GetMesh) (Math|Rotator|MakeRotator 0.0 0.0 9e+01) false false))

(event Custom|OffCustomizeCamera
  (Components|Activation|SetActive (Variables|Default|GetFollowCamera) true false)
  (Components|Activation|SetActive (Variables|Default|GetCamera) false false)
  (Components|Activation|SetActive (Variables|Default|GetCameraArm) false false)
  (Components|Activation|SetActive (Variables|Default|GetCameraBoom) true false)
  (Transformation|SetRelativeRotation (Variables|Character|GetMesh) (Math|Rotator|MakeRotator 0.0 0.0 -9e+01) false false))

(event Custom|ServerChangeParameter
  (params (NewParam :type Linear%20Color%20Structure) (NewParam2 :type Material%20Instance%20Object%20Reference))
  (CallFunction|MultiChangeParameter NewParam NewParam2))

(event Custom|MultiChangeParameter
  (params (NewParam :type Linear%20Color%20Structure) (NewParam2 :type Material%20Instance%20Object%20Reference))
  (bind _returnvalue (Class|GASPlayerCharacter|GetMeshPart "Bangs"))
  (bind _returnvalue_2 (Class|GASPlayerCharacter|GetMeshPart "Bangs"))
  (bind _output_get (Variables|Default|SetNew%20Param%202 NewParam2))
  (if (== _output_get "/Game/Asset/Character/IdaFaber/Materials/Instances/Base/Wavy/MPMI_HAIR_Wavy_23.MPMI_HAIR_Wavy_23")
    (Utilities|FlowControl|Sequence
      (:then_0
        (bind _returnvalue_3 (Rendering|Material|CreateDynamicMaterialInstance (Class|GASPlayerCharacter|GetMeshPart "Hair") 0 (Variables|Default|GetNew%20Param%202) "None" :!class /Script/Engine.PrimitiveComponent))
        (bind _output_get_2 (Variables|Default|SetHairMID _returnvalue_3))
        (Utilities|Map|Add (Variables|Default|GetPartsMIDs) "Hair" _output_get_2)
        (Rendering|Material|SetVectorParameterValue (.Value (Utilities|Map|Find (Variables|Default|GetPartsMIDs) "Hair")) "CustomHairColor" NewParam :!class /Script/Engine.MaterialInstanceDynamic))
      (:then_1
        (if (Variables|/Script/Engine.SceneComponent|GetbVisible _returnvalue_2)
          (bind _returnvalue_4 (Rendering|Material|CreateDynamicMaterialInstance _returnvalue_2 0 (Variables|Default|GetNew%20Param%202) "None" :!class /Script/Engine.PrimitiveComponent))
          (bind _output_get_3 (Variables|Default|SetBangsMID _returnvalue_4))
          (Utilities|Map|Add (Variables|Default|GetPartsMIDs) "Bangs" _output_get_3)
          (Rendering|Material|SetVectorParameterValue (.Value (Utilities|Map|Find (Variables|Default|GetPartsMIDs) "Bangs")) "CustomHairColor" NewParam :!class /Script/Engine.MaterialInstanceDynamic))))
    (else
      (Utilities|FlowControl|Sequence
        (:then_0
          (bind _returnvalue_5 (Rendering|Material|CreateDynamicMaterialInstance (Class|GASPlayerCharacter|GetMeshPart "Hair") 0 (Variables|Default|GetNew%20Param%202) "None" :!class /Script/Engine.PrimitiveComponent))
          (bind _output_get_4 (Variables|Default|SetHairMID _returnvalue_5))
          (Utilities|Map|Add (Variables|Default|GetPartsMIDs) "Hair" _output_get_4))
        (:then_1
          (if (Variables|/Script/Engine.SceneComponent|GetbVisible _returnvalue)
            (bind _returnvalue_6 (Rendering|Material|CreateDynamicMaterialInstance _returnvalue 0 (Variables|Default|GetNew%20Param%202) "None" :!class /Script/Engine.PrimitiveComponent))
            (bind _output_get_5 (Variables|Default|SetBangsMID _returnvalue_6))
            (Utilities|Map|Add (Variables|Default|GetPartsMIDs) "Bangs" _output_get_5)))))))

(event Custom|HairMIDColor
  (params (NewParam :type Linear%20Color%20Structure) (NewParam2 :type Material%20Instance%20Object%20Reference))
  (CallFunction|ServerChangeParameter NewParam NewParam2))

(event Input|EnhancedActionEvents|EnhancedInputActionIA_CustomizerLeftMouse
  (params (ActionValue :type Boolean) (ElapsedSeconds :type Float%20%28double-precision%29) (TriggeredSeconds :type Float%20%28double-precision%29) (InputAction :type Input%20Action%20Object%20Reference :default "/Game/Controller/PlayerController/Input/IA/Customizer/IA_CustomizerLeftMouse.IA_CustomizerLeftMouse"))
  (:Started
    (Variables|Default|SetLMBDown true))
  (:Completed
    (Variables|Default|SetLMBDown false)))

(event Input|EnhancedActionEvents|EnhancedInputActionIA_CustomizerRightMouse
  (params (ActionValue :type Boolean) (ElapsedSeconds :type Float%20%28double-precision%29) (TriggeredSeconds :type Float%20%28double-precision%29) (InputAction :type Input%20Action%20Object%20Reference :default "/Game/Controller/PlayerController/Input/IA/Customizer/IA_CustomizerRightMouse.IA_CustomizerRightMouse"))
  (:Started
    (Variables|Default|SetRMBDown true))
  (:Completed
    (Variables|Default|SetRMBDown false)))

(event Input|EnhancedActionEvents|EnhancedInputActionIA_CustomizerMouseWheel
  (params (ActionValue :type Float%20%28double-precision%29) (ElapsedSeconds :type Float%20%28double-precision%29) (TriggeredSeconds :type Float%20%28double-precision%29) (InputAction :type Input%20Action%20Object%20Reference :default "/Game/Controller/PlayerController/Input/IA/Customizer/IA_CustomizerMouseWheel.IA_CustomizerMouseWheel"))
  (bind _returnvalue (Viewport|GetViewportSize))
  (bind (_x _y) (Math|Vector2D|BreakVector2D _returnvalue))
  (bind _returnvalue_2 (/ _x _y))
  (bind _returnvalue_3 (Math|Float|MapRangeClamped _returnvalue_2 1.3 2.4 -2e+01 6e+01))
  (if (!= ActionValue 0.0)
    (Variables|Default|SetDefaultCameraDistance (Math|Float|Clamp(Float) (- (Variables|/Script/Engine.SpringArmComponent|GetTargetArmLength (Variables|Default|GetCameraArm)) (* ActionValue (Math|Curves|GetFloatValue (Variables|Default|GetCameraZoom) (Variables|/Script/Engine.SpringArmComponent|GetTargetArmLength (Variables|Default|GetCameraArm))))) (+ (Variables|Default|GetMinCameraDistance) _returnvalue_3) (+ _returnvalue_3 (Variables|Default|GetMaxCameraDistance))))))

(event Input|EnhancedActionEvents|EnhancedInputActionIA_CustomizerLookX
  (params (ActionValue :type Float%20%28double-precision%29) (ElapsedSeconds :type Float%20%28double-precision%29) (TriggeredSeconds :type Float%20%28double-precision%29) (InputAction :type Input%20Action%20Object%20Reference :default "/Game/Controller/PlayerController/Input/IA/Customizer/IA_CustomizerLookX.IA_CustomizerLookX"))
  (if (Variables|Default|GetLMBDown)
    (Pawn|Input|AddControllerYawInput (* ActionValue -2.0))))

(event Input|EnhancedActionEvents|EnhancedInputActionIA_CustomizerLookY
  (params (ActionValue :type Float%20%28double-precision%29) (ElapsedSeconds :type Float%20%28double-precision%29) (TriggeredSeconds :type Float%20%28double-precision%29) (InputAction :type Input%20Action%20Object%20Reference :default "/Game/Controller/PlayerController/Input/IA/Customizer/IA_CustomizerLookY.IA_CustomizerLookY"))
  (bind _cameraarm (Variables|Default|GetCameraArm))
  (bind _relativerotation (Variables|/Script/Engine.SceneComponent|GetRelativeRotation _cameraarm))
  (if (Variables|Default|GetRMBDown)
    (Transformation|SetRelativeLocation (Variables|Default|GetCameraArm) (Math|Vector|MakeVector 0.0 0.0 (Math|Float|Clamp(Float) (+ (* ActionValue 0.5) (.z (Variables|/Script/Engine.SceneComponent|GetRelativeLocation (Variables|Default|GetCameraArm)))) 36.0 5e+01)) false false)
    (Transformation|SetRelativeRotation (Variables|Default|GetCameraArm) (Math|Rotator|MakeRotator (.roll _relativerotation) (Math|Float|Clamp(Float) (- (.pitch _relativerotation) (* ActionValue 0.04)) -5.0 -4.0) (.yaw _relativerotation)) false false)))

(event EventTick
  (params (DeltaSeconds :type Float%20%28single-precision%29))
  (bind _returnvalue (Viewport|GetViewportSize))
  (bind (_x _y) (Math|Vector2D|BreakVector2D _returnvalue))
  (bind _returnvalue_2 (/ _x _y))
  (bind _returnvalue_3 (Math|Float|MapRangeClamped _returnvalue_2 1.3 2.4 -2e+01 6e+01))
  (if (Variables|/Game/BluePrints/PlayerController/BP_GASWorldPlayerController.BP_GASWorldPlayerController_C|GetOnCustomizing (Variables|Default|GetAs%20BP%20GASWorld%20Player%20Controller))
    (Variables|Default|SetDelta%20Seconds DeltaSeconds)
    (bind _interpspeed (Timeline|Zoom Play)
      (:Update
        (Variables|/Script/Engine.SpringArmComponent|SetTargetArmLength (Variables|Default|GetCameraArm) (Math|Interpolation|FInterpTo (Variables|/Script/Engine.SpringArmComponent|GetTargetArmLength (Variables|Default|GetCameraArm)) (Variables|Default|GetDefaultCameraDistance) (Variables|Default|GetDelta%20Seconds) _interpspeed))
        (Transformation|SetRelativeLocation (Variables|Default|GetCamera) (Math|Vector|MakeVector 0.0 0.0 (Math|Float|Lerp (- (Variables|Default|GetViewportHeightFaceLevel) (Math|Float|MapRangeClamped _returnvalue_2 1.3 2.4 -2.0 2.0)) (+ (Variables|Default|GetViewportHeightBodyLevel) (Math|Float|MapRangeClamped _returnvalue_2 1.3 2.4 2e+01 -1e+01)) (Math|Float|MapRangeClamped (Variables|/Script/Engine.SpringArmComponent|GetTargetArmLength (Variables|Default|GetCameraArm)) (+ (Variables|Default|GetMinCameraDistance) _returnvalue_3) (+ _returnvalue_3 (Variables|Default|GetMaxCameraDistance)) 0.0 1.0))) false false)))))

(event EventBeginPlay
  (bind _asbp_gasworld_player_controller (Utilities|Casting|CastToBP_GASWorldPlayerController (Game|GetPlayerController 0)))
  (Variables|Default|SetAs%20BP%20GASWorld%20Player%20Controller _asbp_gasworld_player_controller)
  (Components|Activation|SetActive (Variables|Default|GetFollowCamera) true false)
  (Components|Activation|SetActive (Variables|Default|GetCamera) false false)
  (Components|Activation|SetActive (Variables|Default|GetCameraArm) false false)
  (Components|Activation|SetActive (Variables|Default|GetCameraBoom) true false))

(event EventOnHealthChanged
  (params (CurrentHealth :type Float%20%28single-precision%29) (MaxHealth :type Float%20%28single-precision%29))
  (bind _healthbarwidgetref (Variables|Default|GetHealthBarWidgetRef))
  (Utilities|IsValid _healthbarwidgetref
    (:Is%20Valid
      (Default|SetHealthBar _healthbarwidgetref CurrentHealth MaxHealth))))

(fn ConstructionScript)

(fn InitOverlay
  (bind _returnvalue (UserInterface|CreateWidget "/Game/UI/World/Player/WBP_HealthBar.WBP_HealthBar_C"))
  (bind _output_get (Variables|Default|SetHealthBarWidgetRef _returnvalue))
  (UserInterface|Viewport|AddtoViewport _output_get 0))