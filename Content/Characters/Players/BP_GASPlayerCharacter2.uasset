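; GAS-based player character with a modular body, driven by the ABP_IdaGASPlayer animation blueprint.
; The construction script makes hair, head, eyes, lashes, caruncle and teeth follow the main mesh's pose as leader.
; GroundLoop passes a ground-pattern flag to the anim instance, and SendEventByTag fires gameplay events on the character itself.
; The M key plays the limit-break montage directly; inventory and equipment getters are empty stubs.
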(event Custom|GroundLoop
  (params (GroundPatternActive :type Boolean))
  (bind _asabp_ida_gasplayer (Utilities|Casting|CastToABP_IdaGASPlayer (Components|SkeletalMesh|GetAnimInstance (Variables|Character|GetMesh))))
  (Variables|/Game/Characters/Players/IdaFaberChar/ABP/ABP_IdaGASPlayer.ABP_IdaGASPlayer_C|SetGroundPatternActive _asabp_ida_gasplayer GroundPatternActive))

(event Custom|SendEventByTag
  (params (EventTag :type Gameplay%20Tag%20Structure))
  (Ability|SendGameplayEventtoActor self EventTag))

(event EventBeginPlay)

(event Collision|EventActorBeginOverlap
  (params (OtherActor :type Actor%20Object%20Reference)))

(event EventTick
  (params (DeltaSeconds :type Float%20%28single-precision%29)))

(event Input|KeyboardEvents|M
  (params (Key :type Key%20Structure))
  (:Pressed
    (Animation|Montage|PlayMontage (Variables|Character|GetMesh) "/Game/Characters/Players/IdaFaberChar/AM/Skill/AM_LimitBreak.AM_LimitBreak")))

(fn ConstructionScript
  (Components|SkinnedMesh|SetLeaderPoseComponent (Variables|Default|GetHair) (Variables|Character|GetMesh) false false)
  (Components|SkinnedMesh|SetLeaderPoseComponent (Variables|Default|GetEyes) (Variables|Character|GetMesh) false false)
  (Components|SkinnedMesh|SetLeaderPoseComponent (Variables|Default|GetHead) (Variables|Character|GetMesh) false false)
  (Components|SkinnedMesh|SetLeaderPoseComponent (Variables|Default|GetEyesLashes) (Variables|Character|GetMesh) false false)
  (Components|SkinnedMesh|SetLeaderPoseComponent (Variables|Default|GetCARUNCLE) (Variables|Character|GetMesh) false false)
  (Components|SkinnedMesh|SetLeaderPoseComponent (Variables|Default|GetTeeth) (Variables|Character|GetMesh) false false))

(fn GetInventoryComponent
  (return 0))

(fn GetEquipmentComponent
  (return 0))