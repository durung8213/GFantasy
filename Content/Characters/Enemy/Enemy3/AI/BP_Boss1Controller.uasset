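; AI controller for Boss 1 that runs the two-phase death when BossonDie fires.
; It stops the brain logic, then branches on BossLife.
; With a life left, it decrements it, plays the phase-two sequence for area players and heals the boss with a GAS effect.
; On the final death, it retags and ragdolls the boss, resets player views, notifies player states and starts a timed teleport.
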(event EventBeginPlay)

(event EventTick
  (params (DeltaSeconds :type Float%20%28single-precision%29)))

(event EventBossonDie
  (bind _returnvalue (Pawn|GetControlledPawn))
  (bind _returnvalue_2 (Pawn|GetControlledPawn))
  (bind _returnvalue_3 (Ability|GetAbilitySystemComponent _returnvalue))
  (AI|Logic|StopLogic (Variables|Default|GetBrainComponent) "PazeOneEnd")
  (switch int (Variables|Default|GetBossLife)
    (:0
      (Variables|/Script/Engine.Actor|SetTags _returnvalue_2 (Variables|Default|Get태그))
      (bind _asbp_boss_1 (Utilities|Casting|CastToBP_Boss1 _returnvalue_2))
      (Class|GASCombatNPC|Ragdoll _asbp_boss_1)
      (for _array_element (Variables|Default|GetInAreaPlayerArr)
        (bind _asbp_gasworld_player_controller (Utilities|Casting|CastToBP_GASWorldPlayerController (Pawn|GetController (Utilities|Struct|BreakInArrayPlayer _array_element))))
        (Game|Player|SetViewTargetwithBlend _asbp_gasworld_player_controller (Utilities|Struct|BreakInArrayPlayer _array_element) 0.0 "VTBlend_Linear" 0.0 false)
        (bind _asbp_world_player_state (Utilities|Casting|CastToBP_WorldPlayerState (Variables|/Script/Engine.Pawn|GetPlayerState (Utilities|Struct|BreakInArrayPlayer _array_element))))
        (Class|BossAIControllerBase|SendtoPlayerifDie _asbp_world_player_state)
        (Class|BossAIControllerBase|TpPlayerbyTime "-9187.000000,1072.000000,-114.000000" (Utilities|Struct|BreakInArrayPlayer _array_element) 8.0)))
    (:1
      (AI|ClearFocus)
      (Math|Integer|DecrementInt (Variables|Default|GetBossLife)
        (:%20%20
          (for _array_element_2 (Variables|Default|GetInAreaPlayerArr)
            (bind _asbp_kimmh_test_gas_world_player_controller (Utilities|Casting|CastToBP_KimmhTestGasWorldPlayerController (Pawn|GetController (Utilities|Struct|BreakInArrayPlayer _array_element_2)))
              (:then
                (Default|PlaySequence _asbp_kimmh_test_gas_world_player_controller "/Game/Scquence/Boss1/LS_Boss1Paze2.LS_Boss1Paze2"))
              (:CastFailed
                (bind _asbp_gasworld_player_controller_2 (Utilities|Casting|CastToBP_GASWorldPlayerController (Pawn|GetController (Utilities|Struct|BreakInArrayPlayer _array_element_2))))
                (Default|PlaySequence _asbp_gasworld_player_controller_2 "/Game/Scquence/Boss1/LS_Boss1Paze2.LS_Boss1Paze2")
                (Game|Player|SetViewTargetwithBlend _asbp_gasworld_player_controller_2 (Utilities|Struct|BreakInArrayPlayer _array_element_2) 0.0 "VTBlend_Linear" 0.0 false))))
          (Utilities|IsValid _returnvalue_3
            (:Is%20Valid
              (GameplayEffects|ApplyGameplayEffectSpecToSelf _returnvalue_3 (GameplayEffects|MakeOutgoingSpec _returnvalue_3 "/Game/BluePrints/GAS/GameplayEffect/Enemy/Enemy3/GE_BossHpHeal.GE_BossHpHeal_C" 1.0 (GameplayEffects|MakeEffectContext _returnvalue_3))))))))))

(fn ConstructionScript)