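; BP_Boss1 is a boss enemy character that supplies the data and hooks used to drive its behavior.
; Getters expose its patrol route, fixed attack and defend radii, and focus flag, while SetMovementSpeed writes the walk speed to CharacterMovement.
; The IRagdoll event triggers ragdoll and sets the dead flag, guarded so it runs only while the boss is not already dead.
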(event EventBeginPlay)

(event Collision|EventActorBeginOverlap
  (params (OtherActor :type Actor%20Object%20Reference)))

(event EventTick
  (params (DeltaSeconds :type Float%20%28single-precision%29)))

(event EventIRagdoll
  (bind _returnvalue (Class|BossLilither|GetIsDead))
  (if (not _returnvalue)
    (Class|GASCombatNPC|Ragdoll)
    (Class|BossLilither|SetIsDead true)))

(fn ConstructionScript)

(fn GetPatrolRoute
  (return (Variables|Default|GetPatrolRoute)))

(fn GetIdealRange
  (return 1e+03 2e+03))

(fn GetIsFocus
  (return (Variables|Default|GetbIsFocus)))

(fn SetMovementSpeed
  (params (Speed :type Float%20%28double-precision%29))
  (bind _output_get (Variables|/Script/Engine.CharacterMovementComponent|SetMaxWalkSpeed (Variables|Character|GetCharacterMovement) Speed))
  (return _output_get))