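; Wolf enemy Blueprint that gives each wolf a random coat by applying a material from the WolfMaterial array to its mesh on BeginPlay.
; Overlap and Tick events are empty.
; An unconnected, never-executed branch holds client-side logic that shows the enemy state widget when the wolf is within range and line of sight of the player, requesting ServerInitHealths once per appearance.
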(event EventBeginPlay
  (Rendering|Material|SetMaterial (Variables|Character|GetMesh) 0 (.OutItem (Utilities|Array|Random (Variables|Default|GetWolfMaterial)))))

(event Collision|EventActorBeginOverlap
  (params (OtherActor :type Actor%20Object%20Reference)))

(event EventTick
  (params (DeltaSeconds :type Float%20%28single-precision%29)))

(fn ConstructionScript)