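; BP_Dummy is a dummy enemy character that equips a great sword on BeginPlay.
; An IRagdoll event triggers Ragdoll once, guarded by the IsRagdoll flag.
; Patrol route, ideal range, focus and movement speed functions are stubs returning empty, zero or false values.
; An unconnected chain that would disable CharacterMovement physics push and print a collision-prevention message never runs.
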(event EventBeginPlay
  (Class|GASCombatNPC|SetWeapon (Variables|Default|GetBP_GreatSword)))

(event Collision|EventActorBeginOverlap
  (params (OtherActor :type Actor%20Object%20Reference)))

(event EventTick
  (params (DeltaSeconds :type Float%20%28single-precision%29)))

(event EventIRagdoll
  (if (not (Variables|Default|GetbIsRagdoll))
    (Class|GASCombatNPC|Ragdoll)))

(fn ConstructionScript)

(fn GetPatrolRoute
  (return 0))

(fn GetIdealRange
  (return 0.0 0.0))

(fn GetIsFocus
  (return false))

(fn SetMovementSpeed
  (params (Speed :type Float%20%28double-precision%29))
  (return 0.0))