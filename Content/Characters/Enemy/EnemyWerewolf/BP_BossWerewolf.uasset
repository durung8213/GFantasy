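; Werewolf boss enemy whose second phase swaps clothing meshes and body material and trades the dagger for two claws.
; Construction makes child skeletal meshes follow the main mesh's pose and builds the per-phase mesh lists used by two near-duplicate phase-change events.
; Unless spawner-spawned, BeginPlay registers all three child-actor weapons, retrying on a timer until valid, with claws hidden.
; Multi-prefixed events toggle the power-up Niagara effect and reposition the camera.
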(event Custom|ChangeMesh2Phase
  (Utilities|FlowControl|Sequence
    (:then_0
      (for _array_element (Variables|Default|GetPhase2HideMesh)
        (Rendering|SetVisibility _array_element false false)))
    (:then_1
      (for _array_element_2 (Variables|Default|GetPhase2Mesh)
        (Rendering|SetVisibility _array_element_2 true false)))
    (:then_2
      (Rendering|Material|SetMaterial (Variables|Character|GetMesh) 4 "/Game/Asset/Character/Druid_Werewolf/Materials/MI_Druid_Werewolf_Body_Inst.MI_Druid_Werewolf_Body_Inst"))
    (:then_3
      (Components|Activation|Activate (Variables|Default|GetPowerUpPartical) false))
    (:then_4
      (Rendering|SetVisibility (Variables|Default|GetBP_WerewolfDagger) false false)
      (Rendering|SetVisibility (Variables|Default|GetBP_ClawL) true false)
      (Rendering|SetVisibility (Variables|Default|GetBP_ClawR) true false))))

(event Custom|MultiSetCameraRelativeLocationAndRotation
  (params (NewLocation :type Vector) (NewRotation :type Rotator))
  (Transformation|SetRelativeLocationAndRotation (Variables|Default|GetCamera) NewLocation NewRotation false false))

(event Custom|MultiActivePowerUp
  (Components|Activation|Activate (Variables|Default|GetPowerUpNiagra) true))

(event Custom|MultiDeactivePowerUp
  (Components|Activation|Deactivate (Variables|Default|GetPowerUpNiagra)))

(event EventBeginPlay
  (if (not (Variables|Default|GetbIsSpawnBySpawner))
    (Class|GASCombatNPC|InitWeapon)
    (Development|PrintString "무기 장착(BeginPlay)" true true "(R=0.089390,G=0.175747,B=1.000000,A=1.000000)")))

(event Collision|EventActorBeginOverlap
  (params (OtherActor :type Actor%20Object%20Reference)))

(event EventTick
  (params (DeltaSeconds :type Float%20%28single-precision%29)))

(event EventChangeMeshTwoPhase
  (bind _bp_clawr (Variables|Default|GetBP_ClawR))
  (bind _bp_clawl (Variables|Default|GetBP_ClawL))
  (Utilities|FlowControl|Sequence
    (:then_0
      (for _array_element (Variables|Default|GetPhase2HideMesh)
        (Rendering|SetVisibility _array_element false false)))
    (:then_1
      (for _array_element_2 (Variables|Default|GetPhase2Mesh)
        (Rendering|SetVisibility _array_element_2 true false)))
    (:then_2
      (Rendering|Material|SetMaterial (Variables|Character|GetMesh) 4 "/Game/Asset/Character/Druid_Werewolf/Materials/MI_Druid_Werewolf_Body_Inst.MI_Druid_Werewolf_Body_Inst"))
    (:then_4
      (Rendering|SetVisibility (Variables|Default|GetBP_WerewolfDagger) false false)
      (Utilities|FlowControl|Sequence
        (:then_0
          (Rendering|SetVisibility _bp_clawl true false)
          (Rendering|SetVisibility (Variables|/Script/Engine.Actor|GetRootComponent (Variables|/Script/Engine.ChildActorComponent|GetChildActor _bp_clawl)) true false))
        (:then_1
          (Rendering|SetVisibility _bp_clawr true false)
          (Rendering|SetVisibility (Variables|/Script/Engine.Actor|GetRootComponent (Variables|/Script/Engine.ChildActorComponent|GetChildActor _bp_clawr)) true false))))))

(event EventInitWeapon
  (bind _bp_clawl (Variables|Default|GetBP_ClawL))
  (bind _bp_werewolfdagger (Variables|Default|GetBP_WerewolfDagger))
  (bind _bp_clawl_2 (Variables|Default|GetBP_ClawL))
  (bind _bp_clawr (Variables|Default|GetBP_ClawR))
  (bind _bp_clawr_2 (Variables|Default|GetBP_ClawR))
  (if (Math|Boolean|ANDBoolean (Utilities|IsValidClass (Variables|/Script/Engine.ChildActorComponent|GetChildActorClass _bp_werewolfdagger)) (Utilities|IsValid (Variables|/Script/Engine.ChildActorComponent|GetChildActor _bp_werewolfdagger)) (Utilities|IsValidClass (Variables|/Script/Engine.ChildActorComponent|GetChildActorClass _bp_clawl_2)) (Utilities|IsValid (Variables|/Script/Engine.ChildActorComponent|GetChildActor _bp_clawl_2)) (Utilities|IsValidClass (Variables|/Script/Engine.ChildActorComponent|GetChildActorClass _bp_clawr_2)) (Utilities|IsValid (Variables|/Script/Engine.ChildActorComponent|GetChildActor _bp_clawr_2)))
    (Utilities|FlowControl|Sequence
      (:then_0
        (Class|GASCombatNPC|SetWeapon (Variables|Default|GetBP_WerewolfDagger)))
      (:then_1
        (Class|GASCombatNPC|AddWeaponArr (Variables|Default|GetBP_WerewolfDagger)))
      (:then_2
        (Class|GASCombatNPC|AddWeaponArr (Variables|Default|GetBP_ClawL)))
      (:then_3
        (Class|GASCombatNPC|AddWeaponArr (Variables|Default|GetBP_ClawR)))
      (:then_4
        (Rendering|SetVisibility _bp_clawl false false)
        (Rendering|SetVisibility (Variables|/Script/Engine.Actor|GetRootComponent (Variables|/Script/Engine.ChildActorComponent|GetChildActor _bp_clawl)) false false))
      (:then_5
        (Rendering|SetVisibility _bp_clawr false false)
        (Rendering|SetVisibility (Variables|/Script/Engine.Actor|GetRootComponent (Variables|/Script/Engine.ChildActorComponent|GetChildActor _bp_clawr)) false false)))
    (else
      (Utilities|Time|SetTimerbyEvent (delegate EventInitWeapon) 0.5))))

(fn ConstructionScript
  (bind _sk_druid_werewolf_capfur (Variables|Default|GetSK_Druid_Werewolf_CapFur))
  (bind _sk_druid_werewolf_pants (Variables|Default|GetSK_Druid_Werewolf_Pants))
  (Utilities|FlowControl|Sequence
    (:then_0
      (for _array_element (Components|GetChildrenComponents (Variables|Character|GetMesh) true)
        (bind _asskeletal_mesh_component (Utilities|Casting|CastToSkeletalMeshComponent _array_element))
        (Components|SkinnedMesh|SetLeaderPoseComponent _asskeletal_mesh_component (Variables|Character|GetMesh) true true)))
    (:then_1
      (Utilities|Array|Add (Variables|Default|GetPhase2Mesh) _sk_druid_werewolf_capfur)
      (for _array_element_2 (Components|GetChildrenComponents _sk_druid_werewolf_capfur true)
        (bind _asskeletal_mesh_component_2 (Utilities|Casting|CastToSkeletalMeshComponent _array_element_2))
        (Utilities|Array|Add (Variables|Default|GetPhase2Mesh) _asskeletal_mesh_component_2)))
    (:then_2
      (for _array_element_3 (Variables|Default|GetPhase2Mesh)
        (Rendering|SetVisibility _array_element_3 false false)))
    (:then_3
      (Utilities|Array|Add (Variables|Default|GetPhase2HideMesh) _sk_druid_werewolf_pants)
      (for _array_element_4 (Components|GetChildrenComponents _sk_druid_werewolf_pants true)
        (bind _asskeletal_mesh_component_3 (Utilities|Casting|CastToSkeletalMeshComponent _array_element_4))
        (Utilities|Array|Add (Variables|Default|GetPhase2HideMesh) _asskeletal_mesh_component_3))
      (Utilities|Array|Add (Variables|Default|GetPhase2HideMesh) (Variables|Default|GetShirt))
      (Utilities|Array|Add (Variables|Default|GetPhase2HideMesh) (Variables|Default|GetSK_Druid_Werewolf_Armlets)))
    (:then_4
      (for _array_element_5 (Variables|Default|GetPhase2HideMesh)
        (Rendering|SetVisibility _array_element_5 true false)))))