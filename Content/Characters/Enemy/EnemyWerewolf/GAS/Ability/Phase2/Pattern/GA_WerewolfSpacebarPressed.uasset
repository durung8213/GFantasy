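; Player gameplay ability for a spacebar press in the werewolf boss's phase 2 pattern, feeding an extra gauge.
; On activation it notifies the player controller's extra gauge UI of the click.
; It then applies GE_ExtraGaugeAdd from its own ability system component to each BP_BossWerewolf whose first tag is Enemy.
; The ability ends immediately afterwards, so each activation counts as one press.
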(event Ability|EventActivateAbility
  (Utilities|FlowControl|Sequence
    (:then_0
      (bind _asbp_gasplayer_character (Utilities|Casting|CastToBP_GASPlayerCharacter (Ability|GetAvatarActorfromActorInfo)))
      (bind _asbp_gasworld_player_controller (Utilities|Casting|CastToBP_GASWorldPlayerController (Pawn|GetController _asbp_gasplayer_character)))
      (Class|GASWorldPlayerController|ExtraGaugeUISpacebarClick _asbp_gasworld_player_controller))
    (:then_1
      (bind _outactors (Actor|GetAllActorsOfClass "/Game/Characters/Enemy/EnemyWerewolf/BP_BossWerewolf.BP_BossWerewolf_C"))
      (bind _array_element (Utilities|Array|ForEachLoopwithBreak _outactors)
        (:LoopBody
          (if (== (Utilities|Array|Get(acopy) (Variables|/Script/Engine.Actor|GetTags _array_element)) "Enemy")
            (Class|GASAbilitySystemLibrary|ApplyGASEffecttoTargettoASC (Ability|GetAbilitySystemComponentfromActorInfo) (Ability|GetAbilitySystemComponent _array_element) "/Game/Characters/Enemy/EnemyWerewolf/GAS/Effect/Phase2/Pattern/GE_ExtraGaugeAdd.GE_ExtraGaugeAdd_C" 1.0)))
        (:Completed
          (Ability|EndAbility))))))

(event Ability|EventOnEndAbility
  (params (bWasCancelled :type Boolean)))