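; Werewolf boss phase 2 ability for the looping ground pattern, run against the AI's focus actor.
; It grants and activates the target's paired ability by tag and plays the loop montage.
; Each loop event applies attack damage and camera shake, until the extra-gauge-full event arrives or the target's checked attribute hits zero.
; Either exit sets Blackboard outcome flags, signals the player, removes the spacebar effect and ends the ability.
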(event Ability|EventActivateAbility
  (bind _returnvalue (Class|GAEndDelegateBase|GetCurrentController))
  (bind _returnvalue_2 (Class|AIController|GetFocusActor _returnvalue))
  (bind _returnvalue_3 (Ability|GetAbilitySystemComponent _returnvalue_2))
  (Utilities|FlowControl|Sequence
    (:then_0
      (Utilities|IsValid _returnvalue_2
        (:Is%20Valid
          (Variables|Default|SetOtherActor _returnvalue_2)
          (Utilities|IsValid _returnvalue_3
            (:Is%20Valid
              (Variables|Default|SetOtherActorAbilityComponent _returnvalue_3))))))
    (:then_1
      (bind _returnvalue_4 (Class|GASAbilitySystemLibrary|ApplyGASEffecttoTargettoASC (Ability|GetAbilitySystemComponentfromActorInfo) (Variables|Default|GetOtherActorAbilityComponent) "/Game/Characters/Enemy/EnemyWerewolf/GAS/Effect/Phase2/Pattern/GE_GivePatternGroundLoopAbility.GE_GivePatternGroundLoopAbility_C" 1.0))
      (if _returnvalue_4
        (Abilities|TryActivateAbilitiesbyTag (Variables|Default|GetOtherActorAbilityComponent) (Variables|Default|GetGameplay%20Tag%20Container) true)
        (else
          (Ability|EndAbility))))
    (:then_2
      (|PlayMontageandWaitProxy "None" "/Game/Characters/Enemy/EnemyWerewolf/Animation/PhaseTwo/Pattern/Ground/AM_Ground_loop.AM_Ground_loop" 1.0 "None" true 1.0 0.0 false))
    (:then_3
      (bind _asynctaskproxy (Ability|Tasks|WaitGameplayEvent "(TagName=\"Enemy.Boss.ExtraGaugeFull\")" 0)
        (:then
          (Variables|Default|SetExtraGaugeAsyncTask _asynctaskproxy))
        (:EventReceived
          (Utilities|FlowControl|Sequence
            (:then_0
              (AI|Components|Blackboard|SetValueasBool (Variables|/Script/AIModule.AIController|GetBlackboard (AI|GetAIController (Ability|GetAvatarActorfromActorInfo))) (Variables|Default|GetKey%20bCanGroundPattern) false))
            (:then_1
              (Utilities|Casting|CastToBP_GASPlayerCharacter (Variables|Default|GetOtherActor))
              (Ability|SendGameplayEventtoActor (Variables|Default|GetOtherActor) "(TagName=\"Combat.Pattern1.Loop\")"))
            (:then_2
              (AI|Components|Blackboard|SetValueasBool (Variables|/Script/AIModule.AIController|GetBlackboard (AI|GetAIController (Ability|GetAvatarActorfromActorInfo))) (Variables|Default|GetKey%20bGroundPatternPlayerDie) false))
            (:then_3
              (GameplayEffects|RemoveActiveGameplayEffectbySourceEffect (Variables|Default|GetOtherActorAbilityComponent) "/Game/Characters/Enemy/EnemyWerewolf/GAS/Effect/Phase2/Pattern/GE_GivePatternGroundSpacebarPressed.GE_GivePatternGroundSpacebarPressed_C" 0 -1))
            (:then_4
              (Ability|EndAbility))))))
    (:then_4
      (bind _asynctaskproxy_2 (Ability|Tasks|WaitGameplayEvent "(TagName=\"Combat.Pattern1.Loop\")" 0)
        (:then
          (Variables|Default|SetAttackAsyncTask _asynctaskproxy_2))
        (:EventReceived
          (Class|GASAbilitySystemLibrary|ApplyGASEffecttoTargettoASC (Ability|GetAbilitySystemComponentfromActorInfo) (Variables|Default|GetOtherActorAbilityComponent) "/Game/Characters/Enemy/EnemyWerewolf/GAS/Effect/Phase2/Pattern/GE_PatternGroundAttack.GE_PatternGroundAttack_C" 1.0)
          (bind _asbp_gasplayer_character (Utilities|Casting|CastToBP_GASPlayerCharacter (Variables|Default|GetOtherActor)))
          (bind _as플레이어_컨트롤러 (Utilities|Casting|CastToPlayerController (Pawn|GetController _asbp_gasplayer_character)))
          (Game|Feedback|ClientStartCameraShake _as플레이어_컨트롤러 "/Game/BluePrints/Combat/PlayerSkill/Camera/BP_CS_ChargeShake.BP_CS_ChargeShake_C" 1.0 "CameraLocal" "0, 0, 0")
          (if (<= (.ReturnValue (Class|AbilitySystemComponent|GetGameplayAttributeValue (Variables|Default|GetOtherActorAbilityComponent) "(AttributeName=\"Health\",Attribute=/Script/GFantasy.GASCharacterAS:Health,AttributeOwner=\"/Script/CoreUObject.Class'/Script/GFantasy.GASCharacterAS'\")")) 0.0)
            (Utilities|FlowControl|Sequence
              (:then_0
                (AI|Components|Blackboard|SetValueasBool (Variables|/Script/AIModule.AIController|GetBlackboard (AI|GetAIController (Ability|GetAvatarActorfromActorInfo))) (Variables|Default|GetKey%20bCanGroundPattern) false))
              (:then_1
                (Utilities|Casting|CastToBP_GASPlayerCharacter (Variables|Default|GetOtherActor))
                (Ability|SendGameplayEventtoActor (Variables|Default|GetOtherActor) "(TagName=\"Combat.Pattern1.Loop\")"))
              (:then_2
                (AI|Components|Blackboard|SetValueasBool (Variables|/Script/AIModule.AIController|GetBlackboard (AI|GetAIController (Ability|GetAvatarActorfromActorInfo))) (Variables|Default|GetKey%20bGroundPatternPlayerDie) true))
              (:then_3
                (GameplayEffects|RemoveActiveGameplayEffectbySourceEffect (Variables|Default|GetOtherActorAbilityComponent) "/Game/Characters/Enemy/EnemyWerewolf/GAS/Effect/Phase2/Pattern/GE_GivePatternGroundSpacebarPressed.GE_GivePatternGroundSpacebarPressed_C" 0 -1))
              (:then_4
                (Ability|EndAbility)))))))))

(event Ability|EventOnEndAbility
  (params (bWasCancelled :type Boolean))
  (bind _attackasynctask (Variables|Default|GetAttackAsyncTask))
  (bind _extragaugeasynctask (Variables|Default|GetExtraGaugeAsyncTask))
  (Utilities|IsValid _attackasynctask
    (:Is%20Valid
      (GameplayTasks|EndTask _attackasynctask))
    (:Is%20Not%20Valid
      _))
  (Utilities|IsValid _extragaugeasynctask
    (:Is%20Valid
      (GameplayTasks|EndTask _extragaugeasynctask))))