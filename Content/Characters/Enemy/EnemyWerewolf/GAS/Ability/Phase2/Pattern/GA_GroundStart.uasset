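; Werewolf boss GAS ability that starts the phase 2 ground pattern against the controller's focus actor.
; It repositions the boss camera, turns the target to face the boss, grants and activates the target's pattern ability through a gameplay effect, and plays the start montage.
; On the Combat.Pattern1.Start event, it applies the spacebar effect, switches the player's view to the boss and binds the boss extra gauge UI.
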(event Ability|EventActivateAbility
  (bind _returnvalue (Class|GAEndDelegateBase|GetCurrentController))
  (bind _returnvalue_2 (Class|AIController|GetFocusActor _returnvalue))
  (bind _returnvalue_3 (Ability|GetAbilitySystemComponent _returnvalue_2))
  (Utilities|FlowControl|Sequence
    (:then_0
      (Utilities|IsValid _returnvalue_2
        (:Is%20Valid
          (Variables|Default|SetOtherActor _returnvalue_2)
          (Utilities|IsValid _returnvalue_3
            (:Is%20Valid
              (Variables|Default|SetOtherActorAbilityComponent _returnvalue_3))))))
    (:then_1
      (bind _asbp_boss_werewolf (Utilities|Casting|CastToBP_BossWerewolf (Ability|GetAvatarActorfromActorInfo)))
      (Default|MultiSetCameraRelativeLocationandRotation _asbp_boss_werewolf "-12.800000,93.500000,62.200000" "30.000000,270.000000,0.000000"))
    (:then_2
      (bind _asboss_were_wolf_character (Utilities|Casting|CastToBossWereWolfCharacter (Ability|GetAvatarActorfromActorInfo)))
      (Class|BossWereWolfCharacter|MultiRotateActor _asboss_were_wolf_character (Variables|Default|GetOtherActor) (Math|Rotator|MakeRotator 0.0 0.0 (.yaw (Math|Rotator|MakeRotfromX (- (Transformation|GetActorLocation (Ability|GetAvatarActorfromActorInfo)) (Transformation|GetActorLocation (Variables|Default|GetOtherActor))))))))
    (:then_3
      (bind _returnvalue_4 (Class|GASAbilitySystemLibrary|ApplyGASEffecttoTargettoASC (Ability|GetAbilitySystemComponentfromActorInfo) (Variables|Default|GetOtherActorAbilityComponent) "/Game/Characters/Enemy/EnemyWerewolf/GAS/Effect/Phase2/Pattern/GE_GivePatternGroundStartAbility.GE_GivePatternGroundStartAbility_C" 1.0))
      (if _returnvalue_4
        (Abilities|TryActivateAbilitiesbyTag (Variables|Default|GetOtherActorAbilityComponent) (Variables|Default|GetGameplay%20Tag%20Container) true)
        (else
          (Ability|EndAbility))))
    (:then_4
      (bind _asynctaskproxy (Ability|Tasks|WaitGameplayEvent "(TagName=\"Combat.Pattern1.Start\")" 0)
        (:then
          (Variables|Default|SetChnageCameraTask _asynctaskproxy))
        (:EventReceived
          (Class|GASAbilitySystemLibrary|ApplyGASEffecttoTargettoASC (Ability|GetAbilitySystemComponentfromActorInfo) (Variables|Default|GetOtherActorAbilityComponent) "/Game/Characters/Enemy/EnemyWerewolf/GAS/Effect/Phase2/Pattern/GE_GivePatternGroundSpacebarPressed.GE_GivePatternGroundSpacebarPressed_C" 1.0)
          (bind _asbp_gasplayer_character (Utilities|Casting|CastToBP_GASPlayerCharacter (Variables|Default|GetOtherActor)))
          (bind _asbp_gasworld_player_controller (Utilities|Casting|CastToBP_GASWorldPlayerController (Pawn|GetController _asbp_gasplayer_character))
            (:then
              (Game|Player|SetViewTargetwithBlend _asbp_gasworld_player_controller (Ability|GetAvatarActorfromActorInfo) 0.0 "VTBlend_Linear" 0.0 false)
              (Class|GASWorldPlayerController|ClientShowBossExtraGaugeUI _asbp_gasworld_player_controller)
              (bind _asbp_boss_werewolf_2 (Utilities|Casting|CastToBP_BossWerewolf (Ability|GetAvatarActorfromActorInfo)))
              (Class|GASWorldPlayerController|BindBossExtraGauge _asbp_gasworld_player_controller _asbp_boss_werewolf_2))
            (:CastFailed
              (Development|PrintString "OtherActor의 컨트롤러가 BP_GasWorldPlayerController 가 아님" true true "(R=1.000000,G=0.119460,B=0.000000,A=1.000000)"))))))
    (:then_5
      (|PlayMontageandWaitProxy "None" "/Game/Characters/Enemy/EnemyWerewolf/Animation/PhaseTwo/Pattern/Ground/AM_Ground_Start.AM_Ground_Start" 1.0 "None" true 1.0 0.0 false
        (:OnCompleted
          (Ability|EndAbility))))))

(event Ability|EventOnEndAbility
  (params (bWasCancelled :type Boolean))
  (GameplayTasks|EndTask (Variables|Default|GetChnageCameraTask)))