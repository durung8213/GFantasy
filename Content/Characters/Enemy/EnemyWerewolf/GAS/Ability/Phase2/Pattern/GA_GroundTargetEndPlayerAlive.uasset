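; Player-side gameplay ability in the werewolf boss's phase 2 pattern, apparently ending a ground-target sequence in which the player survives.
; On activation it turns off the player character's ground loop, returns the controller's view target to that character, and has the client destroy the boss extra gauge UI.
; It then plays the end-alive montage and ends the ability only when that montage completes.
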(event Ability|EventActivateAbility
  (Utilities|FlowControl|Sequence
    (:then_0
      (bind _asbp_gasplayer_character (Utilities|Casting|CastToBP_GASPlayerCharacter (Ability|GetAvatarActorfromActorInfo)))
      (Utilities|FlowControl|Sequence
        (:then_0
          (Default|GroundLoop _asbp_gasplayer_character false))
        (:then_1
          (bind _asbp_gasworld_player_controller (Utilities|Casting|CastToBP_GASWorldPlayerController (Pawn|GetController _asbp_gasplayer_character)))
          (Game|Player|SetViewTargetwithBlend _asbp_gasworld_player_controller _asbp_gasplayer_character 0.0 "VTBlend_Linear" 0.0 false)
          (Class|GASWorldPlayerController|ClientDestroyBossExtraGaugeUI _asbp_gasworld_player_controller))))
    (:then_1
      (|PlayMontageandWaitProxy "None" "/Game/Characters/Enemy/EnemyWerewolf/Animation/PhaseTwo/Pattern/Ground/Target/AM_Ground_Target_EndAlive.AM_Ground_Target_EndAlive" 1.0 "None" true 1.0 0.0 false
        (:OnCompleted
          (Ability|EndAbility))))))

(event Ability|EventOnEndAbility
  (params (bWasCancelled :type Boolean)))