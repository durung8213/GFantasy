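; Werewolf boss Phase 2 gameplay ability for the ending of the Ground pattern that, by its name, kills the player.
; It caches the AI focus actor's ability system, plays the ground-end montage and immediately applies the pattern's player-die effect to that target.
; On success it remotely activates a tagged ability on the target, otherwise it ends.
; Ending the ability applies an extra-gauge reset effect to the werewolf.
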(event Ability|EventActivateAbility
  (bind _returnvalue (Class|GAEndDelegateBase|GetCurrentController))
  (bind _returnvalue_2 (Class|AIController|GetFocusActor _returnvalue))
  (bind _returnvalue_3 (Ability|GetAbilitySystemComponent _returnvalue_2))
  (Utilities|FlowControl|Sequence
    (:then_0
      (Utilities|IsValid _returnvalue_2
        (:Is%20Valid
          (Variables|Default|SetOtherActor _returnvalue_2)
          (Utilities|IsValid _returnvalue_3
            (:Is%20Valid
              (Variables|Default|SetOtherActorAbilityComponent _returnvalue_3))))))
    (:then_1
      (|PlayMontageandWaitProxy "None" "/Game/Characters/Enemy/EnemyWerewolf/Animation/PhaseTwo/Pattern/Ground/AM_Ground_End.AM_Ground_End" 1.0 "None" true 1.0 0.0 false
        (:then
          (bind _returnvalue_4 (Class|GASAbilitySystemLibrary|ApplyGASEffecttoTargettoASC (Ability|GetAbilitySystemComponentfromActorInfo) (Variables|Default|GetOtherActorAbilityComponent) "/Game/Characters/Enemy/EnemyWerewolf/GAS/Effect/Phase2/Pattern/GE_GivePatternGroundEndPlayerDie.GE_GivePatternGroundEndPlayerDie_C" 1.0))
          (if _returnvalue_4
            (Abilities|TryActivateAbilitiesbyTag (Variables|Default|GetOtherActorAbilityComponent) (Variables|Default|GetGameplay%20Tag%20Container) true)
            (else
              (Ability|EndAbility))))
        (:OnCompleted
          (Ability|EndAbility))))))

(event Ability|EventOnEndAbility
  (params (bWasCancelled :type Boolean))
  (Class|GASAbilitySystemLibrary|ApplyGASEffecttoSelftoASC (Ability|GetAbilitySystemComponentfromActorInfo) "/Game/Characters/Enemy/EnemyWerewolf/GAS/Effect/Phase2/Pattern/GE_ResetExtraGauge.GE_ResetExtraGauge_C" 1.0))