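; Gameplay ability for the Werewolf enemy's Phase 1 second attack, a montage combo of up to two swings.
; A combo event received on the avatar during the first montage sets a flag that triggers the second montage on completion; otherwise the ability ends.
; Per-montage sound events apply the same Attack1 sound GameplayEffect to self.
; Ending the ability stops the combo listener and resets the flag.
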(event Ability|EventActivateAbility
  (|PlayMontageandWaitProxy "None" "/Game/Characters/Enemy/EnemyWerewolf/Animation/PhaseOne/Attack/AM_Attack2_1.AM_Attack2_1" 1.0 "None" true 1.0 0.0 false
    (:then
      (bind _asynctaskproxy (Ability|Tasks|WaitGameplayEvent "(TagName=\"GameplayCue.Sound.Enemy.Werewolf.Phase1.Attack2_1\")" 0)
        (:then
          (bind _asynctaskproxy_2 (Ability|Async|WaitGameplayEventToActor (Ability|GetAvatarActorfromActorInfo) "(TagName=\"Enemy.Attack.Combo2\")")
            (:then
              (Variables|Default|SetNextCombo%20Async%20Action _asynctaskproxy_2))
            (:EventReceived
              (Variables|Default|SetbNextCombo true))))
        (:EventReceived
          (Class|GASAbilitySystemLibrary|ApplyGASEffecttoSelftoASC (Ability|GetAbilitySystemComponentfromActorInfo) "/Game/Characters/Enemy/EnemyWerewolf/GAS/Effect/Phase1/SoundGE/GE_WerewolfPlayPhase1Attack1Sound1.GE_WerewolfPlayPhase1Attack1Sound1_C" 1.0)
          (GameplayTasks|EndTask _asynctaskproxy))))
    (:OnCompleted
      (if (Variables|Default|GetbNextCombo)
        (|PlayMontageandWaitProxy "None" "/Game/Characters/Enemy/EnemyWerewolf/Animation/PhaseOne/Attack/AM_Attack2_2.AM_Attack2_2" 1.0 "None" true 1.0 0.0 false
          (:then
            (bind _asynctaskproxy_3 (Ability|Tasks|WaitGameplayEvent "(TagName=\"GameplayCue.Sound.Enemy.Werewolf.Phase1.Attack2_2\")" 0)
              (:EventReceived
                (Class|GASAbilitySystemLibrary|ApplyGASEffecttoSelftoASC (Ability|GetAbilitySystemComponentfromActorInfo) "/Game/Characters/Enemy/EnemyWerewolf/GAS/Effect/Phase1/SoundGE/GE_WerewolfPlayPhase1Attack1Sound1.GE_WerewolfPlayPhase1Attack1Sound1_C" 1.0)
                (GameplayTasks|EndTask _asynctaskproxy_3))))
          (:OnCompleted
            (Ability|EndAbility :!label _label))
          (:OnBlendOut
            (goto _label))
          (:OnInterrupted
            (goto _label))
          (:OnCancelled
            (goto _label)))
        (else
          (Ability|EndAbility))))))

(event Ability|EventOnEndAbility
  (params (bWasCancelled :type Boolean))
  (Ability|Async|EndAction (Variables|Default|GetNextCombo%20Async%20Action))
  (Variables|Default|SetbNextCombo false))