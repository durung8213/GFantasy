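; Werewolf boss ability for phase 1 pattern 1: a paired stab execution on the AI's focused player.
; It snaps the player in front of the boss, blends their view to the boss's repositioned camera, and forces a temporarily granted ability on them.
; Montage-timed gameplay events apply slash sound and kill effects.
; A TargetAlive event from the player blocks the kill, clears focus and ends the ability after a delay.
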(event Ability|EventActivateAbility
  (bind _returnvalue (Ability|GetAvatarActorfromActorInfo))
  (bind _returnvalue_2 (Class|GAEndDelegateBase|GetCurrentController))
  (bind _returnvalue_3 (Ability|GetAvatarActorfromActorInfo))
  (bind _returnvalue_4 (Class|AIController|GetFocusActor _returnvalue_2))
  (bind _returnvalue_5 (AI|GetAIController _returnvalue_3))
  (bind _returnvalue_6 (Ability|GetAbilitySystemComponent _returnvalue_4))
  (Utilities|FlowControl|Sequence
    (:then_0
      ;[1 1 1] 카메라를 페이즈 1 패턴 1에 맞게 회전
      (bind _asbp_boss_werewolf (Utilities|Casting|CastToBP_BossWerewolf (Ability|GetAvatarActorfromActorInfo)))
      (Default|MultiSetCameraRelativeLocationandRotation _asbp_boss_werewolf "70.000000,-8.500000,106.600000" "0.000000,130.000000,0.000000"))
    (:then_1
      ;[1 1 1] 타겟 플레이어 액터 및 어빌리티 컴포넌트 가져오기
      (Utilities|IsValid _returnvalue_4
        (:Is%20Valid
          (Variables|Default|SetOtherActor _returnvalue_4)
          (Utilities|IsValid _returnvalue_6
            (:Is%20Valid
              (Variables|Default|SetOtherActorAbilityComponent _returnvalue_6))))))
    (:then_2
      ;[1 1 1] 풀래아어가 회피를 했다면
      (bind _asynctaskproxy (Ability|Async|WaitGameplayEventToActor (Variables|Default|GetOtherActor) "(TagName=\"Combat.Pattern1.End.TargetAlive\")")
        (:then
          (Variables|Default|SetPlayer%20Alive%20Async%20Action _asynctaskproxy))
        (:EventReceived
          (Utilities|IsValid _returnvalue_5
            (:Is%20Valid
              (AI|ClearFocus _returnvalue_5))
            (:Is%20Not%20Valid
              _))
          (Variables|Default|SetbIsPlayerParry true)
          (Ability|Tasks|WaitDelay 2.0
            (:OnFinish
              (Ability|EndAbility))))))
    (:then_3
      ;[1 1 1] 타겟이 된 플레이어 강제 위치 조정 및 회전
      (bind _asboss_were_wolf_character (Utilities|Casting|CastToBossWereWolfCharacter (Ability|GetAvatarActorfromActorInfo)))
      (Class|BossWereWolfCharacter|MultiRotateActor _asboss_were_wolf_character (Variables|Default|GetOtherActor) (Math|Rotator|MakeRotator 0.0 0.0 (.yaw (Math|Rotator|MakeRotfromX (- (Transformation|GetActorLocation (Ability|GetAvatarActorfromActorInfo)) (Transformation|GetActorLocation (Variables|Default|GetOtherActor)))))))
      (Class|BossWereWolfCharacter|MultiSetLocationActor _asboss_were_wolf_character (Variables|Default|GetOtherActor) (+ (* (Transformation|GetActorForwardVector _returnvalue) "220.000000,220.000000,220.000000") (Transformation|GetActorLocation _returnvalue))))
    (:then_4
      ;[1 1 1] 타겟 플레이어게 강제로 어빌리티를 부여하고 실행 시킴
      (Class|GAEndDelegateBase|ApplyEffecttoTarget (Ability|GetAbilitySystemComponentfromActorInfo) (Variables|Default|GetOtherActorAbilityComponent) "/Game/Characters/Enemy/EnemyWerewolf/GAS/Effect/Phase1/Pattern/GE_GiveTempAbiliy.GE_GiveTempAbiliy_C")
      (Abilities|TryActivateAbilitiesbyTag (Variables|Default|GetOtherActorAbilityComponent) (Variables|Default|GetGameplay%20Tag%20Container) true))
    (:then_5
      ;[1 1 1] 찌르기 몽타주 재생 및 플레이어 타격 및 칼 휘두르는 사운드 재생
      (|PlayMontageandWaitProxy "None" "/Game/Characters/Enemy/EnemyWerewolf/Animation/PhaseOne/Pattern/AM_Paired_1HM_StabStomach_Att.AM_Paired_1HM_StabStomach_Att" 1.0 "None" true 1.0 0.0 false
        (:then
          (bind _asynctaskproxy_2 (Ability|Tasks|WaitGameplayEvent "(TagName=\"Enemy.Attack.Combo3\")" 0)
            (:then
              (Variables|Default|SetAttack%20Player%20Async%20Task _asynctaskproxy_2)
              (bind _asynctaskproxy_3 (Ability|Tasks|WaitGameplayEvent "(TagName=\"GameplayCue.Sound.Enemy.Werewolf.Phase1.Pattern1Hit\")" 0)
                (:then
                  (Variables|Default|SetAttack%20Sound%20Async%20Task _asynctaskproxy_3))
                (:EventReceived
                  (Class|GAEndDelegateBase|ApplyEffecttoTarget (Ability|GetAbilitySystemComponentfromActorInfo) (Variables|Default|GetOtherActorAbilityComponent) "/Game/Characters/Enemy/EnemyWerewolf/GAS/Effect/Phase1/SoundGE/GE_WerewolfPlayPhase1Pattern1SlashSound.GE_WerewolfPlayPhase1Pattern1SlashSound_C"))))
            (:EventReceived
              (if (not (Variables|Default|GetbIsPlayerParry))
                (Class|GAEndDelegateBase|ApplyEffecttoTarget (Ability|GetAbilitySystemComponentfromActorInfo) (Variables|Default|GetOtherActorAbilityComponent) "/Game/Characters/Enemy/GAS/Effect/GE_Kill.GE_Kill_C")))))
        (:OnCompleted
          (Ability|EndAbility))))
    (:then_6
      ;[1 1 1] 플레이어 카메라 변경
      (bind _as캐릭터 (Utilities|Casting|CastToCharacter (Variables|Default|GetOtherActor)))
      (bind _as플레이어_컨트롤러 (Utilities|Casting|CastToPlayerController (Pawn|GetController _as캐릭터)))
      (Game|Player|SetViewTargetwithBlend _as플레이어_컨트롤러 (Ability|GetAvatarActorfromActorInfo) 0.1 "VTBlend_Linear" 0.0 false))))

(event Ability|EventOnEndAbility
  (params (bWasCancelled :type Boolean))
  (bind _attack_player_async_task (Variables|Default|GetAttack%20Player%20Async%20Task))
  (bind _attack_sound_async_task (Variables|Default|GetAttack%20Sound%20Async%20Task))
  (bind _player_alive_async_action (Variables|Default|GetPlayer%20Alive%20Async%20Action))
  (Utilities|FlowControl|Sequence
    (:then_0
      (Utilities|IsValid _attack_player_async_task
        (:Is%20Valid
          (GameplayTasks|EndTask _attack_player_async_task))))
    (:then_1
      (Utilities|IsValid _attack_sound_async_task
        (:Is%20Valid
          (GameplayTasks|EndTask _attack_sound_async_task))))
    (:then_2
      (Utilities|IsValid _player_alive_async_action
        (:Is%20Valid
          (Ability|Async|EndAction _player_alive_async_action))))
    (:then_3
      (Variables|Default|SetbIsPlayerParry false))))