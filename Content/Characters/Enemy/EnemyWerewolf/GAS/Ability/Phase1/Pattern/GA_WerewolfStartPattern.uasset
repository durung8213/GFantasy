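; Gameplay ability that plays the werewolf boss's buff montage to start a Phase 1 attack pattern.
; A gameplay event, awaited during the montage, applies the start-sound effect to itself and calls MultiActivePowerUp on BP_BossWerewolf.
; Montage completion ends the ability, and OnEndAbility calls MultiDeactivePowerUp to switch the power-up off.
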(event Ability|EventActivateAbility
  (|PlayMontageandWaitProxy "None" "/Game/Characters/Enemy/EnemyWerewolf/Animation/PhaseOne/Pattern/AM_A_buff_01.AM_A_buff_01" 1.0 "None" true 1.0 0.0 false
    (:then
      (bind _asynctaskproxy (Ability|Tasks|WaitGameplayEvent "(TagName=\"GameplayCue.Sound.Enemy.Werewolf.Phase1.Pattern1Start\")" 0)
        (:EventReceived
          (Class|GASAbilitySystemLibrary|ApplyGASEffecttoSelftoASC (Ability|GetAbilitySystemComponentfromActorInfo) "/Game/Characters/Enemy/EnemyWerewolf/GAS/Effect/Phase1/SoundGE/GE_WerewolfPlayPhase1Pattern1StartSound.GE_WerewolfPlayPhase1Pattern1StartSound_C" 1.0)
          (bind _asbp_boss_werewolf (Utilities|Casting|CastToBP_BossWerewolf (Ability|GetAvatarActorfromActorInfo))
            (:then
              (bind _output_get (Variables|Default|SetAs%20BP%20Boss%20Werewolf _asbp_boss_werewolf))
              (Default|MultiActivePowerUp _asbp_boss_werewolf))
            (:CastFailed
              _))
          (GameplayTasks|EndTask _asynctaskproxy))))
    (:OnCompleted
      (Ability|EndAbility))))

(event Ability|EventOnEndAbility
  (params (bWasCancelled :type Boolean))
  (Default|MultiDeactivePowerUp (Variables|Default|GetAs%20BP%20Boss%20Werewolf)))