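; Player-side gameplay ability for the werewolf's phase 1 pattern hit, playing a paired stab-victim montage with combat blocked.
; Gameplay events drive it: State.Parry lifts the block and starts a timer-drained defense progress bar, while State.Ability.Blocked restores the block and marks the player hit.
; A strong hit-react event restores the camera.
; Ending cleans up effects, tasks, UI and camera, sending a target-alive event if the player was not hit.
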(event Custom|ToZeroTimer
  ;[1 1 1] 방어 타이밍 발동
  (Variables|Default|SetElapsedTime (+ (Variables|Default|GetElapsedTime) 0.03))
  (Class|GASWorldPlayerController|ClientSetWerewolfPattern1ProgressbarPercent (Variables|Default|GetAs%20BP%20GASWorld%20Player%20Controller) (Math|Float|Lerp 1.0 0.0 (/ (Variables|Default|GetElapsedTime) 0.5))))

(event Ability|EventActivateAbility
  (bind _returnvalue (Ability|GetAvatarActorfromActorInfo))
  (Class|GASAbilitySystemLibrary|ApplyGASEffecttoSelftoASC (Ability|GetAbilitySystemComponentfromActorInfo) "/Game/Characters/Enemy/EnemyWerewolf/GAS/Effect/Phase1/Pattern/GE_BlockPlayerCombat.GE_BlockPlayerCombat_C" 1.0)
  (|PlayMontageandWaitProxy "None" "/Game/Characters/Enemy/EnemyWerewolf/Animation/PhaseOne/Pattern/AM_Paired_1HM_StabStomach_Vic1.AM_Paired_1HM_StabStomach_Vic1" 1.0 "None" true 1.0 0.0 false
    (:then
      (Utilities|FlowControl|Sequence
        (:then_0
          ;[1 1 1] 회피 막기
          (bind _asynctaskproxy (Ability|Tasks|WaitGameplayEvent "(TagName=\"State.Ability.Blocked\")" 0)
            (:then
              (Variables|Default|SetBlockCombatTask _asynctaskproxy))
            (:EventReceived
              (Class|GASAbilitySystemLibrary|ApplyGASEffecttoSelftoASC (Ability|GetAbilitySystemComponentfromActorInfo) "/Game/Characters/Enemy/EnemyWerewolf/GAS/Effect/Phase1/Pattern/GE_BlockPlayerCombat.GE_BlockPlayerCombat_C" 1.0)
              (Utilities|FlowControl|Sequence
                (:then_0
                  (if (Utilities|Time|IsValidTimerHandle (Variables|Default|GetProgressbarTimerHnadle))
                    (Utilities|Time|ClearandInvalidateTimerbyHandle (Variables|Default|GetProgressbarTimerHnadle))))
                (:then_1
                  (Utilities|IsValid (Variables|Default|GetAs%20BP%20GASWorld%20Player%20Controller)
                    (:Is%20Valid
                      (Class|GASWorldPlayerController|ClientHideWerewolfPattern1Progressbar (Variables|Default|GetAs%20BP%20GASWorld%20Player%20Controller)))))
                (:then_2
                  (Variables|Default|SetbIsPlayerHit true))))))
        (:then_1
          ;[1 1 1] 방어 타이밍 발동
          (Ability|Tasks|WaitGameplayEvent "(TagName=\"State.Parry\")" 0
            (:EventReceived
              (GameplayEffects|RemoveActiveGameplayEffectbySourceEffect (Ability|GetAbilitySystemComponentfromActorInfo) "/Game/Characters/Enemy/EnemyWerewolf/GAS/Effect/Phase1/Pattern/GE_BlockPlayerCombat.GE_BlockPlayerCombat_C" 0 -1)
              (bind _as캐릭터 (Utilities|Casting|CastToCharacter (Ability|GetAvatarActorfromActorInfo)))
              (bind _asbp_gasworld_player_controller (Utilities|Casting|CastToBP_GASWorldPlayerController (Pawn|GetController _as캐릭터)))
              (bind _output_get (Variables|Default|SetAs%20BP%20GASWorld%20Player%20Controller _asbp_gasworld_player_controller))
              (Class|GASWorldPlayerController|ClientShowWerewolfPattern1Progressbar _output_get)
              (bind _returnvalue_2 (Utilities|Time|SetTimerbyEvent (delegate Custom|ToZeroTimer) 0.03 true))
              (Variables|Default|SetProgressbarTimerHnadle _returnvalue_2))))
        (:then_2
          ;[1 1 1] 칼빵 맞는 소리 내기
          (bind _asynctaskproxy_2 (Ability|Tasks|WaitGameplayEvent "(TagName=\"GameplayCue.Sound.Enemy.Werewolf.Phase1.Pattern1Hit\")" 0)
            (:then
              (Variables|Default|SetPatternHitTask _asynctaskproxy_2))))
        (:then_3
          ;[1 1 1] 플레이어 카메라 원래대로 돌리기
          (bind _asynctaskproxy_3 (Ability|Tasks|WaitGameplayEvent "(TagName=\"Ability.HitReact.Strong\")" 0)
            (:then
              (Variables|Default|SetChangeCameraTask _asynctaskproxy_3))
            (:EventReceived
              (bind _as캐릭터_2 (Utilities|Casting|CastToCharacter _returnvalue))
              (bind _as플레이어_컨트롤러 (Utilities|Casting|CastToPlayerController (Pawn|GetController _as캐릭터_2)))
              (Game|Player|SetViewTargetwithBlend _as플레이어_컨트롤러 _returnvalue 0.1 "VTBlend_Linear" 0.0 false)
              (Variables|Default|SetbCameraRestore true))))))
    (:OnCompleted
      (Ability|EndAbility :!label _label))
    (:OnBlendOut
      (goto _label))
    (:OnInterrupted
      (goto _label))
    (:OnCancelled
      (goto _label))))

(event Ability|EventOnEndAbility
  (params (bWasCancelled :type Boolean))
  (bind _returnvalue (Ability|GetAvatarActorfromActorInfo))
  (bind _blockcombattask (Variables|Default|GetBlockCombatTask))
  (bind _patternhittask (Variables|Default|GetPatternHitTask))
  (bind _as_bp_gasworld_player_controller (Variables|Default|GetAs%20BP%20GASWorld%20Player%20Controller))
  (Utilities|FlowControl|Sequence
    (:then_0
      (GameplayEffects|RemoveActiveGameplayEffectbySourceEffect (Ability|GetAbilitySystemComponentfromActorInfo) "/Game/Characters/Enemy/EnemyWerewolf/GAS/Effect/Phase1/Pattern/GE_GiveTempAbiliy.GE_GiveTempAbiliy_C" 0 -1))
    (:then_1
      (if (not (Variables|Default|GetbCameraRestore))
        (bind _as캐릭터 (Utilities|Casting|CastToCharacter _returnvalue))
        (bind _as플레이어_컨트롤러 (Utilities|Casting|CastToPlayerController (Pawn|GetController _as캐릭터)))
        (Game|Player|SetViewTargetwithBlend _as플레이어_컨트롤러 _returnvalue 0.1 "VTBlend_Linear" 0.0 false)))
    (:then_2
      (GameplayEffects|RemoveActiveGameplayEffectbySourceEffect (Ability|GetAbilitySystemComponentfromActorInfo) "/Game/Characters/Enemy/EnemyWerewolf/GAS/Effect/Phase1/Pattern/GE_BlockPlayerCombat.GE_BlockPlayerCombat_C" 0 -1))
    (:then_3
      (Utilities|IsValid _blockcombattask
        (:Is%20Valid
          (GameplayTasks|EndTask _blockcombattask))))
    (:then_4
      (Utilities|IsValid _patternhittask
        (:Is%20Valid
          (GameplayTasks|EndTask _patternhittask))))
    (:then_5
      (Variables|Default|SetbCameraRestore false)
      (Variables|Default|SetElapsedTime 0.0)
      (if (Utilities|Time|IsValidTimerHandle (Variables|Default|GetProgressbarTimerHnadle))
        (Utilities|Time|ClearandInvalidateTimerbyHandle (Variables|Default|GetProgressbarTimerHnadle))))
    (:then_6
      (Utilities|IsValid _as_bp_gasworld_player_controller
        (:Is%20Valid
          (Class|GASWorldPlayerController|ClientHideWerewolfPattern1Progressbar _as_bp_gasworld_player_controller))))
    (:then_7
      (if (not (Variables|Default|GetbIsPlayerHit))
        (Ability|SendGameplayEventtoActor (Ability|GetAvatarActorfromActorInfo) "(TagName=\"Combat.Pattern1.End.TargetAlive\")")))))