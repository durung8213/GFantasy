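; Base AI controller for werewolf enemies, handling boss hit reactions and cinematic requests.
; The normal and strong attack hit events each apply their matching groggy Gameplay Effect to the controlled pawn through its Ability System Component, then print the pawn's name as debug output.
; PlaySequence forwards a Level Sequence to the given player's BP_GASWorldPlayerController for playback.
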(event EventBeginPlay)

(event EventTick
  (params (DeltaSeconds :type Float%20%28single-precision%29)))

(event EventBossHitNormalAttack
  (params (EffectSpec :type Gameplay%20Effect%20Spec%20Structure%20%28by%20ref%29) (EvaluatedData :type Gameplay%20Modifier%20Evaluated%20Data%20Structure%20%28by%20ref%29) (Target :type Ability%20System%20Component%20Object%20Reference))
  (bind _returnvalue (Pawn|GetControlledPawn))
  (GameplayEffects|ApplyGameplayEffectToSelf :self (Ability|GetAbilitySystemComponent (Pawn|GetControlledPawn)) :GameplayEffectClass "/Game/Characters/Enemy/EnemyWerewolf/GAS/Effect/Phase1/Groggy/GE_NormalAttackGroggy.GE_NormalAttackGroggy_C" :Level 1.0)
  (Utilities|IsValid _returnvalue
    (:Is%20Valid
      (Development|PrintString (Utilities|GetDisplayName _returnvalue) true true "(R=0.030625,G=1.000000,B=0.000000,A=1.000000)" 1e+01))))

(event EventBossHitStrongAttack
  (params (EffectSpec :type Gameplay%20Effect%20Spec%20Structure%20%28by%20ref%29) (EvaluatedData :type Gameplay%20Modifier%20Evaluated%20Data%20Structure%20%28by%20ref%29) (Target :type Ability%20System%20Component%20Object%20Reference))
  (bind _returnvalue (Pawn|GetControlledPawn))
  (GameplayEffects|ApplyGameplayEffectToSelf :self (Ability|GetAbilitySystemComponent (Pawn|GetControlledPawn)) :GameplayEffectClass "/Game/Characters/Enemy/EnemyWerewolf/GAS/Effect/Phase1/Groggy/GE_StrongAttackGroggy.GE_StrongAttackGroggy_C" :Level 1.0)
  (Utilities|IsValid _returnvalue
    (:Is%20Valid
      (Development|PrintString (Utilities|GetDisplayName _returnvalue) true true "(R=0.030625,G=1.000000,B=0.000000,A=1.000000)" 1e+01))))

(event EventPlaySequence
  (params (Player :type GAS%20Player%20Character%20Object%20Reference) (LevelSequence :type Level%20Sequence%20Object%20Reference))
  (bind _asbp_gasworld_player_controller (Utilities|Casting|CastToBP_GASWorldPlayerController (Pawn|GetController Player)))
  (Default|PlaySequence _asbp_gasworld_player_controller LevelSequence))

(fn ConstructionScript)