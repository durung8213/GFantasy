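; AI controller for the Succubus boss that handles its groggy reactions and triggers cinematic playback.
; Normal and strong hit events apply the matching groggy GameplayEffect to the controlled pawn's Ability System Component.
; PlaySequence casts the given player's controller to BP_GASWorldPlayerController and forwards a Level Sequence to it.
; BeginPlay, Tick and the construction script are empty.
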(event EventBeginPlay)

(event EventTick
  (params (DeltaSeconds :type Float%20%28single-precision%29)))

(event EventBossHitNormalAttack
  (params (EffectSpec :type Gameplay%20Effect%20Spec%20Structure%20%28by%20ref%29) (EvaluatedData :type Gameplay%20Modifier%20Evaluated%20Data%20Structure%20%28by%20ref%29) (Target :type Ability%20System%20Component%20Object%20Reference))
  (GameplayEffects|ApplyGameplayEffectToSelf :self (Ability|GetAbilitySystemComponent (Pawn|GetControlledPawn)) :GameplayEffectClass "/Game/Characters/Enemy/EnemySuccubus/GAS/Effect/Groggy/GE_SuccubusNormalAttackGroggy.GE_SuccubusNormalAttackGroggy_C" :Level 1.0))

(event EventBossHitStrongAttack
  (params (EffectSpec :type Gameplay%20Effect%20Spec%20Structure%20%28by%20ref%29) (EvaluatedData :type Gameplay%20Modifier%20Evaluated%20Data%20Structure%20%28by%20ref%29) (Target :type Ability%20System%20Component%20Object%20Reference))
  (GameplayEffects|ApplyGameplayEffectToSelf :self (Ability|GetAbilitySystemComponent (Pawn|GetControlledPawn)) :GameplayEffectClass "/Game/Characters/Enemy/EnemySuccubus/GAS/Effect/Groggy/GE_SuccubusStrongAttackGroggy.GE_SuccubusStrongAttackGroggy_C" :Level 1.0))

(event EventPlaySequence
  (params (Player :type GAS%20Player%20Character%20Object%20Reference) (LevelSequence :type Level%20Sequence%20Object%20Reference))
  (bind _asbp_gasworld_player_controller (Utilities|Casting|CastToBP_GASWorldPlayerController (Pawn|GetController Player)))
  (Default|PlaySequence _asbp_gasworld_player_controller LevelSequence))

(fn ConstructionScript)