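; Phase 2 death gameplay ability for the Succubus boss, handling its death and loot.
; It applies GE_Dead, plays the death montage and waits for a Combat.Dead.Dead event to call OnDieMessage.
; It then gives the boss's passive pickup items to each player in the AI controller's area list.
; It also spawns DarkKnightSoul drops at the boss, with a random count scaled by player count.
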(event Ability|EventActivateAbility
  (bind _returnvalue (Ability|GetAvatarActorfromActorInfo))
  (Ability|ApplyGameplayEffectToOwner "/Game/BluePrints/GAS/GameplayEffect/Enemy/GE_Dead.GE_Dead_C")
  (|PlayMontageandWaitProxy "None" "/Game/Characters/Enemy/EnemySuccubus/Anim/Phase2/AM_death.AM_death" 1.0 "None" true 1.0 0.0 false
    (:then
      (Ability|Tasks|WaitGameplayEvent "(TagName=\"Combat.Dead.Dead\")" 0
        (:EventReceived
          (Class|EnemyInterface|OnDie(Message) (Ability|GetAvatarActorfromActorInfo))
          (bind _asgascombat_boss_npc (Utilities|Casting|CastToGASCombatBossNPC _returnvalue))
          (bind _asboss_aicontroller_base (Utilities|Casting|CastToBossAIControllerBase (Pawn|GetController _asgascombat_boss_npc)))
          (Utilities|FlowControl|Sequence
            (:then_0
              (for _array_element (Variables|/Script/GFantasy.BossAIControllerBase|GetInAreaPlayerArr _asboss_aicontroller_base)
                (bind _asbp_gasworld_player_controller (Utilities|Casting|CastToBP_GASWorldPlayerController (Pawn|GetController (Utilities|Struct|BreakInArrayPlayer _array_element))))
                (for _array_element_2 (Variables|/Script/GFantasy.GASCombatBossNPC|GetPassivePickupItemArr _asgascombat_boss_npc)
                  (Class|InventoryComponent|AddItem (Variables|/Script/GFantasy.GASWorldPlayerController|GetInventoryComponent _asbp_gasworld_player_controller) _array_element_2 1))))
            (:then_1
              (for _index (range (* (Utilities|Array|Length (Variables|/Script/GFantasy.BossAIControllerBase|GetInAreaPlayerArr _asboss_aicontroller_base)) 2) (* (Utilities|Array|Length (Variables|/Script/GFantasy.BossAIControllerBase|GetInAreaPlayerArr _asboss_aicontroller_base)) (Math|Random|RandomIntegerinRange 0 4)))
                (|SpawnActor 0 (Transformation|GetActorLocation _returnvalue) "0, 0, 0" "/Game/BluePrints/Actor/Item/BP_ItemSpawn.BP_ItemSpawn_C" false true "0.000000,0.000000,600.000000" "(TagName=\"Item.Material.Drop.DarkKnightSoul\")" 0)))))))))

(event Ability|EventOnEndAbility
  (params (bWasCancelled :type Boolean)))