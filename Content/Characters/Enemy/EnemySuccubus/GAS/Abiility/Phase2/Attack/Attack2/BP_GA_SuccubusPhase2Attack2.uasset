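; Gameplay ability for the Succubus enemy's second phase-2 attack, which launches a sickle aura projectile.
; It plays two montages in sequence, ending when the second completes.
; During the attack it listens for the Spawn.Skill.Projectile gameplay event and spawns the aura on authority, lowered below the avatar's origin, moving along its forward vector and carrying the boss's ability system component.
; The stored event task is ended with the ability.
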(event Ability|EventActivateAbility
  (bind _returnvalue (Ability|GetAvatarActorfromActorInfo))
  (bind _returnvalue_2 (Class|GASuccubusPhase2Attack2|GetSickleAuraSpawnLocation 5e+01))
  (bind _returnvalue_3 (Transformation|GetActorForwardVector _returnvalue))
  (|PlayMontageandWaitProxy "None" "/Game/Characters/Enemy/EnemySuccubus/Anim/Phase2/Attack/Attack2/AM_Attack2_1.AM_Attack2_1" 1.0 "None" true 1.0 0.0 false
    (:then
      (bind _asynctaskproxy (Ability|Tasks|WaitGameplayEvent "(TagName=\"Spawn.Skill.Projectile\")" 0)
        (:then
          (Variables|Default|SetSpawn%20Async%20Task _asynctaskproxy))
        (:EventReceived
          (|SpawnActor 0 (Math|Vector|MakeVector (.x _returnvalue_2) (.y _returnvalue_2) (- (.z (Transformation|GetActorLocation (Ability|GetAvatarActorfromActorInfo))) 8e+01)) (Math|Conversions|RotationFromXVector (Math|Vector|Normalize _returnvalue_3)) "/Game/Characters/Enemy/EnemySuccubus/GAS/Abiility/Phase2/Attack/Attack2/BP_SuccubusSickleAuraActor.BP_SuccubusSickleAuraActor_C" true (* _returnvalue_3 "2500.000000,2500.000000,2500.000000") (Ability|GetAbilitySystemComponentfromActorInfo) 0))))
    (:OnCompleted
      (|PlayMontageandWaitProxy "None" "/Game/Characters/Enemy/EnemySuccubus/Anim/Phase2/Attack/Attack2/AM_Attack2_2.AM_Attack2_2" 1.0 "None" true 1.0 0.0 false
        (:OnCompleted
          (Ability|EndAbility))))))

(event Ability|EventOnEndAbility
  (params (bWasCancelled :type Boolean))
  (GameplayTasks|EndTask (Variables|Default|GetSpawn%20Async%20Task)))