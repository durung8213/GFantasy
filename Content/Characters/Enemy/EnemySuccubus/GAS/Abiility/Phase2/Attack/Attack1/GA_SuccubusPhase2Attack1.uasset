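; Gameplay ability for the Succubus enemy's first Phase 2 attack.
; On activation it plays the AM_Attack1 montage and ends the ability when the montage completes.
; An unconnected dash variant remains: a looping timer would lerp the avatar along a float curve toward the AI focus actor's captured location, alongside a dash montage, but nothing runs it.
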(event Custom|Dash
  (bind _output_get (Variables|Default|SetElapsedTime (+ (Variables|Default|GetElapsedTime) 0.03)))
  (Transformation|SetActorLocation (Ability|GetAvatarActorfromActorInfo) (Math|Vector|Lerp(Vector) (Variables|Default|GetStartLocation) (Variables|Default|GetTargetLocation) (Math|Curves|GetFloatValue (Variables|Default|GetCurveFloat) _output_get)) false false)
  (if (>= (Variables|Default|GetElapsedTime) (.MaxTime (Math|Curves|GetTimeRange (Variables|Default|GetCurveFloat))))
    (Utilities|Time|ClearandInvalidateTimerbyHandle (Variables|Default|GetDashTimerHandle))))

(event Ability|EventActivateAbility
  (|PlayMontageandWaitProxy "None" "/Game/Characters/Enemy/EnemySuccubus/Anim/Phase2/Attack/Attack1/AM_Attack1.AM_Attack1" 1.0 "None" true 1.0 0.0 false
    (:OnCompleted
      (Ability|EndAbility))))

(event Ability|EventOnEndAbility
  (params (bWasCancelled :type Boolean)))