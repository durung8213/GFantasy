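; Gameplay ability for the Succubus boss's second Phase 2 attack, a flying slash that fires a projectile.
; It plays the attack montage at half speed and listens for a Spawn.Skill.Projectile gameplay event.
; Each event spawns an authority-only slash projectile at the weapon socket, aimed from the boss toward slightly below the AI focus actor.
; The ability ends when the montage completes, and ending it stops the event listener.
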(event Ability|EventActivateAbility
  (bind _returnvalue (Ability|GetAvatarActorfromActorInfo))
  (|PlayMontageandWaitProxy "None" "/Game/Characters/Enemy/EnemySuccubus/Anim/Phase2/Attack/Attack2/AM_Flying_attack13.AM_Flying_attack13" 0.5 "None" true 1.0 0.0 false
    (:then
      (bind _asynctaskproxy (Ability|Tasks|WaitGameplayEvent "(TagName=\"Spawn.Skill.Projectile\")" 0)
        (:then
          (Variables|Default|SetSpawn%20Async%20Task _asynctaskproxy))
        (:EventReceived
          (bind _asbp_boss_succubus (Utilities|Casting|CastToBP_BossSuccubus _returnvalue))
          (bind _returnvalue_2 (Class|GASCombatNPC|GetWeapon _asbp_boss_succubus))
          (bind _asbp_succubus_weapon (Utilities|Casting|CastToBP_SuccubusWeapon _returnvalue_2))
          (|SpawnActor 0 (Transformation|GetSocketLocation (Variables|/Script/GFantasy.BaseStaticMeshWeapon|GetWeaponMesh _asbp_succubus_weapon) "ProjectileSpawnPoint") "0, 0, 0" "/Game/BluePrints/Actor/Projectile/BossSuccubus/BP_SuccubusSlash1.BP_SuccubusSlash1_C" true (Math|Vector|Normalize (- (+ (Transformation|GetActorLocation (Class|AIController|GetFocusActor (AI|GetAIController _returnvalue))) (Math|Vector|MakeVector 0.0 0.0 -1e+02)) (Transformation|GetActorLocation _returnvalue))) 6e+03 6e+03 true false 0 0.0 (.AsGASCBase (Utilities|Casting|CastToGASCBase (Ability|GetAbilitySystemComponent _returnvalue))) 0))))
    (:OnCompleted
      (Ability|EndAbility))))

(event Ability|EventOnEndAbility
  (params (bWasCancelled :type Boolean))
  (GameplayTasks|EndTask (Variables|Default|GetSpawn%20Async%20Task)))