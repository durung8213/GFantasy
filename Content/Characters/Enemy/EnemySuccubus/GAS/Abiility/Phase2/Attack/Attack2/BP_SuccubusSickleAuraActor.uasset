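; Sickle aura projectile for the Succubus boss's phase 2 Attack2, which players can parry back at the boss.
; It flies at a preset velocity, handles box overlaps only on authority, and destroys itself after a timeout.
; A player in a combo attack redirects it along their forward vector, and it then applies a GAS effect only to the boss.
; Otherwise it applies the boss's effect to a non-dodging player and destroys itself.
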(event OnComponentBeginOverlap(Box)
  (params (OverlappedComponent :type Primitive%20Component%20Object%20Reference) (OtherActor :type Actor%20Object%20Reference) (OtherComp :type Primitive%20Component%20Object%20Reference) (OtherBodyIndex :type Integer) (bFromSweep :type Boolean) (SweepResult :type Hit%20Result%20Structure%20%28by%20ref%29))
  (Networking|SwitchHasAuthority
    (:Authority
      (if (Variables|SickleAura|GetbIsActive)
        (if (Variables|SickleAura|GetbIsPlayerParry)
          (bind _asbp_boss_succubus (Utilities|Casting|CastToBP_BossSuccubus OtherActor))
          (if (and (Utilities|IsValid (Variables|SickleAura|GetParryPlayerAbilitySystem)) (Utilities|IsValid (Ability|GetAbilitySystemComponent _asbp_boss_succubus)))
            (Class|GASAbilitySystemLibrary|ApplyGASEffecttoTargettoASC (Variables|SickleAura|GetParryPlayerAbilitySystem) (Ability|GetAbilitySystemComponent _asbp_boss_succubus) "/Game/Characters/Enemy/EnemySuccubus/GAS/Effect/Phase2/GE_SuccubusPhase2Attack2ToBoss.GE_SuccubusPhase2Attack2ToBoss_C" 1.0)
            (Variables|SickleAura|SetbIsActive false)
            (Actor|DestroyActor))
          (else
            (bind _asbp_gasplayer_character (Utilities|Casting|CastToBP_GASPlayerCharacter OtherActor))
            (CallFunction|PlayerHit _asbp_gasplayer_character)))))))

(event Custom|DestoryActor
  (Actor|DestroyActor))

(event EventBeginPlay
  (Variables|/Script/Engine.MovementComponent|SetVelocity (Variables|Default|GetProjectileMovement) (Variables|SickleAura|GetProjectileVelocity))
  (Utilities|Time|SetTimerbyEvent (delegate Custom|DestoryActor) 15.0))

(event Collision|EventActorBeginOverlap
  (params (OtherActor :type Actor%20Object%20Reference)))

(event EventTick
  (params (DeltaSeconds :type Float%20%28single-precision%29)))

(fn ConstructionScript)

(fn PlayerHit
  (params (HitPlayer :type BP%20GAS%20Player%20Character%20Object%20Reference))
  (bind _returnvalue (Ability|GetAbilitySystemComponent HitPlayer))
  (bind _returnvalue_2 (Transformation|GetActorForwardVector HitPlayer))
  (bind _returnvalue_3 (Math|Vector|Normalize _returnvalue_2))
  (if (GameplayTags|HasMatchingGameplayTag _returnvalue "(TagName=\"Ability.Attack.Combo\")")
    (Variables|SickleAura|SetParryPlayerAbilitySystem _returnvalue)
    (Utilities|IsValid HitPlayer
      (:Is%20Valid
        (Transformation|SetActorRotation (Math|Conversions|RotationFromXVector _returnvalue_3))
        (Variables|/Script/Engine.MovementComponent|SetVelocity (Variables|Default|GetProjectileMovement) (* _returnvalue_3 "2500.000000,2500.000000,2500.000000"))
        (Variables|SickleAura|SetbIsPlayerParry true)))
    (elif (not (GameplayTags|HasMatchingGameplayTag _returnvalue "(TagName=\"Ability.Dodge\")"))
      (Class|GASAbilitySystemLibrary|ApplyGASEffecttoTargettoASC (Variables|SickleAura|GetBossAbilitySystemComponent) _returnvalue "/Game/Characters/Enemy/EnemySuccubus/GAS/Effect/Phase2/GE_SuccubusPhase2Attack2ToPlayer.GE_SuccubusPhase2Attack2ToPlayer_C" 1.0)
      (Variables|SickleAura|SetbIsActive false)
      (Actor|DestroyActor))))