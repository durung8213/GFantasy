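; Gameplay ability for the succubus enemy's third phase 2 attack, placing a set of five attack decals on the ground.
; It plays a montage and waits for the Enemy.Attack.Combo3 gameplay event.
; On that event it line-traces down from each computed spawn location and spawns a decal actor on hits, authority-only, passing in its ability system component.
; The ability ends when the montage completes; an older forward-line trace loop remains unconnected.
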(event Ability|EventActivateAbility
  (|PlayMontageandWaitProxy "None" "/Game/Characters/Enemy/EnemySuccubus/Anim/Phase2/Attack/Attack3/AM_10_buff.AM_10_buff" 1.0 "None" true 1.0 0.0 false
    (:then
      (Ability|Tasks|WaitGameplayEvent "(TagName=\"Enemy.Attack.Combo3\")" 0
        (:EventReceived
          (for _index (range 0 4)
            (bind _returnvalue (Class|GASuccubusPhase2Attack3|GetAttackSpawnLocation _index))
            (bind (_outhit _returnvalue_2) (Collision|LineTraceForObjects _returnvalue (- _returnvalue "0.000000,0.000000,1000.000000") (Variables|Default|GetObject%20Types) false 0 "None"))
            (if _returnvalue_2
              (|SpawnActor 0 (.Location (Collision|BreakHitResult _outhit)) "0, 0, 0" "/Game/Characters/Enemy/EnemySuccubus/GAS/Abiility/Phase2/Attack/Attack3/BP_SuccubusAttack3Decal.BP_SuccubusAttack3Decal_C" true "(R=0.662745,G=0.000000,B=0.000000,A=1.000000)" 1.0 (Ability|GetAbilitySystemComponentfromActorInfo) 0
                (:Success
                  (Development|PrintString "소환 성공"))
                (:DidNotSpawn
                  (Development|PrintString "소환 실패"))))))))
    (:OnCompleted
      (Ability|EndAbility))))

(event Ability|EventOnEndAbility
  (params (bWasCancelled :type Boolean)))