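; Telegraphed ground-strike area for the Succubus phase 2 pattern 1 attack, drawn with two dynamic decal materials.
; A timeline animates the area fill, then fires the purple strike Niagara effect.
; On authority, a delayed looping timer repeatedly sphere-traces and applies a GAS effect to hit actors, destroying itself after a fixed hit count.
; Decal color updates through OnRep and multicast events; the trace radius is hardcoded, independent of decal Radius.
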(event Custom|MultiSetDecalColor
  (params (Value :type Linear%20Color%20Structure))
  (CallFunction|SetDecalColor Value))

(event Custom|ServerSetDecalColor
  (params (Value :type Linear%20Color%20Structure))
  (Variables|Default|SetColor Value))

(event Custom|Hit
  (bind _returnvalue (Transformation|GetActorLocation))
  (bind _outhits (Collision|MultiSphereTraceForObjects _returnvalue _returnvalue 2.6e+02 (Variables|Default|GetObject%20Types) false 0 "ForDuration"))
  (for _array_element _outhits
    (if (and (Utilities|IsValid (Variables|Decal|GetSource%20Ability%20System%20Component)) (Utilities|IsValid (Ability|GetAbilitySystemComponent (.HitActor (Collision|BreakHitResult _array_element)))))
      (Class|GASAbilitySystemLibrary|ApplyGASEffecttoTargettoASC (Variables|Decal|GetSource%20Ability%20System%20Component) (Ability|GetAbilitySystemComponent (.HitActor (Collision|BreakHitResult _array_element))) "/Game/Characters/Enemy/EnemySuccubus/GAS/Effect/Phase2/GE_SuccubusPhase2Pattern.GE_SuccubusPhase2Pattern_C" 1.0)))
  (bind _result (Math|Integer|IncrementInt (Variables|Default|GetHitCount))
    (:%20%20
      (if (>= _result 13)
        (Utilities|Time|ClearandInvalidateTimerbyHandle (Variables|Default|GetHitTimerHandle))
        (Actor|DestroyActor)))))

(event Custom|HitTimerStart
  (bind _returnvalue (Utilities|Time|SetTimerbyEvent (delegate Custom|Hit) 0.4 true))
  (Variables|Default|SetHitTimerHandle _returnvalue))

(event EventBeginPlay
  (Utilities|FlowControl|Sequence
    (:then_0
      (bind _returnvalue (Rendering|Material|CreateDynamicMaterialInstance (Variables|Default|GetCircum) :!class /Script/Engine.DecalComponent))
      (bind _output_get (Variables|Default|SetCircumRef _returnvalue))
      (Rendering|Material|SetScalarParameterValue _output_get "Circum1Area0" 0.0 :!class /Script/Engine.MaterialInstanceDynamic)
      (Rendering|Material|SetScalarParameterValue (Variables|Default|GetCircumRef) "AreaValue" 0.5 :!class /Script/Engine.MaterialInstanceDynamic))
    (:then_1
      (bind _returnvalue_2 (Rendering|Material|CreateDynamicMaterialInstance (Variables|Default|GetArea) :!class /Script/Engine.DecalComponent))
      (bind _output_get_2 (Variables|Default|SetAreaRef _returnvalue_2))
      (Rendering|Material|SetScalarParameterValue _output_get_2 "Circum1Area0" 0.0 :!class /Script/Engine.MaterialInstanceDynamic))
    (:then_2
      (CallFunction|SetDecalColor (Variables|Default|GetColor)))
    (:then_3
      (CallFunction|SetDecalRadius (Variables|Default|GetRadius)))
    (:then_4
      (bind _areavaluealpha (Timeline|AreaValueTimeline Play)
        (:Update
          (Utilities|IsValid (Variables|Default|GetAreaRef)
            (:Is%20Valid
              (Rendering|Material|SetScalarParameterValue (Variables|Default|GetAreaRef) "AreaValue" _areavaluealpha :!class /Script/Engine.MaterialInstanceDynamic))))
        (:Finished
          (Components|Activation|Activate (Variables|Default|GetNS_PurpleStrike) true)
          (Networking|SwitchHasAuthority
            (:Authority
              (Utilities|Time|SetTimerbyEvent (delegate Custom|HitTimerStart) 1.0))))))))

(fn ConstructionScript)

(fn OnRepValue0)

(fn SetDecalColor
  (params (Value :type Linear%20Color%20Structure))
  (bind _circumref (Variables|Default|GetCircumRef))
  (if (and (Utilities|IsValid _circumref) (Utilities|IsValid (Variables|Default|GetAreaRef)))
    (Rendering|Material|SetVectorParameterValue _circumref "DecalColor" Value :!class /Script/Engine.MaterialInstanceDynamic)))

(fn SetDecalRadius
  (params (Value :type Float%20%28single-precision%29))
  (Rendering|Material|SetScalarParameterValue (Variables|Default|GetCircumRef) "RadianValue" Value :!class /Script/Engine.MaterialInstanceDynamic))

(fn OnRepColor
  (CallFunction|SetDecalColor (Variables|Default|GetColor)))