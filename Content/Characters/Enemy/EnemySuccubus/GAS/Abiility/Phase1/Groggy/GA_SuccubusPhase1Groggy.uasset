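; Gameplay ability that plays the Succubus boss's phase 1 groggy start and puts the spotlight on it.
; On activation it points the view target of each player in the boss AI controller's area at the boss and plays the groggy start montage.
; The ability ends when the montage completes, or at once if the controller cast fails.
; On end it calls SetGroggy on the controller and returns each player's view to their own character.
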(event Ability|EventActivateAbility
  (Utilities|FlowControl|Sequence
    (:then_0
      (bind _asboss_aicontroller_base (Utilities|Casting|CastToBossAIControllerBase (AI|GetAIController (Ability|GetAvatarActorfromActorInfo)))
        (:then
          (bind _output_get (Variables|Default|SetAs%20Boss%20AIController%20Base _asboss_aicontroller_base))
          (bind _output_get_2 (Variables|Default|SetIn%20Area%20Player%20Arr (Variables|/Script/GFantasy.BossAIControllerBase|GetInAreaPlayerArr _output_get)))
          (for _array_element _output_get_2
            (bind _as플레이어_컨트롤러 (Utilities|Casting|CastToPlayerController (Pawn|GetController (Utilities|Struct|BreakInArrayPlayer _array_element))))
            (Game|Player|SetViewTargetwithBlend _as플레이어_컨트롤러 (Ability|GetAvatarActorfromActorInfo) 0.0 "VTBlend_Linear" 0.0 false)))
        (:CastFailed
          (Ability|EndAbility))))
    (:then_1
      (|PlayMontageandWaitProxy "None" "/Game/Characters/Enemy/EnemySuccubus/Anim/Phase1/Groggy/AM_GroggyStart.AM_GroggyStart" 0.9 "None" true 1.0 0.0 false
        (:OnCompleted
          (Ability|EndAbility))))))

(event Ability|EventOnEndAbility
  (params (bWasCancelled :type Boolean))
  (bind _as_boss_aicontroller_base (Variables|Default|GetAs%20Boss%20AIController%20Base))
  (Utilities|FlowControl|Sequence
    (:then_0
      (Utilities|IsValid _as_boss_aicontroller_base
        (:Is%20Valid
          (Class|BossAIControllerBase|SetGroggy _as_boss_aicontroller_base))))
    (:then_1
      (for _array_element (Variables|Default|GetIn%20Area%20Player%20Arr)
        (bind _as플레이어_컨트롤러 (Utilities|Casting|CastToPlayerController (Pawn|GetController (Utilities|Struct|BreakInArrayPlayer _array_element))))
        (Game|Player|SetViewTargetwithBlend _as플레이어_컨트롤러 (Utilities|Struct|BreakInArrayPlayer _array_element) 0.0 "VTBlend_Linear" 0.0 false)))))