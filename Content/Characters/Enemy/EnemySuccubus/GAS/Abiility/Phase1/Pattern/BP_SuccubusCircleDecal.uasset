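; Succubus boss phase 1 pattern decal actor that scatters BP_ParrentBall actors over a sector area and later detonates them.
; SpawnProjectileRandomLocation spawns balls around its forward axis within an arc set by Radius, using square-root random distance for even coverage and passing on the attacker's ASC.
; Explosion calls MultiExplosion on every stored ball, then destroys the decal.
; SpawnPatternBallInArea is an empty stub.
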(event Custom|SpawnProjectileRandomLocation
  (params (LastIndex :type Integer))
  (bind _radius (Variables|Default|GetRadius))
  (bind _returnvalue (* _radius 3.6e+02))
  (bind _returnvalue_2 (/ _returnvalue 2.0))
  (bind _returnvalue_3 (Math|Trig|DegreesToRadians _returnvalue_2))
  (Utilities|IsValid (Variables|Default|GetAttacker%20ASC)
    (:Is%20Valid
      (for _index (range 0 (- LastIndex 1))
        (Variables|Default|SetRandomRadius (* (Math|Float|Sqrt (Math|Random|RandomFloat)) 1.9e+03))
        (bind _returnvalue_4 (Game|SpawnActorfromClass "/Game/Characters/Enemy/EnemySuccubus/GAS/Abiility/Phase1/Pattern/BP_ParrentBall.BP_ParrentBall_C" (Math|Transform|MakeTransform (+ (- (Transformation|GetActorLocation) "0.000000,0.000000,70.000000") (* (Math|Vector|RotateVectorAroundAxis (Transformation|GetActorForwardVector) (Math|Trig|RadiansToDegrees (Math|Random|RandomFloatinRange (* _returnvalue_3 -1.0) _returnvalue_3)) (Math|Vector|VectorUp)) (Math|Vector|MakeVector (Variables|Default|GetRandomRadius) (Variables|Default|GetRandomRadius) (Variables|Default|GetRandomRadius)))) "0, 0, 0" "1.000000,1.000000,1.000000") "Undefined" "MultiplyWithRoot" 0 (Variables|Default|GetAttacker%20ASC) 0))
        (Utilities|Array|Add (Variables|Default|GetParrentBallArr) _returnvalue_4)))))

(event Custom|Explosion
  (for _array_element (Variables|Default|GetParrentBallArr)
    (Default|MultiExplosion _array_element))
  (Actor|DestroyActor))

(event EventBeginPlay
  (|CallParentFunction))

(event Collision|EventActorBeginOverlap
  (params (OtherActor :type Actor%20Object%20Reference)))

(event EventTick
  (params (DeltaSeconds :type Float%20%28single-precision%29)))

(fn ConstructionScript
  (|CallParentFunction))

(fn SpawnPatternBallinArea)