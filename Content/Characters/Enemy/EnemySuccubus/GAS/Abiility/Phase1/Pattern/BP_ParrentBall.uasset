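; Orb actor for the Succubus enemy's Phase 1 attack pattern that rises on spawn and can explode for area damage.
; An Up timeline lifts it 200 units from its starting height.
; MultiExplosion, called from outside this graph, swaps the orb effect for a hit effect and sphere-traces around it.
; Hit actors with an ASC receive GE_DummyAttack from AttackerASC, then the orb destroys itself after a short delay.
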(event Custom|MultiExplosion
  (bind _returnvalue (Transformation|GetActorLocation))
  (Components|Activation|Deactivate (Variables|Default|GetP_Projectile_Orb01_Purple))
  (Components|Activation|Activate (Variables|Default|GetP_Hit_Orb01_Purple) false)
  (Utilities|IsValid (Variables|Default|GetAttackerASC)
    (:Is%20Valid
      (bind _outhits (Collision|MultiSphereTraceForObjects _returnvalue _returnvalue 3e+02 (Variables|Default|GetObject%20Types) false 0 "None"))
      (for _array_element _outhits
        (Utilities|IsValid (Ability|GetAbilitySystemComponent (.HitActor (Collision|BreakHitResult _array_element)))
          (:Is%20Valid
            (Class|GASAbilitySystemLibrary|ApplyGASEffecttoTargettoASC (Variables|Default|GetAttackerASC) (Ability|GetAbilitySystemComponent (.HitActor (Collision|BreakHitResult _array_element))) "/Game/BluePrints/GAS/GameplayEffect/Enemy/Enemy1/GE_DummyAttack.GE_DummyAttack_C" 1.0))))
      (Utilities|FlowControl|Delay 0.6)
      (Actor|DestroyActor))
    (:Is%20Not%20Valid
      (Utilities|FlowControl|Delay 0.6)
      (Actor|DestroyActor))))

(event EventBeginPlay
  (bind _returnvalue (Transformation|GetActorLocation))
  (bind _returnvalue_2 (Transformation|GetActorLocation))
  (Variables|Default|SetCurrent%20Vector%20Z (.z _returnvalue_2))
  (Variables|Default|SetTargetVectorZ (+ (.z _returnvalue_2) 2e+02))
  (bind _lerp (Timeline|Up Play)
    (:Update
      (Transformation|SetActorLocation (Math|Vector|MakeVector (.x _returnvalue) (.y _returnvalue) (Math|Float|Lerp (Variables|Default|GetCurrent%20Vector%20Z) (Variables|Default|GetTargetVectorZ) _lerp)) false false))))

(event Collision|EventActorBeginOverlap
  (params (OtherActor :type Actor%20Object%20Reference)))

(event EventTick
  (params (DeltaSeconds :type Float%20%28single-precision%29)))

(fn ConstructionScript
  (Components|Activation|SetAutoActivate (Variables|Default|GetP_Hit_Orb01_Purple) false))