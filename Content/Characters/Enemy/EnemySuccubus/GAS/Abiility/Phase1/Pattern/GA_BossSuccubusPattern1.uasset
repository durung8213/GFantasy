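; Gameplay ability for Succubus boss phase-1 pattern 1: moves the boss to the arena middle and plays a montage.
; A Spawn.Skill event spawns a ring of eight wedge decals, shuffles them, then recolors a random subset red and makes those spawn projectiles.
; Enemy.Attack triggers every decal's explosion; ability end stops event waits and can clear leftover balls and decals.
; Player camera switching and the cone-based RangeAttack are left disconnected.
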(event Ability|EventActivateAbility
  (bind _returnvalue (Ability|GetAvatarActorfromActorInfo))
  (bind _returnvalue_2 (Ability|GetAvatarActorfromActorInfo))
  (Utilities|FlowControl|Sequence
    (:then_0
      (bind _outactors (Actor|GetAllActorsOfClass "/Game/Characters/Enemy/EnemySuccubus/GAS/Abiility/Phase1/Pattern/BP_BossSuccubusCameraCamera1.BP_BossSuccubusCameraCamera1_C"))
      (Variables|Default|SetBossCamera (.OutItem (Utilities|Array|Random _outactors))))
    (:then_1
      ;[1 1 1] 보스 위치 변경
      (bind _returnvalue_3 (Class|BossEnemyInterface|GetBossAreaMiddlePositionPointLocation(Message) _returnvalue))
      (Transformation|SetActorLocation _returnvalue _returnvalue_3 false false))
    (:then_2
      (|PlayMontageandWaitProxy "None" "/Game/Characters/Enemy/EnemySuccubus/Anim/Phase1/Pattern/AM_Pattern1.AM_Pattern1" 1.0 "None" true 1.0 0.0 false
        (:then
          (bind _asynctaskproxy (Ability|Async|WaitGameplayEventToActor _returnvalue_2 "(TagName=\"Spawn.Skill\")")
            (:then
              (Variables|Default|SetSkill%20Async%20Action _asynctaskproxy))
            (:EventReceived
              (for _index (range 0 7)
                (bind _returnvalue_4 (Game|SpawnActorfromClass "/Game/Characters/Enemy/EnemySuccubus/GAS/Abiility/Phase1/Pattern/BP_SuccubusCircleDecal.BP_SuccubusCircleDecal_C" (Math|Transform|MakeTransform (- (Transformation|GetActorLocation _returnvalue_2) "0.000000,0.000000,100.000000") (Math|Rotator|MakeRotator 0.0 0.0 (+ (* _index 45.0) 22.5)) "8.000000,8.000000,8.000000") "Undefined" "MultiplyWithRoot" 0 (Ability|GetAbilitySystemComponentfromActorInfo) "(R=0.000000,G=0.804892,B=1.000000,A=1.000000)" 0.125 0))
                (Utilities|Array|Add (Variables|Default|GetDecalActorArr) _returnvalue_4))
              (Utilities|Array|Shuffle (Variables|Default|GetDecalActorArr))
              (bind _output_get (Variables|Default|SetAttackArrIndex (Math|Random|RandomIntegerinRange 4 6)))
              (for _index_2 (range 0 _output_get)
                (Default|ServerSetDecalColor (Utilities|Array|Get(acopy) (Variables|Default|GetDecalActorArr) _index_2) "(R=1.000000,G=0.039216,B=0.000000,A=1.000000)")
                (Default|SpawnProjectileRandomLocation (Utilities|Array|Get(acopy) (Variables|Default|GetDecalActorArr) _index_2) 20)
                (bind _asynctaskproxy_2 (Ability|Async|WaitGameplayEventToActor (Ability|GetAvatarActorfromActorInfo) "(TagName=\"Enemy.Attack\")")
                  (:then
                    (Variables|Default|SetAttack%20Async%20Action _asynctaskproxy_2))
                  (:EventReceived
                    (for _array_element (Variables|Default|GetDecalActorArr)
                      (Utilities|IsValid _array_element
                        (:Is%20Valid
                          (Default|Explosion _array_element))))
                    (Utilities|Array|Clear (Variables|Default|GetDecalActorArr))))))))
        (:OnCompleted
          (Ability|EndAbility))))))

(event Ability|EventOnEndAbility
  (params (bWasCancelled :type Boolean))
  (bind _attack_async_action (Variables|Default|GetAttack%20Async%20Action))
  (bind _decalactorarr (Variables|Default|GetDecalActorArr))
  (Ability|Async|EndAction (Variables|Default|GetSkill%20Async%20Action))
  (Utilities|IsValid _attack_async_action
    (:Is%20Valid
      (Ability|Async|EndAction _attack_async_action)
      (for _array_element _decalactorarr
        (for _array_element_2 (Variables|/Game/Characters/Enemy/EnemySuccubus/GAS/Abiility/Phase1/Pattern/BP_SuccubusCircleDecal.BP_SuccubusCircleDecal_C|GetParrentBallArr _array_element)
          (Actor|DestroyActor _array_element_2)))
      (for _array_element_3 _decalactorarr
        (Actor|DestroyActor _array_element_3))
      (Utilities|Array|Clear _decalactorarr))))

(fn RangeAttack
  (params (Origin :type Vector) (Forward :type Vector) (TargetActor :type GAS%20Player%20Character%20Object%20Reference) (Radius :type Float%20%28double-precision%29) (AngleDegrees :type Float%20%28double-precision%29))
  (bind _returnvalue (Ability|GetOwningActorfromActorInfo))
  (bind _returnvalue_2 (Transformation|GetActorLocation TargetActor))
  (bind _returnvalue_3 (Ability|GetAbilitySystemComponent _returnvalue))
  (bind _returnvalue_4 (- _returnvalue_2 Origin))
  (if (<= (Math|Vector|VectorLength _returnvalue_4) Radius)
    (if (>= (Math|Vector|DotProduct Forward (Math|Vector|Normalize _returnvalue_4)) (Math|Trig|Cos(Radians) (Math|Trig|DegreesToRadians (* AngleDegrees 0.5))))
      (Development|PrintString (Utilities|String|Append (Utilities|GetDisplayName TargetActor) "는 타격 안에 있음"))
      (GameplayEffects|ApplyGameplayEffectSpecToTarget _returnvalue_3 (GameplayEffects|MakeOutgoingSpec _returnvalue_3 "/Game/BluePrints/GAS/GameplayEffect/Enemy/Enemy1/GE_DummyAttack.GE_DummyAttack_C" 1.0 (GameplayEffects|MakeEffectContext _returnvalue_3)) (Ability|GetAbilitySystemComponent TargetActor)))))