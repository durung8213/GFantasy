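; Gameplay ability for the Succubus boss's second phase-1 normal attack, a lightning beam from the right hand along a spline.
; It spawns the spline actor ahead of the boss, clears AI focus and plays the beam montage.
; Montage-driven gameplay events start turning toward the spline start, spawn the beam and end it.
; Looping timers smoothly rotate the boss, tracking the beam's end point once spawned; ability end cleans up beam and spline.
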(event Custom|LerpToStart
  (bind _returnvalue (Ability|GetAvatarActorfromActorInfo))
  (bind _bp_boss_1normal_attack_2beam_spline (Variables|Default|GetBP%20Boss%201Normal%20Attack%202Beam%20Spline))
  (bind _beamspline (Variables|/Game/BluePrints/Actor/Beam/BP_BeamSplineBase.BP_BeamSplineBase_C|GetBeamSpline _bp_boss_1normal_attack_2beam_spline))
  ;[1 0.7384 0] 빔 소환
  (Utilities|IsValid _bp_boss_1normal_attack_2beam_spline
    (:Is%20Valid
      (Utilities|IsValid _beamspline
        (:Is%20Valid
          (Transformation|SetActorRotation _returnvalue (Math|Interpolation|RInterpTo (Transformation|GetActorRotation _returnvalue) (Math|Rotator|FindLookatRotation (Transformation|GetActorLocation _returnvalue) (Spline|GetLocationatDistanceAlongSpline _beamspline 0.0 "World")) 0.03 2.0)))))))

(event Custom|LookOnSpline
  (bind _returnvalue (Ability|GetAvatarActorfromActorInfo))
  (bind _beamactor (Variables|Default|GetBeamActor))
  ;[1 0.7384 0] 빔 소환
  (Utilities|IsValid _beamactor
    (:Is%20Valid
      (Transformation|SetActorRotation _returnvalue (Math|Interpolation|RInterpTo (Transformation|GetActorRotation _returnvalue) (Math|Rotator|FindLookatRotation (Transformation|GetActorLocation _returnvalue) (Variables|/Game/BluePrints/Actor/Beam/BP_BeamBase.BP_BeamBase_C|GetEndLocation _beamactor)) 0.03 2.0)))))

(event Ability|EventActivateAbility
  (bind _returnvalue (Ability|GetAvatarActorfromActorInfo))
  (bind _returnvalue_2 (Ability|GetAvatarActorfromActorInfo))
  (bind _returnvalue_3 (AI|GetAIController _returnvalue))
  (bind (_asbp_boss_succubus _bsuccess) (Utilities|Casting|CastToBP_BossSuccubus _returnvalue))
  (bind _returnvalue_4 (Transformation|GetActorTransform _asbp_boss_succubus))
  (Utilities|FlowControl|Sequence
    (:then_0
      ;[0 0.9354 1] 경로 스플라인 생성
      (bind _spawnedactor (|SpawnActor 0 (- (+ (Transformation|GetActorLocation _returnvalue_2) (* "1000.000000,1000.000000,1000.000000" (Transformation|GetActorForwardVector _returnvalue_2))) "0.000000,0.000000,50.000000") (Transformation|GetActorRotation _returnvalue_2) "/Game/BluePrints/Actor/Beam/Enemy3/BP_Boss1NormalAttack2BeamSpline.BP_Boss1NormalAttack2BeamSpline_C" false 0)
        (:Success
          (bind _asbp_boss_1normal_attack_2beam_spline (Utilities|Casting|CastToBP_Boss1NormalAttack2BeamSpline _spawnedactor))
          (Variables|Default|SetBP%20Boss%201Normal%20Attack%202Beam%20Spline _asbp_boss_1normal_attack_2beam_spline))))
    (:then_1
      (AI|ClearFocus (AI|GetAIController (Ability|GetAvatarActorfromActorInfo))))
    (:then_2
      ;[1 0.7384 0] 빔 소환
      (|PlayMontageandWaitProxy "None" "/Game/Characters/Enemy/EnemySuccubus/Anim/Phase1/Attack/Attack2/04_beam_all.04_beam_all" 1.0 "None" true 1.0 0.0 false
        (:then
          (Utilities|FlowControl|Sequence
            (:then_0
              (bind _asynctaskproxy (Ability|Tasks|WaitGameplayEvent "(TagName=\"Spawn.Beam.End\")" 0)
                (:then
                  (Variables|Default|SetEndBeamAsync%20Task _asynctaskproxy))
                (:EventReceived
                  (Utilities|IsValid (Variables|Default|GetBeamActor)
                    (:Is%20Valid
                      (Default|BeamEnd (Variables|Default|GetBeamActor))
                      (Actor|DestroyActor (Variables|Default|GetBP%20Boss%201Normal%20Attack%202Beam%20Spline))
                      (Utilities|Time|ClearandInvalidateTimerbyHandle (Variables|Default|GetLookOnTimer)))))))
            (:then_1
              (Ability|Tasks|WaitGameplayEvent "(TagName=\"Spawn.Beam\")" 0
                (:EventReceived
                  (bind _returnvalue_5 (Utilities|Time|SetTimerbyEvent (delegate Custom|LerpToStart) 0.03 true))
                  (Variables|Default|SetInitRotationTimer _returnvalue_5))))
            (:then_2
              (bind _asynctaskproxy_2 (Ability|Tasks|WaitGameplayEvent "(TagName=\"Spawn.Beam.Start\")" 0)
                (:then
                  (Variables|Default|SetCreateBeam%20Async%20Task _asynctaskproxy_2)
                  (Utilities|Time|ClearandInvalidateTimerbyHandle (Variables|Default|GetInitRotationTimer)))
                (:EventReceived
                  (if (Math|Boolean|ANDBoolean _bsuccess (Utilities|IsValid _returnvalue_3) true (Utilities|IsValid (Variables|Default|GetBP%20Boss%201Normal%20Attack%202Beam%20Spline)))
                    (AI|ClearFocus _returnvalue_3)
                    (bind _spawnedactor_2 (|SpawnActor 0 (.location _returnvalue_4) (.rotation _returnvalue_4) "/Game/BluePrints/Actor/Beam/BP_BeamBase.BP_BeamBase_C" false 0 _asbp_boss_succubus "hand_r" false (Class|AIController|GetFocusActor _returnvalue_3) (Variables|Default|GetBP%20Boss%201Normal%20Attack%202Beam%20Spline) 1.61 "/Game/Asset/VFX/M5VFXRPG2/Projectile/Beam_Proj/Proj_00_B_S_Lightning2.Proj_00_B_S_Lightning2" "/Game/Asset/VFX/M5VFXRPG2/Projectile/Impact/IMP_B_S_00_Lightning2.IMP_B_S_00_Lightning2" 1e+01 1e+01 0)
                      (:then
                        (bind _returnvalue_6 (Utilities|Time|SetTimerbyEvent (delegate Custom|LookOnSpline) 0.03 true))
                        (Variables|Default|SetLookOnTimer _returnvalue_6))
                      (:Success
                        (bind _asbp_beam_base (Utilities|Casting|CastToBP_BeamBase _spawnedactor_2))
                        (Variables|Default|SetBeamActor _asbp_beam_base)))))))))
        (:OnCompleted
          (Ability|EndAbility :!label _label))
        (:OnBlendOut
          (goto _label))
        (:OnInterrupted
          (goto _label))
        (:OnCancelled
          (goto _label))))))

(event Ability|EventOnEndAbility
  (params (bWasCancelled :type Boolean))
  (bind _beamactor (Variables|Default|GetBeamActor))
  (bind _createbeam_async_task (Variables|Default|GetCreateBeam%20Async%20Task))
  (bind _endbeamasync_task (Variables|Default|GetEndBeamAsync%20Task))
  (Development|PrintString "어빌리티 종료")
  (Utilities|IsValid _createbeam_async_task
    (:Is%20Valid
      (GameplayTasks|EndTask _createbeam_async_task))
    (:Is%20Not%20Valid
      _))
  (Utilities|IsValid _endbeamasync_task
    (:Is%20Valid
      (GameplayTasks|EndTask _endbeamasync_task))
    (:Is%20Not%20Valid
      _))
  (Utilities|IsValid _beamactor
    (:Is%20Valid
      (Default|BeamEnd _beamactor)
      (Actor|DestroyActor (Variables|Default|GetBP%20Boss%201Normal%20Attack%202Beam%20Spline))
      (Utilities|Time|ClearandInvalidateTimerbyHandle (Variables|Default|GetLookOnTimer)))))