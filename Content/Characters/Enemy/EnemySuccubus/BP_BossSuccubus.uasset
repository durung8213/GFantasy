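; Succubus boss character that starts with horns and weapon hidden and exposes events to reveal them, including for its second phase.
; Construction makes child skeletal meshes follow the hidden main Mesh's pose, while BeginPlay retries on a timer until the weapon child actor can be hidden.
; Horns appear through a dissolve timeline on a dynamic material; the phase-two event also registers the weapon.
; Projectile shot point comes from the arm's right-hand bone.
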(event Custom|HornVisible
  (Rendering|SetVisibility (Variables|Default|GetSK_LAUREN_HORNS) true false)
  (Utilities|IsValid (Variables|Default|GetHornDynamicInstance)
    (:Is%20Valid
      (bind _dissolvetime (Timeline|HornDissolveTimeline PlayFromStart)
        (:Update
          (Rendering|Material|SetScalarParameterValue (Variables|Default|GetHornDynamicInstance) "DissolveAmount" _dissolvetime :!class /Script/Engine.MaterialInstanceDynamic))))
    (:Is%20Not%20Valid
      (bind _returnvalue (Rendering|Material|CreateDynamicMaterialInstance (Variables|Default|GetSK_LAUREN_HORNS) 0 "/Game/Asset/Character/Succubus_Lauren/Materials/Clothes/MI_LAUREN_WINGS_Red.MI_LAUREN_WINGS_Red" "None" :!class /Script/Engine.PrimitiveComponent))
      (Variables|Default|SetHornDynamicInstance _returnvalue)
      (Timeline|HornDissolveTimeline PlayFromStart))))

(event Custom|WeaponVisible
  (Rendering|SetVisibility (Variables|Default|GetBP_SuccubusWeapon) true false)
  (bind _asbp_succubus_weapon (Utilities|Casting|CastToBP_SuccubusWeapon (Variables|/Script/Engine.ChildActorComponent|GetChildActor (Variables|Default|GetBP_SuccubusWeapon))))
  (Default|WeaponVisible _asbp_succubus_weapon))

(event Custom|HideWeaponTimer
  (bind _bp_succubusweapon (Variables|Default|GetBP_SuccubusWeapon))
  (Utilities|IsValid _bp_succubusweapon
    (:Is%20Valid
      (bind _asbp_succubus_weapon (Utilities|Casting|CastToBP_SuccubusWeapon (Variables|/Script/Engine.ChildActorComponent|GetChildActor _bp_succubusweapon))
        (:then
          (Default|HideWeapon _asbp_succubus_weapon)
          (Rendering|SetVisibility _bp_succubusweapon false false))
        (:CastFailed
          (Utilities|Time|SetTimerbyEvent (delegate Custom|HideWeaponTimer) 0.0 :!label _label))))
    (:Is%20Not%20Valid
      (goto _label))))

(event EventBeginPlay
  (CallFunction|HideWeaponTimer))

(event Collision|EventActorBeginOverlap
  (params (OtherActor :type Actor%20Object%20Reference)))

(event EventTick
  (params (DeltaSeconds :type Float%20%28single-precision%29)))

(event EventChangeMeshTwoPhase
  (Rendering|SetVisibility (Variables|Default|GetBP_SuccubusWeapon) true false)
  (Rendering|SetVisibility (Variables|Default|GetSK_LAUREN_HORNS) true false)
  (Class|GASCombatNPC|SetWeapon (Variables|Default|GetBP_SuccubusWeapon))
  (Class|GASCombatNPC|AddWeaponArr (Variables|Default|GetBP_SuccubusWeapon)))

(fn ConstructionScript
  (for _array_element (Components|GetChildrenComponents (Variables|Character|GetMesh) true)
    (bind _as스켈레탈_메시_컴포넌트 (Utilities|Casting|CastToSkeletalMeshComponent _array_element))
    (Components|SkinnedMesh|SetLeaderPoseComponent _as스켈레탈_메시_컴포넌트 (Variables|Character|GetMesh) true true))
  (Rendering|SetVisibility (Variables|Default|GetSK_LAUREN_HORNS) false false)
  (Rendering|SetVisibility (Variables|Character|GetMesh) false false)
  (Rendering|SetVisibility (Variables|Default|GetBP_SuccubusWeapon) false false))

(fn GetProjectileShotPoint
  (return (Transformation|GetBoneTransform (Variables|Default|GetArm) "hand_r" "RTS_World")))