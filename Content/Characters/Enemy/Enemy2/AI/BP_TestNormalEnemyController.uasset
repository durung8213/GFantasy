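; AI controller for the test normal enemy that runs its behavior tree and drives a Passive, Investigation or Attacking state through the Blackboard.
; On possess it starts Passive and copies the pawn's attack and defend radii to the Blackboard.
; Perception updates are sorted by sense: sighting the player triggers Attacking, hearing triggers Investigation at the sound location, neither overriding Attacking.
; Damage sensing is left unhandled; helpers toggle focus and hit state.
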(event OnPerceptionUpdated(AIPerception)
  (params (UpdatedActors :type Array%20of%20Actor%20Object%20References))
  (for _array_element UpdatedActors
    (Utilities|FlowControl|Sequence
      (:then_0
        (bind _scens (CallFunction|CanSenseActor _array_element "NewEnumerator1"))
        (if _scens
          (CallFunction|HandleSecondSight _array_element)))
      (:then_1
        (bind (_scens_2 _array_element_2) (CallFunction|CanSenseActor _array_element "NewEnumerator2"))
        (if _scens_2
          (CallFunction|HandleSecondSound 0 (Utilities|Struct|BreakAIStimulus _array_element_2))))
      (:then_2
        (bind _scens_3 (CallFunction|CanSenseActor _array_element "NewEnumerator3"))
        (if _scens_3
          _)))))

(event Custom|SetHitDoing_1
  (params (bIsHitDoing :type Boolean))
  (AI|Components|Blackboard|SetValueasBool (Variables|Default|GetBlackboard) (Variables|KeyName|GetHitDoing%20Key%20Name) bIsHitDoing))

(event EventBeginPlay)

(event EventTick
  (params (DeltaSeconds :type Float%20%28single-precision%29)))

(event EventPossess
  (params (PossessedPawn :type Pawn%20Object%20Reference))
  (AI|RunBehaviorTree "/Game/Characters/Enemy/Enemy2/AI/BT_TestNormalEnemy.BT_TestNormalEnemy")
  (CallFunction|SetStatePassive)
  (bind (_attackradius _defendradius) (Class|BPIEnemyAI|GetIdealRange(Message) PossessedPawn))
  (AI|Components|Blackboard|SetValueasFloat (Variables|Default|GetBlackboard) (Variables|KeyName|GetAttackRadiusKeyName) _attackradius)
  (AI|Components|Blackboard|SetValueasFloat (Variables|Default|GetBlackboard) (Variables|KeyName|GetDefendRadiusKeyName) _defendradius))

(fn ConstructionScript)

(fn GetCurrentState
  (return (Utilities|Enum|ByteToEnumBP_EEnemyState (Class|BlackboardComponent|GetValueasEnum (Variables|Default|GetBlackboard) (Variables|Default|GetStateKeyName)))))

(fn SetStateAttacking
  (params (CurrentAttackTarget :type Actor%20Object%20Reference))
  (AI|Components|Blackboard|SetValueasEnum (Variables|Default|GetBlackboard) (Variables|Default|GetState%20Key%20Name) (Utilities|Enum|LiteralenumBP_EEnemyState "NewEnumerator1"))
  (AI|Components|Blackboard|SetValueasObject (Variables|Default|GetBlackboard) (Variables|KeyName|GetPlayer%20Key%20Name) CurrentAttackTarget)
  (Variables|Default|SetAttackTarget CurrentAttackTarget))

(fn SetStatePassive
  (AI|Components|Blackboard|SetValueasEnum (Variables|Default|GetBlackboard) (Variables|Default|GetStateKeyName) (Utilities|Enum|LiteralenumBP_EEnemyState "NewEnumerator0")))

(fn SetStateInvestigation
  (params (Location :type Vector))
  (AI|Components|Blackboard|SetValueasEnum (Variables|Default|GetBlackboard) (Variables|Default|GetStateKeyName) (Utilities|Enum|LiteralenumBP_EEnemyState "NewEnumerator3"))
  (AI|Components|Blackboard|SetValueasVector (Variables|Default|GetBlackboard) (Variables|KeyName|GetPointOfInterestKeyName) Location))

(fn SetStateStrafe
  (AI|Components|Blackboard|SetValueasEnum (Variables|Default|GetBlackboard) (Variables|Default|GetStateKeyName) (Utilities|Enum|LiteralenumBP_EEnemyState "NewEnumerator1"))
  (bind _returnvalue (Actor|GetActorOfClass "/Game/Characters/Players/BP_GASTestPlayerCharacter.BP_GASTestPlayerCharacter_C"))
  (CallFunction|HandleSecondSight _returnvalue))

(fn CanSenseActor
  (params (Actor :type Actor%20Object%20Reference) (Sense :type EEnemySense%20Enum :default "NewEnumerator0"))
  (bind _info (Class|AIPerceptionComponent|GetActorsPerception (Variables|Default|GetAIPerception) Actor)) ; 주어진 액터가 감지되었는지 검색
  (for _array_element (.LastSensedStimuli (Utilities|Struct|BreakActorPerceptionBlueprintInfo _info))
    (bind _returnvalue (Class|AIPerceptionSystem|GetSenseClassforStimulus _array_element))
    (if (== _returnvalue (Utilities|Select :Index Sense :NewEnumerator0 0 :NewEnumerator1 "/Script/AIModule.AISense_Sight" :NewEnumerator2 "/Script/AIModule.AISense_Hearing" :NewEnumerator3 "/Script/AIModule.AISense_Damage"))
      (return (== _returnvalue (Utilities|Select :Index Sense :NewEnumerator0 0 :NewEnumerator1 "/Script/AIModule.AISense_Sight" :NewEnumerator2 "/Script/AIModule.AISense_Hearing" :NewEnumerator3 "/Script/AIModule.AISense_Damage")) _array_element))))

(fn HandleSecondSight
  (params (Actor :type Actor%20Object%20Reference))
  (bind _asgasplayer_character (Utilities|Casting|CastToGASPlayerCharacter Actor))
  (bind _newparam (CallFunction|GetCurrentState))
  (switch Utilities|FlowControl|Switch|SwitchonBP_EEnemyState _newparam
    (:NewEnumerator0
      _)
    (:NewEnumerator3
      _))
  (CallFunction|SetStateAttacking _asgasplayer_character))

(fn HandleSecondSound
  (params (AActor :type Actor%20Object%20Reference) (Location :type Vector))
  (bind _newparam (CallFunction|GetCurrentState))
  (switch Utilities|FlowControl|Switch|SwitchonBP_EEnemyState _newparam
    (:NewEnumerator0
      _)
    (:NewEnumerator3
      _))
  (CallFunction|SetStateInvestigation Location))

(fn HandleSecondDamage
  (params (AActor :type Actor%20Object%20Reference) (Location :type Vector))
  (bind _newparam (CallFunction|GetCurrentState))
  (switch Utilities|FlowControl|Switch|SwitchonBP_EEnemyState _newparam
    (:NewEnumerator0
      _)
    (:NewEnumerator3
      _))
  (CallFunction|SetStateAttacking))

(fn SetFocusPlayer
  (params (NewFocus :type Actor%20Object%20Reference))
  (AI|SetFocus NewFocus)
  (Class|BPIEnemyAI|SetIsFocus(Message) (Pawn|GetControlledPawn) true))

(fn SetFocalPoint2
  (params (FP :type Vector))
  (AI|SetFocalPoint FP))

(fn SetClearFocus
  (AI|ClearFocus)
  (Class|BPIEnemyAI|SetIsFocus(Message) (Pawn|GetControlledPawn) false))