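; Test enemy character that wields a great sword and exposes patrol, combat range, focus and movement speed accessors.
; On BeginPlay, InitWeapon registers the great sword child actor as the current weapon and adds it to the weapon array, retrying on a timer until that actor is valid.
; Getters supply the patrol route, fixed attack and defend radii and focus state, while events and setters handle focus, walk speed and ragdoll.
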(event EventBeginPlay
  (Class|GASCombatNPC|InitWeapon))

(event Collision|EventActorBeginOverlap
  (params (OtherActor :type Actor%20Object%20Reference)))

(event EventIRagdoll
  (Class|GASCombatNPC|Ragdoll))

(event EventSetIsFocus
  (params (IsFocus :type Boolean))
  (Class|GASCombatNPC|SetbIsFocus IsFocus))

(event EventInitWeapon
  (bind _bp_greatsword (Variables|Default|GetBP_GreatSword))
  (if (and (Utilities|IsValidClass (Variables|/Script/Engine.ChildActorComponent|GetChildActorClass _bp_greatsword)) (Utilities|IsValid (Variables|/Script/Engine.ChildActorComponent|GetChildActor _bp_greatsword)))
    (Utilities|FlowControl|Sequence
      (:then_0
        (Class|GASCombatNPC|SetWeapon (Variables|Default|GetBP_GreatSword)))
      (:then_1
        (Class|GASCombatNPC|AddWeaponArr (Variables|Default|GetBP_GreatSword))))
    (else
      (Utilities|Time|SetTimerbyEvent (delegate EventInitWeapon) 0.5))))

(fn ConstructionScript)

(fn GetPatrolRoute
  (return (Variables|Default|GetPatrolRoute)))

(fn GetIdealRange
  (return 1.5e+02 3.5e+02))

(fn GetIsFocus
  (return (Variables|Default|GetbIsFocus)))

(fn SetMovementSpeed
  (params (Speed :type Float%20%28double-precision%29))
  (bind _output_get (Variables|/Script/Engine.CharacterMovementComponent|SetMaxWalkSpeed (Variables|Character|GetCharacterMovement) Speed))
  (return _output_get))