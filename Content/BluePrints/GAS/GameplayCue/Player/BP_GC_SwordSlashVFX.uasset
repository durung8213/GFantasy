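; Gameplay Cue for the player's sword slash that spawns a slash hit particle where the hit lands.
; Both OnActive and OnExecute read the instigator and hit result from the effect context, spawning at the impact point, oriented by instigator forward and impact normal.
; OnActive uses a fixed slash-hit emitter, while OnExecute uses the Particle variable at a larger scale.
; Both print debug messages.
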(event EventBeginPlay)

(event Collision|EventActorBeginOverlap
  (params (OtherActor :type Actor%20Object%20Reference)))

(event EventTick
  (params (DeltaSeconds :type Float%20%28single-precision%29)))

(fn ConstructionScript)

(fn OnActive
  (params (MyTarget :type Actor%20Object%20Reference) (Parameters :type Gameplay%20Cue%20Parameters%20Structure%20%28by%20ref%29))
  (bind _effectcontext (Ability|GameplayCue|BreakGameplayCueParameters Parameters))
  (bind _returnvalue (Class|AbilitySystemBlueprintLibrary|EffectContextGetHitResult _effectcontext))
  (bind (_bblockinghit _binitialoverlap _time _distance _location _impactpoint _normal _impactnormal) (Collision|BreakHitResult _returnvalue))
  (Development|PrintString 0 "Slash VFX" true true "(R=0.378946,G=0.000000,B=1.000000,A=1.000000)")
  (bind _output_get (Variables|Default|SetCurrentInstigator (Class|AbilitySystemBlueprintLibrary|EffectContextGetInstigatorActor _effectcontext)))
  (Effects|SpawnEmitteratLocation 0 "/Game/Asset/VFX/FantasyVFXCollection/3_ParticleSystem/SlashHit/Element_SlashHit_01/P_Element_SlashHit_01.P_Element_SlashHit_01" _impactpoint (Math|Rotator|MakeRotfromXZ (Transformation|GetActorForwardVector _output_get) _impactnormal))
  (return true))

(fn OnExecute
  (params (MyTarget :type Actor%20Object%20Reference) (Parameters :type Gameplay%20Cue%20Parameters%20Structure%20%28by%20ref%29))
  (bind _effectcontext (Ability|GameplayCue|BreakGameplayCueParameters Parameters))
  (bind _returnvalue (Class|AbilitySystemBlueprintLibrary|EffectContextGetHitResult _effectcontext))
  (bind (_bblockinghit _binitialoverlap _time _distance _location _impactpoint _normal _impactnormal) (Collision|BreakHitResult _returnvalue))
  (Development|PrintString 0 "Slash VFX" true true "(R=0.378946,G=0.000000,B=1.000000,A=1.000000)")
  (bind _output_get (Variables|Default|SetCurrentInstigator (Class|AbilitySystemBlueprintLibrary|EffectContextGetInstigatorActor _effectcontext)))
  (bind _returnvalue_2 (Effects|SpawnEmitteratLocation 0 (LocalVariables|GetParticle) _impactpoint (Math|Rotator|MakeRotfromXZ (Transformation|GetActorForwardVector _output_get) _impactnormal) "1.500000,1.500000,1.500000"))
  (Development|PrintString 0 "Spawn Emiiter :: " (Utilities|IsValid _returnvalue_2))
  (return true))