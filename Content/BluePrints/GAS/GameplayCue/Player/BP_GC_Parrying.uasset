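; Gameplay cue for a player parry, giving the local player impact feedback when it becomes active.
; OnActive checks for a locally controlled GAS player character, then spawns a pooled effect system at the cue location.
; It then passes the player's camera manager to a client event that plays the parry camera shake.
; A brief global time-dilation hit-stop is present but never runs.
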(event Custom|Client_ParryDelay
  (params (cameraManager :type Player%20Camera%20Manager%20Object%20Reference))
  (CameraShakes|StartCameraShake cameraManager "/Game/BluePrints/Combat/PlayerSkill/Camera/BP_CS_ParryShake.BP_CS_ParryShake_C" 1.0 "CameraLocal" "0, 0, 0"))

(event EventBeginPlay)

(event Collision|EventActorBeginOverlap
  (params (OtherActor :type Actor%20Object%20Reference)))

(event EventTick
  (params (DeltaSeconds :type Float%20%28single-precision%29)))

(fn ConstructionScript)

(fn OnActive
  (params (MyTarget :type Actor%20Object%20Reference) (Parameters :type Gameplay%20Cue%20Parameters%20Structure%20%28by%20ref%29))
  (bind _asbp_gasplayer_character (Utilities|Casting|CastToBP_GASPlayerCharacter MyTarget)
    (:then
      (if (Pawn|IsLocallyControlled _asbp_gasplayer_character)
        (Niagara|SpawnSystematLocation 0 (LocalVariables|GetNewLocalVar) (.Location (Ability|GameplayCue|BreakGameplayCueParameters Parameters)) "0, 0, 0" "1.000000,1.000000,1.000000" true true "AutoRelease")
        (bind _asbp_gasworld_player_controller (Utilities|Casting|CastToBP_GASWorldPlayerController (Pawn|GetController _asbp_gasplayer_character)))
        (CallFunction|ClientParryDelay (Variables|/Script/Engine.PlayerController|GetPlayerCameraManager _asbp_gasworld_player_controller))
        (return true)))
    (:CastFailed
      (Development|PrintString 0 "NO Panw"))))