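; Gameplay cue notify that plays the parry hit feedback for the player character.
; On execute, it acts only when the target is a locally controlled GAS player character, so other clients see nothing from it.
; It spawns a pooled Niagara effect at the cue's location, then starts a parry camera shake through the player controller's camera manager.
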(fn OnExecute
  (params (MyTarget :type Actor%20Object%20Reference) (Parameters :type Gameplay%20Cue%20Parameters%20Structure%20%28by%20ref%29))
  (bind _asbp_gasplayer_character (Utilities|Casting|CastToBP_GASPlayerCharacter MyTarget)
    (:then
      (if (Pawn|IsLocallyControlled _asbp_gasplayer_character)
        (Niagara|SpawnSystematLocation 0 (LocalVariables|GetNiagara) (.Location (Ability|GameplayCue|BreakGameplayCueParameters Parameters)) "0, 0, 0" "1.000000,1.000000,1.000000" true true "AutoRelease")
        (bind _asbp_gasworld_player_controller (Utilities|Casting|CastToBP_GASWorldPlayerController (Pawn|GetController _asbp_gasplayer_character)))
        (CameraShakes|StartCameraShake (Variables|/Script/Engine.PlayerController|GetPlayerCameraManager _asbp_gasworld_player_controller) "/Game/BluePrints/Combat/PlayerSkill/Camera/BP_CS_ParryShake.BP_CS_ParryShake_C" 1.0 "CameraLocal" "0, 0, 0")
        (return true)))
    (:CastFailed
      (Development|PrintString 0 "NO Panw"))))