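; Looping gameplay cue that shows a sword charging Niagara effect on the GAS player character.
; OnActive casts the target to BP_GASPlayerCharacter, deactivates any existing effect, then attaches an auto-release pooled system to the mesh's ChargeSocket and stores the reference.
; OnRemove deactivates and clears that stored effect.
; Both events print debug strings.
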(fn ConstructionScript)

(fn OnRemove
  (params (MyTarget :type Actor%20Object%20Reference) (Parameters :type Gameplay%20Cue%20Parameters%20Structure%20%28by%20ref%29))
  (Utilities|IsValid (Variables|Default|GetSpawnedEffect)
    (:Is%20Valid
      (Components|Activation|Deactivate (Variables|Default|GetSpawnedEffect))
      (Development|PrintString 0 "Deactivate Effect" true true "(R=0.063658,G=1.000000,B=0.099171,A=1.000000)")
      (Variables|Default|SetSpawnedEffect 0)
      (return true))
    (:Is%20Not%20Valid
      (Development|PrintString 0 "No Spawned Effect"))))

(fn OnActive
  (params (MyTarget :type Actor%20Object%20Reference) (Parameters :type Gameplay%20Cue%20Parameters%20Structure%20%28by%20ref%29))
  (bind _asbp_gasplayer_character (Utilities|Casting|CastToBP_GASPlayerCharacter MyTarget))
  (bind _spawnedeffect (Variables|Default|GetSpawnedEffect)
    (:then
      (Components|Activation|Deactivate _spawnedeffect)
      (Development|PrintString 0 "Deactivate" true true (LocalVariables|GetNewLocalVar_0)))
    (:else
      _))
  (bind _returnvalue (Niagara|SpawnSystemAttached (Variables|Default|GetNiagaraEffect) (Variables|/Script/Engine.Character|GetMesh _asbp_gasplayer_character) "ChargeSocket" "0, 0, 0" "0, 0, 0" "KeepRelativeOffset" false true "AutoRelease"))
  (bind _output_get (Variables|Default|SetSpawnedEffect _returnvalue))
  (Development|PrintString 0 "SpawnEffect" true true (LocalVariables|GetNewLocalVar))
  (return (Utilities|IsValid _output_get)))