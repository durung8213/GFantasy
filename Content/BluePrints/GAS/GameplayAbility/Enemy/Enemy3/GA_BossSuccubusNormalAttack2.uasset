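; Gameplay ability for the Succubus boss's second normal attack, a lightning beam timed by montage gameplay events.
; On activation it spawns a beam path spline ahead of the boss and plays the attack montage.
; Spawn.Beam.Start clears AI focus and spawns the beam at the boss, while Spawn.Beam.End ends it and destroys the spline.
; The ability finishes with the montage, ending both event wait tasks.
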(event Ability|EventActivateAbility
  (bind _returnvalue (Ability|GetAvatarActorfromActorInfo))
  (bind _returnvalue_2 (Ability|GetAvatarActorfromActorInfo))
  (bind _returnvalue_3 (AI|GetAIController _returnvalue_2))
  (bind (_asbp_boss_succubus _bsuccess) (Utilities|Casting|CastToBP_BossSuccubus _returnvalue_2))
  (Utilities|FlowControl|Sequence
    (:then_0
      ;[0 0.9354 1] 경로 스플라인 생성
      (bind _spawnedactor (|SpawnActor 0 (+ (Transformation|GetActorLocation _returnvalue) (* "1000.000000,1000.000000,1000.000000" (Transformation|GetActorForwardVector _returnvalue))) (Transformation|GetActorRotation _returnvalue) "/Game/BluePrints/Actor/Beam/Enemy3/BP_Boss1NormalAttack2BeamSpline.BP_Boss1NormalAttack2BeamSpline_C" false 0)
        (:Success
          (bind _asbp_boss_1normal_attack_2beam_spline (Utilities|Casting|CastToBP_Boss1NormalAttack2BeamSpline _spawnedactor))
          (Variables|Default|SetBP%20Boss%201Normal%20Attack%202Beam%20Spline _asbp_boss_1normal_attack_2beam_spline))))
    (:then_1
      ;[1 0.7384 0] 빔 소환
      (|PlayMontageandWaitProxy "None" "/Game/Characters/Enemy/EnemySuccubus/Anim/Phase1/Attack/AttackTemp/AM_NormalAttack2.AM_NormalAttack2" 1.0 "None" true 1.0 0.0 false
        (:then
          (bind _asynctaskproxy (Ability|Tasks|WaitGameplayEvent "(TagName=\"Spawn.Beam.Start\")" 0)
            (:then
              (Variables|Default|SetCreateBeam%20Async%20Task _asynctaskproxy)
              (bind _asynctaskproxy_2 (Ability|Tasks|WaitGameplayEvent "(TagName=\"Spawn.Beam.End\")" 0)
                (:then
                  (Variables|Default|SetEndBeamAsync%20Task _asynctaskproxy_2))
                (:EventReceived
                  (Utilities|IsValid (Variables|Default|GetBeamActor)
                    (:Is%20Valid
                      (Default|BeamEnd (Variables|Default|GetBeamActor))
                      (Actor|DestroyActor (Variables|Default|GetBP%20Boss%201Normal%20Attack%202Beam%20Spline)))))))
            (:EventReceived
              (if (Math|Boolean|ANDBoolean _bsuccess (Utilities|IsValid _returnvalue_3) (Utilities|IsValid (Class|AIController|GetFocusActor _returnvalue_3)) (Utilities|IsValid (Variables|Default|GetBP%20Boss%201Normal%20Attack%202Beam%20Spline)))
                (AI|ClearFocus _returnvalue_3)
                (bind _spawnedactor_2 (|SpawnActor 0 (.location (Transformation|GetActorTransform _asbp_boss_succubus)) "0, 0, 0" "/Game/BluePrints/Actor/Beam/BP_BeamBase.BP_BeamBase_C" false 0 0 "0.000000,0.000000,0.000000" false 0 0 0.0 "/Game/Asset/VFX/M5VFXRPG2/Projectile/Beam_Proj/Proj_00_B_S_Lightning2.Proj_00_B_S_Lightning2" "/Game/Asset/VFX/M5VFXRPG2/Projectile/Impact/IMP_B_S_00_Lightning2.IMP_B_S_00_Lightning2" 0.0 0.0 0 0)
                  (:Success
                    (bind _asbp_beam_base (Utilities|Casting|CastToBP_BeamBase _spawnedactor_2))
                    (Variables|Default|SetBeamActor _asbp_beam_base)))))))
        (:OnCompleted
          (Ability|EndAbility :!label _label))
        (:OnBlendOut
          (goto _label))
        (:OnInterrupted
          (goto _label))
        (:OnCancelled
          (goto _label))))))

(event Ability|EventOnEndAbility
  (params (bWasCancelled :type Boolean))
  (bind _createbeam_async_task (Variables|Default|GetCreateBeam%20Async%20Task))
  (bind _endbeamasync_task (Variables|Default|GetEndBeamAsync%20Task))
  (Development|PrintString "어빌리티 종료")
  (Utilities|IsValid _createbeam_async_task
    (:Is%20Valid
      (GameplayTasks|EndTask _createbeam_async_task))
    (:Is%20Not%20Valid
      _))
  (Utilities|IsValid _endbeamasync_task
    (:Is%20Valid
      (GameplayTasks|EndTask _endbeamasync_task))))