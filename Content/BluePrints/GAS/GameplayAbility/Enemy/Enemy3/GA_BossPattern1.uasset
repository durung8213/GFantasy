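; Boss gameplay ability for attack pattern 1: switches in-area players to a boss camera, teleports the boss to a pattern point and plays the montage.
; A Spawn.Skill event spawns four quadrant decals and recolors a random one to three red.
; Enemy.Attack events apply GE_DummyAttack to players inside red quadrants via a distance and dot-product cone check, restore player views and clear decals.
; The ability ends with the montage.
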(event Ability|EventActivateAbility
  (bind _returnvalue (Ability|GetAvatarActorfromActorInfo))
  (bind _returnvalue_2 (Ability|GetAvatarActorfromActorInfo))
  (Utilities|FlowControl|Sequence
    (:then_0
      (bind _outactors (Actor|GetAllActorsOfClass "/Game/BluePrints/Actor/BossArea/BP_Boss1Camera1.BP_Boss1Camera1_C"))
      (Variables|Default|SetBossCamera (.OutItem (Utilities|Array|Random _outactors)))
      (bind _returnvalue_3 (Class|BossEnemyInterface|GetinAreaPlayers(Message) (Ability|GetAvatarActorfromActorInfo)))
      (for _array_element _returnvalue_3
        (bind _as플레이어_컨트롤러 (Utilities|Casting|CastToPlayerController (Pawn|GetController _array_element)))
        (Game|Player|SetViewTargetwithBlend _as플레이어_컨트롤러 (Variables|Default|GetBossCamera) 0.0 "VTBlend_Linear" 0.0 false)))
    (:then_1
      ;[1 1 1] 보스 위치 변경
      (bind _returnvalue_4 (Class|BossEnemyInterface|GetBossPositionPointLocationbyIndex(Message) _returnvalue))
      (Transformation|SetActorLocation _returnvalue _returnvalue_4 false false))
    (:then_2
      (|PlayMontageandWaitProxy "None" "/Game/Characters/Enemy/Enemy3/Animaion/paze1/Attack/AM_Pattern1.AM_Pattern1" 1.0 "None" true 1.0 0.0 false
        (:then
          (bind _asynctaskproxy (Ability|Async|WaitGameplayEventToActor _returnvalue_2 "(TagName=\"Spawn.Skill\")")
            (:then
              (Variables|Default|SetSkill%20Async%20Action _asynctaskproxy))
            (:EventReceived
              (for _index (range 0 3)
                (bind _returnvalue_5 (Game|SpawnActorfromClass "/Game/BluePrints/Actor/Beam/BP_CircleDecal.BP_CircleDecal_C" (Math|Transform|MakeTransform (Transformation|GetActorLocation _returnvalue_2) (Math|Rotator|MakeRotator 0.0 0.0 (+ (* _index 9e+01) 45.0)) "8.000000,8.000000,8.000000") "Undefined" "MultiplyWithRoot" 0 "(R=0.000000,G=0.804892,B=1.000000,A=1.000000)" 0.25 0))
                (Utilities|Array|Add (Variables|Default|GetDecalActorArr) _returnvalue_5))
              (Utilities|Array|Shuffle (Variables|Default|GetIntArr))
              (bind _output_get (Variables|Default|SetAttackArrIndex (Math|Random|RandomIntegerinRange 0 2)))
              (for _index_2 (range 0 _output_get)
                (Default|ServerSetDecalColor (Utilities|Array|Get(acopy) (Variables|Default|GetDecalActorArr) (Utilities|Array|Get(acopy) (Variables|Default|GetIntArr) _index_2)) "(R=1.000000,G=0.039216,B=0.000000,A=1.000000)")
                (bind _asynctaskproxy_2 (Ability|Async|WaitGameplayEventToActor (Ability|GetAvatarActorfromActorInfo) "(TagName=\"Enemy.Attack\")")
                  (:then
                    (Variables|Default|SetAttack%20Async%20Action _asynctaskproxy_2))
                  (:EventReceived
                    (for _index_3 (range 0 (Variables|Default|GetAttackArrIndex))
                      (bind _returnvalue_6 (Class|BossEnemyInterface|GetinAreaPlayers(Message) (Ability|GetAvatarActorfromActorInfo)))
                      (for _array_element_2 _returnvalue_6
                        (CallFunction|RangeAttack (Transformation|GetActorLocation (Utilities|Array|Get(acopy) (Variables|Default|GetDecalActorArr) (Utilities|Array|Get(acopy) (Variables|Default|GetIntArr) _index_3))) (Transformation|GetActorForwardVector (Utilities|Array|Get(acopy) (Variables|Default|GetDecalActorArr) (Utilities|Array|Get(acopy) (Variables|Default|GetIntArr) _index_3))) _array_element_2 2e+03 9e+01)
                        (bind _as플레이어_컨트롤러_2 (Utilities|Casting|CastToPlayerController (Pawn|GetController _array_element_2)))
                        (Game|Player|SetViewTargetwithBlend _as플레이어_컨트롤러_2 _array_element_2 0.0 "VTBlend_Linear" 0.0 false)))
                    (Utilities|FlowControl|Delay 0.2)
                    (for _array_element_3 (Variables|Default|GetDecalActorArr)
                      (Utilities|IsValid _array_element_3
                        (:Is%20Valid
                          (Actor|DestroyActor _array_element_3))))
                    (Utilities|Array|Clear (Variables|Default|GetDecalActorArr))))))))
        (:OnCompleted
          (Ability|EndAbility :!label _label))
        (:OnBlendOut
          (goto _label))
        (:OnInterrupted
          (goto _label))
        (:OnCancelled
          (goto _label))))))

(event Ability|EventOnEndAbility
  (params (bWasCancelled :type Boolean))
  (bind _attack_async_action (Variables|Default|GetAttack%20Async%20Action))
  (Ability|Async|EndAction (Variables|Default|GetSkill%20Async%20Action))
  (Utilities|IsValid _attack_async_action
    (:Is%20Valid
      (Ability|Async|EndAction _attack_async_action))))

(fn RangeAttack
  (params (Origin :type Vector) (Forward :type Vector) (TargetActor :type GAS%20Player%20Character%20Object%20Reference) (Radius :type Float%20%28double-precision%29) (AngleDegrees :type Float%20%28double-precision%29))
  (bind _returnvalue (Ability|GetOwningActorfromActorInfo))
  (bind _returnvalue_2 (Transformation|GetActorLocation TargetActor))
  (bind _returnvalue_3 (Ability|GetAbilitySystemComponent _returnvalue))
  (bind _returnvalue_4 (- _returnvalue_2 Origin))
  (if (<= (Math|Vector|VectorLength _returnvalue_4) Radius)
    (if (>= (Math|Vector|DotProduct Forward (Math|Vector|Normalize _returnvalue_4)) (Math|Trig|Cos(Radians) (Math|Trig|DegreesToRadians (* AngleDegrees 0.5))))
      (Development|PrintString (Utilities|String|Append (Utilities|GetDisplayName TargetActor) "는 타격 안에 있음"))
      (GameplayEffects|ApplyGameplayEffectSpecToTarget _returnvalue_3 (GameplayEffects|MakeOutgoingSpec _returnvalue_3 "/Game/BluePrints/GAS/GameplayEffect/Enemy/Enemy1/GE_DummyAttack.GE_DummyAttack_C" 1.0 (GameplayEffects|MakeEffectContext _returnvalue_3)) (Ability|GetAbilitySystemComponent TargetActor)))))