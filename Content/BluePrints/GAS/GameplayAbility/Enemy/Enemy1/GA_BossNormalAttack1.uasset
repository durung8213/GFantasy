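; Gameplay ability for a boss's first normal attack, which fires a BP_NormalAttack1 projectile at the AI controller's focus actor.
; It plays AM_NormalAttack1 and waits for a Spawn.Skill.Projectile gameplay event on the avatar to time the shot.
; The projectile spawns at the right-hand bone, aimed slightly below the focus actor's location, and receives the shooter's ASC.
; The ability ends when the montage completes, blends out, is interrupted or is cancelled.
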(event Ability|EventActivateAbility
  (bind _returnvalue (Ability|GetAvatarActorfromActorInfo))
  (Development|PrintString "보스 어빌리티 시행" true true "(R=1.000000,G=0.109283,B=0.000000,A=1.000000)")
  (|PlayMontageandWaitProxy "None" "/Game/Characters/Enemy/Enemy3/Animaion/paze1/Attack/AM_NormalAttack1.AM_NormalAttack1" 1.0 "None" true 1.0 0.0 false
    (:then
      (bind _asynctaskproxy (Ability|Async|WaitGameplayEventToActor _returnvalue "(TagName=\"Spawn.Skill.Projectile\")")
        (:EventReceived
          (bind _as캐릭터 (Utilities|Casting|CastToCharacter _returnvalue))
          (Game|SpawnActorfromClass "/Game/BluePrints/Actor/Projectile/Enemy3/BP_NormalAttack1.BP_NormalAttack1_C" (Transformation|GetBoneTransform (Variables|/Script/Engine.Character|GetMesh _as캐릭터) "hand_r" "RTS_World") "Undefined" "MultiplyWithRoot" 0 (Math|Vector|Normalize (- (+ (Transformation|GetActorLocation (Class|AIController|GetFocusActor (AI|GetAIController _returnvalue))) (Math|Vector|MakeVector 0.0 0.0 -1e+02)) (Transformation|GetActorLocation _returnvalue))) 5e+03 5e+03 true false 0 0.0 (.AsGASCBase (Utilities|Casting|CastToGASCBase (Ability|GetAbilitySystemComponent _returnvalue))) 0)
          (Development|PrintString "보스 공격 고체 스폰" true true "(R=1.000000,G=0.000000,B=0.692669,A=1.000000)")
          (Ability|Async|EndAction _asynctaskproxy))))
    (:OnCompleted
      (Ability|EndAbility :!label _label))
    (:OnBlendOut
      (goto _label))
    (:OnInterrupted
      (goto _label))
    (:OnCancelled
      (goto _label))))

(event Ability|EventOnEndAbility
  (params (bWasCancelled :type Boolean))
  (Development|PrintString "보스 일반 공격 어빌리티 종료"))