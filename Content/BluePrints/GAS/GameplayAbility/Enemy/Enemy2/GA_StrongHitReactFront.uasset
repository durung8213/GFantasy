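; GA_StrongHitReactFront is a gameplay ability that plays Enemy2's strong front hit reaction.
; On activation it flags the hit on the AI controller, applies GE_StrongHitReact to the owner and plays the greatsword large-hit montage.
; When the montage completes, is interrupted or is cancelled, it removes the effect by its stored handle and ends.
; OnEndAbility clears the AI controller's hit flag.
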(event Ability|EventActivateAbility
  (Class|BPIAIController|SetHitDoing(Message) (AI|GetAIController (Ability|GetAvatarActorfromActorInfo)) true)
  (bind _returnvalue (Ability|ApplyGameplayEffectToOwner "/Game/BluePrints/GAS/GameplayEffect/Enemy/Enemy2/GE_StrongHitReact.GE_StrongHitReact_C"))
  (Variables|Default|SetActiveGEHitReact _returnvalue)
  (|PlayMontageandWaitProxy "None" "/Game/Characters/Enemy/Enemy2/Animation/Hit/AM_GreatSword_Large_Hit_Montage.AM_GreatSword_Large_Hit_Montage" 1.0 "None" true 1.0 0.0 false
    (:OnCompleted
      _)
    (:OnInterrupted
      _)
    (:OnCancelled
      _))
  (Ability|RemoveGameplayEffectFromOwnerWithHandle (Variables|Default|GetActiveGEHitReact))
  (Ability|EndAbility))

(event Ability|EventOnEndAbility
  (params (bWasCancelled :type Boolean))
  (Class|BPIAIController|SetHitDoing(Message) (AI|GetAIController (Ability|GetAvatarActorfromActorInfo)) false))