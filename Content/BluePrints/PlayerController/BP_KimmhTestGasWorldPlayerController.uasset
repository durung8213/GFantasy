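; Test player controller with debug keys for triggering AI perception stimuli from the controlled pawn.
; L calls ServerMakeNoise to emit a noise at the pawn's location.
; K calls ServerReportDamageEvent to report damage on the BP_TestEnemy found in the world, with the pawn as instigator, without applying damage.
; A separate PlaySequence event creates a player for a given Level Sequence and plays it.
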(event Custom|ServerMakeNoise
  (bind _returnvalue (Pawn|GetControlledPawn))
  (Class|Actor|MakeNoise _returnvalue 1.0 _returnvalue (Transformation|GetActorLocation _returnvalue) 0.0 "None"))

(event Custom|ServerReportDamageEvent
  (bind _returnvalue (Pawn|GetControlledPawn))
  (bind _returnvalue_2 (Transformation|GetActorLocation _returnvalue))
  (bind _returnvalue_3 (Actor|GetActorOfClass "/Game/Characters/Enemy/Enemy2/BP_TestEnemy.BP_TestEnemy_C"))
  (Class|AISenseDamage|ReportDamageEvent _returnvalue_3 _returnvalue 1e+01 _returnvalue_2 _returnvalue_2 "None"))

(event Custom|PlaySequence
  (params (LevelSequence :type Level%20Sequence%20Object%20Reference))
  (bind _returnvalue (Sequencer|Player|CreateLevelSequencePlayer LevelSequence))
  (Sequencer|Player|Play _returnvalue :!class /Script/MovieScene.MovieSceneSequencePlayer))

(event EventBeginPlay)

(event EventTick
  (params (DeltaSeconds :type Float%20%28single-precision%29)))

(event Input|KeyboardEvents|1
  (params (Key :type Key%20Structure :default "None")))

(event Input|KeyboardEvents|L
  (params (Key :type Key%20Structure :default "None"))
  (:Pressed
    (CallFunction|ServerMakeNoise)))

(event Input|KeyboardEvents|K
  (params (Key :type Key%20Structure :default "None"))
  (:Pressed
    (CallFunction|ServerReportDamageEvent)))

(fn ConstructionScript
  (|CallParentFunction))