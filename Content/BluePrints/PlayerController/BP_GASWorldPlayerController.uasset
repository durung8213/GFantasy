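; Player controller for the GAS world character, handling inventory, quest, crafting, enhancement, shop, options menu and character customization UI.
; Per-screen flags drive input mode and cursor, gate opening, and let Escape close open panels before showing the menu.
; Quick-slot keys use inventory items unless matching GameplayCue tags are active, with consumable count changes forwarded to the slot widget.
; Customization branches on authority; debug keys grant items and LevelSequence playback is included.
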(event Custom|ServerCustomizingEnd
  (CallFunction|CustomizingEnd))

(event Custom|CustomizingEnd
  (bind _playercharacterref (Variables|Default|GetPlayerCharacterRef))
  (Networking|SwitchHasAuthority
    (:Authority
      (Default|OFfRPC (Variables|Default|GetPlayerCharacterRef))
      (bind _returnvalue (Actor|GetActorOfClass "/Script/Engine.PlayerStart"))
      (Transformation|Teleport (Variables|Default|GetPlayerCharacterRef) (Transformation|GetActorLocation _returnvalue) (Transformation|GetActorRotation _returnvalue)))
    (:Remote
      (Widget|RemovefromParent (Variables|Default|GetCustomizeWidgetRef))
      (Variables|OnWidget|SetOnCustomizing false)
      (CallFunction|SelectGameMode)
      (if (Pawn|IsLocalController self)
        (Input|RemoveMappingContext (PlayerController|LocalPlayerSubsystems|GetEnhancedInputLocalPlayerSubsystem) "/Game/Controller/PlayerController/Input/IMC/IMC_Customizer.IMC_Customizer" "(bIgnoreAllPressedKeysUntilRelease=True,bForceImmediately=False,bNotifyUserSettings=False)")
        (if (Utilities|IsValid (Variables|/Script/GFantasy.GASPlayerCharacter|GetCurrentWeapon _playercharacterref))
          (Class|GASPlayerCharacter|ApplyIMC _playercharacterref "/Game/Controller/PlayerController/Input/IMC/IMC_UnArmed.IMC_UnArmed")
          (Rendering|SetVisibility (Variables|/Script/GFantasy.WeaponBase|GetWeaponMesh (Variables|/Script/GFantasy.GASPlayerCharacter|GetCurrentWeapon (Variables|Default|GetPlayerCharacterRef))) true false)
          (else
            (Class|GASPlayerCharacter|ApplyIMC _playercharacterref "/Game/Controller/PlayerController/Input/IMC/IMC_UnArmed.IMC_UnArmed")))
        (bind _asworld_hud (Utilities|Casting|CastToWorldHUD (Class|GASPlayerController|GetMyHUD self)))
        (bind _aswbp_player_world_hud (Utilities|Casting|CastToWBP_PlayerWorldHUD (Variables|/Script/GFantasy.WorldHUD|GetPlayerHUD _asworld_hud)))
        (Utilities|IsValid _aswbp_player_world_hud
          (:Is%20Valid
            (Widget|SetVisibility _aswbp_player_world_hud "Visible")))))))

(event Custom|PlaySequence
  (params (LevelSequence :type Level%20Sequence%20Object%20Reference))
  (bind _returnvalue (Sequencer|Player|CreateLevelSequencePlayer LevelSequence))
  (Sequencer|Player|Play _returnvalue :!class /Script/MovieScene.MovieSceneSequencePlayer))

(event Custom|CustomizingStart
  (bind _playercharacterref (Variables|Default|GetPlayerCharacterRef))
  (bind _currentweapon (Variables|/Script/GFantasy.GASPlayerCharacter|GetCurrentWeapon _playercharacterref))
  (Networking|SwitchHasAuthority
    (:Authority
      (Default|RPC (Variables|Default|GetPlayerCharacterRef)))
    (:Remote
      (bind _returnvalue (UserInterface|CreateWidget "/Game/UI/Customizer/WBP_CharacterCustomization.WBP_CharacterCustomization_C" self))
      (bind _output_get (Variables|Default|SetCustomizeWidgetRef _returnvalue))
      (UserInterface|Viewport|AddtoViewport _output_get 0)
      (Variables|OnWidget|SetOnCustomizing true)
      (CallFunction|SelectGameMode)
      (if (Pawn|IsLocalController self)
        (Input|AddMappingContext (PlayerController|LocalPlayerSubsystems|GetEnhancedInputLocalPlayerSubsystem) "/Game/Controller/PlayerController/Input/IMC/IMC_Customizer.IMC_Customizer" 0 "(bIgnoreAllPressedKeysUntilRelease=True,bForceImmediately=False,bNotifyUserSettings=False)")
        (Class|GASPlayerCharacter|ApplyIMC (Variables|Default|GetPlayerCharacterRef) "/Game/Controller/PlayerController/Input/IMC/IMC_Customizer.IMC_Customizer")
        (Utilities|IsValid _currentweapon
          (:Is%20Valid
            (Rendering|SetVisibility (Variables|/Script/GFantasy.WeaponBase|GetWeaponMesh _currentweapon) false false))
          (:Is%20Not%20Valid
            _))
        (bind _asworld_hud (Utilities|Casting|CastToWorldHUD (Class|GASPlayerController|GetMyHUD self)))
        (bind _aswbp_player_world_hud (Utilities|Casting|CastToWBP_PlayerWorldHUD (Variables|/Script/GFantasy.WorldHUD|GetPlayerHUD _asworld_hud)))
        (Utilities|IsValid _aswbp_player_world_hud
          (:Is%20Valid
            (Widget|SetVisibility _aswbp_player_world_hud "Hidden")))))))

(event Custom|ItemCountChanged
  (params (ItemTag :type Gameplay%20Tag%20Structure%20%28by%20ref%29) (ChangeCount :type Integer))
  ;[1 1 1] ItemSlot 수량 바인딩
  (if (GameplayTags|MatchesTag ItemTag "(TagName=\"Item.Consumable\")")
    (CallFunction|OwningItemCountChaged ItemTag ChangeCount)))

(event Custom|ServerCustomizingStart
  (CallFunction|CustomizingStart))

(event Custom|ServerItemCountChaged
  ;[1 1 1] ItemSlot 수량 바인딩
  (EventDispatchers|BindEventtoOnItemCountChanged (Variables|Default|GetInventoryComponent) (delegate Custom|ItemCountChanged)))

(event Custom|OwningItemCountChaged
  (params (ItemTag :type Gameplay%20Tag%20Structure) (ChangeCount :type Integer))
  ;[1 1 1] ItemSlot 수량 바인딩
  (Default|PotionUse (Variables|Default|GetItemSlotWidgetRef) ItemTag ChangeCount))

(event Custom|BindItemSlot
  (params (ItemSlotWidget :type WBP%20Item%20Slot%20Object%20Reference))
  ;[1 1 1] ItemSlot 수량 바인딩
  (Variables|Default|SetItemSlotWidgetRef ItemSlotWidget)
  (CallFunction|ServerItemCountChaged))

(event Input|EnhancedActionEvents|EnhancedInputActionIA_Inventory
  (params (ActionValue :type Boolean) (ElapsedSeconds :type Float%20%28double-precision%29) (TriggeredSeconds :type Float%20%28double-precision%29) (InputAction :type Input%20Action%20Object%20Reference :default "/Game/Controller/PlayerController/Input/IA/Inventory/IA_Inventory.IA_Inventory"))
  (bind _inventorywidget (Variables|Default|GetInventoryWidget))
  ;[1 1 1] 인벤토리
  (bind _playercharacterref (Variables|Default|GetPlayerCharacterRef)
    (:then
      (if (Utilities|Enum|Equal(Enum) (Variables|/Script/GFantasy.GASPlayerCharacter|GetCombatState _playercharacterref) "NonCombat") ; 비전투 상태일때만 인벤토리 사용 가능
        (bind _canwidget (CallFunction|CanonWidget?))
        (if _canwidget
          (if (not (Variables|OnWidget|GetOnInventory))
            (Class|GASWorldPlayerController|CreateInventoryWidget)
            (Variables|OnWidget|SetOnInventory true)
            (CallFunction|SelectGameMode)
            (else
              (Utilities|IsValid _inventorywidget
                (:Is%20Valid
                  (Widget|RemovefromParent _inventorywidget)
                  (Variables|OnWidget|SetOnInventory false)
                  (CallFunction|SelectGameMode))))))))
    (:else)))

(event EventSelectInputModewhenUIOnly
  (CallFunction|CanonWidget?)
  (CallFunction|SelectGameMode))

(event EventBeginPlay
  ;[1 1 1] BeginPlay, OnPossess
  (Class|InventoryComponent|AddItem (Variables|Default|GetInventoryComponent) (Variables|Default|GetCash) 0)
  (bind _asbp_gasplayer_character (Utilities|Casting|CastToBP_GASPlayerCharacter (Pawn|GetControlledPawn)))
  (Variables|Default|SetPlayerCharacterRef _asbp_gasplayer_character))

(event EventPossess
  (params (PossessedPawn :type Pawn%20Object%20Reference))
  ;[1 1 1] BeginPlay, OnPossess
  (bind _asbp_gasplayer_character (Utilities|Casting|CastToBP_GASPlayerCharacter (Pawn|GetControlledPawn)))
  (Variables|Default|SetPlayerCharacterRef _asbp_gasplayer_character))

(event Input|KeyboardEvents|1
  (params (Key :type Key%20Structure :default "None"))
  ;[1 1 1] ItemSlot 사용
  (:Pressed
    (bind _returnvalue (Class|InventoryComponent|GetInventoryEntries (Variables|Default|GetInventoryComponent)))
    (for _array_element _returnvalue
      (if (GameplayTags|MatchesTag (Utilities|Struct|BreakGFInventoryEntry _array_element) (Variables|Default|GetQuikSlot1) true)
        (if (not (GameplayTags|HasMatchingGameplayTag (Ability|GetAbilitySystemComponent (Variables|Default|GetPlayerCharacterRef)) "(TagName=\"GameplayCue.Heal\")"))
          (Class|InventoryComponent|UseItem (Variables|Default|GetInventoryComponent) _array_element 1))))))

(event Input|KeyboardEvents|U
  (params (Key :type Key%20Structure :default "None"))
  ;[1 1 1] 퀘스트
  (:Pressed
    (bind _asworld_hud (Utilities|Casting|CastToWorldHUD (HUD|GetHUD)))
    (bind _aswbp_player_world_hud (Utilities|Casting|CastToWBP_PlayerWorldHUD (Variables|/Script/GFantasy.WorldHUD|GetPlayerHUD _asworld_hud)))
    (bind _canwidget (CallFunction|CanonWidget?))
    (if _canwidget
      (if (not (Variables|OnWidget|GetOnQuest))
        (Widget|SetVisibility (Variables|/Script/GFantasy.PlayerHUD|GetWBP_QuestList _aswbp_player_world_hud) "Visible")
        (Variables|OnWidget|SetOnQuest true)
        (CallFunction|SelectGameMode)
        (else
          (Widget|SetVisibility (Variables|/Script/GFantasy.PlayerHUD|GetWBP_QuestList _aswbp_player_world_hud) "Hidden")
          (Variables|OnWidget|SetOnQuest false)
          (CallFunction|SelectGameMode))))))

(event Input|KeyboardEvents|2
  (params (Key :type Key%20Structure :default "None"))
  ;[1 1 1] ItemSlot 사용
  (:Pressed
    (bind _returnvalue (Class|InventoryComponent|GetInventoryEntries (Variables|Default|GetInventoryComponent)))
    (for _array_element _returnvalue
      (if (GameplayTags|MatchesTag (Utilities|Struct|BreakGFInventoryEntry _array_element) "(TagName=\"Item.Consumable.AtkPotion\")" true)
        (if (not (GameplayTags|HasMatchingGameplayTag (Ability|GetAbilitySystemComponent (Variables|Default|GetPlayerCharacterRef)) "(TagName=\"GameplayCue.Buff.AtkUp\")"))
          (Class|InventoryComponent|UseItem (Variables|Default|GetInventoryComponent) _array_element 1))))))

(event Input|KeyboardEvents|Escape
  (params (Key :type Key%20Structure :default "None"))
  ;[1 1 1] 옵션
  (:Pressed
    (bind _canmenu_ (CallFunction|OffUI))
    (if _canmenu_
      (if (not (Variables|OnWidget|GetOnMenu))
        (bind _returnvalue (UserInterface|CreateWidget "/Game/UI/World/WBP_Menu.WBP_Menu_C" self))
        (bind _output_get (Variables|Default|SetWBP_MenuWidget _returnvalue))
        (UserInterface|Viewport|AddtoViewport _output_get 0)
        (Variables|OnWidget|SetOnMenu true)
        (CallFunction|SelectGameMode)
        (else
          (Utilities|IsValid (Variables|Default|GetWBP_MenuWidget)
            (:Is%20Valid
              (Widget|RemovefromParent (Variables|Default|GetWBP_MenuWidget))
              (bind _asbp_world_hud (Utilities|Casting|CastToBP_WorldHUD (HUD|GetHUD)))
              (Default|CloseOption _asbp_world_hud)
              (Default|CloseDescription _asbp_world_hud)
              (Variables|OnWidget|SetOnMenu false)
              (CallFunction|SelectGameMode)))))
      (else
        (CallFunction|SelectGameMode)))))

(event Input|KeyboardEvents|0
  (params (Key :type Key%20Structure :default "None"))
  ;[1 1 1] 옵션
  (:Pressed
    (bind _canmenu_ (CallFunction|OffUI))
    (if _canmenu_
      (if (not (Variables|OnWidget|GetOnMenu))
        (bind _returnvalue (UserInterface|CreateWidget "/Game/UI/World/WBP_Menu.WBP_Menu_C" self))
        (bind _output_get (Variables|Default|SetWBP_MenuWidget _returnvalue))
        (UserInterface|Viewport|AddtoViewport _output_get 0)
        (Variables|OnWidget|SetOnMenu true)
        (CallFunction|SelectGameMode)
        (else
          (Utilities|IsValid (Variables|Default|GetWBP_MenuWidget)
            (:Is%20Valid
              (Widget|RemovefromParent (Variables|Default|GetWBP_MenuWidget))
              (bind _asbp_world_hud (Utilities|Casting|CastToBP_WorldHUD (HUD|GetHUD)))
              (Default|CloseOption _asbp_world_hud)
              (Default|CloseDescription _asbp_world_hud)
              (Variables|OnWidget|SetOnMenu false)
              (CallFunction|SelectGameMode)))))
      (else
        (CallFunction|SelectGameMode)))))

(event Input|KeyboardEvents|7
  (params (Key :type Key%20Structure :default "None"))
  ;[1 1 1] 디버그용 아이템 획득
  (:Pressed
    (Class|InventoryComponent|AddItem (Variables|Default|GetInventoryComponent) (GameplayTags|MakeLiteralGameplayTag "(TagName=\"Item.Material.Misc.Gift\")") 1)))

(event Input|KeyboardEvents|8
  (params (Key :type Key%20Structure :default "None"))
  ;[1 1 1] 디버그용 아이템 획득
  (:Pressed
    (Class|InventoryComponent|AddItem (Variables|Default|GetInventoryComponent) (.OutItem (Utilities|Array|Random (Variables|Debug|GetCraftRecipe))) 1)))

(event Input|KeyboardEvents|9
  (params (Key :type Key%20Structure :default "None"))
  ;[1 1 1] 디버그용 아이템 획득
  (:Pressed
    (Class|InventoryComponent|AddItem (Variables|Default|GetInventoryComponent) (.OutItem (Utilities|Array|Random (Variables|Debug|GetTestMaterials))) 1)))

(fn ConstructionScript)

(fn CanonWidget?
  (if (Math|Boolean|ORBoolean (Variables|OnWidget|GetOnCraft) (Variables|OnWidget|GetOnEnhanced) (Variables|OnWidget|GetOnShop) (Variables|OnWidget|GetOnCustomizing) (Variables|OnWidget|GetOnMenu))
    (Variables|OnWidget|SetOnWidget true)
    (else
      (Variables|OnWidget|SetOnWidget false)))
  (return (not (Variables|OnWidget|GetOnWidget))))

(fn SetGameandUIMode
  (bind _self self)
  (Input|SetInputModeGameandUI _self 0 "DoNotLock" true false)
  (Variables|Default|SetbShowMouseCursor _self true))

(fn SetUIOnlyMode
  (bind _self self)
  (Input|SetInputModeUIOnly _self 0 "DoNotLock" false)
  (Variables|Default|SetbShowMouseCursor _self true))

(fn SelectGameMode
  (if (Math|Boolean|ORBoolean (Variables|OnWidget|GetOnInventory) (Variables|OnWidget|GetOnQuest) (Variables|OnWidget|GetOnCraft) (Variables|OnWidget|GetOnEnhanced) (Variables|OnWidget|GetOnMenu) (Variables|OnWidget|GetOnCustomizing) (Variables|OnWidget|GetOnShop))
    (CallFunction|SetGameandUIMode)
    (else
      (CallFunction|SetGameOnlyMode))))

(fn SetGameOnlyMode
  (bind _self self)
  (Input|SetInputModeGameOnly _self false)
  (Variables|Default|SetbShowMouseCursor _self false))

(fn OnCraftWidget
  (params (OnWidget :type Boolean))
  (bind _craftwidget (Variables|Default|GetCraftWidget))
  (bind _inventorywidget (Variables|Default|GetInventoryWidget))
  (if OnWidget
    (Class|GASWorldPlayerController|CreateInventoryWidget)
    (Class|GASWorldPlayerController|CreateCraftWidget)
    (Variables|OnWidget|SetOnCraft true)
    (CallFunction|SelectGameMode)
    (Class|GASWorldPlayerController|ClientSwitchInteractionIMC true)
    (else
      (Utilities|IsValid _craftwidget
        (:Is%20Valid
          (Widget|RemovefromParent _craftwidget)
          (Utilities|IsValid _inventorywidget
            (:Is%20Valid
              (Widget|RemovefromParent _inventorywidget)
              (Variables|OnWidget|SetOnCraft false)
              (CallFunction|SelectGameMode)
              (Class|GASWorldPlayerController|ClientSwitchInteractionIMC false))))))))

(fn OnEnhancedWidget
  (params (OnWidget :type Boolean))
  (bind _inventorywidget (Variables|Default|GetInventoryWidget))
  (bind _enhancedwidget (Variables|Default|GetEnhancedWidget))
  (if OnWidget
    (Class|GASWorldPlayerController|CreateInventoryWidget)
    (Class|GASWorldPlayerController|CreateEnhancedWidget)
    (Variables|OnWidget|SetOnEnhanced true)
    (CallFunction|SelectGameMode)
    (Class|GASWorldPlayerController|ClientSwitchInteractionIMC true)
    (else
      (Utilities|IsValid _enhancedwidget
        (:Is%20Valid
          (Widget|RemovefromParent _enhancedwidget)
          (Utilities|IsValid _inventorywidget
            (:Is%20Valid
              (Widget|RemovefromParent _inventorywidget)
              (Variables|OnWidget|SetOnEnhanced false)
              (CallFunction|SelectGameMode)
              (Class|GASWorldPlayerController|ClientSwitchInteractionIMC false))))))))

(fn OnShopWidget
  (params (OnWidget :type Boolean))
  (bind _inventorywidget (Variables|Default|GetInventoryWidget))
  (if OnWidget
    (Class|GASWorldPlayerController|CreateInventoryWidget)
    (bind _returnvalue (UserInterface|CreateWidget "/Game/UI/Shop/WBP_Shop.WBP_Shop_C" self))
    (bind _output_get (Variables|Default|SetShowWidgetRef _returnvalue))
    (UserInterface|Viewport|AddtoViewport _output_get 0)
    (bind _output_get_2 (Variables|OnWidget|SetOnShop true))
    (Class|GASWorldPlayerController|ClientSwitchInteractionIMC _output_get_2)
    (else
      (Utilities|IsValid (Variables|Default|GetShowWidgetRef)
        (:Is%20Valid
          (Widget|RemovefromParent (Variables|Default|GetShowWidgetRef))
          (Utilities|IsValid _inventorywidget
            (:Is%20Valid
              (Widget|RemovefromParent _inventorywidget)
              (bind _output_get_3 (Variables|OnWidget|SetOnShop false))
              (CallFunction|SelectGameMode)
              (Class|GASWorldPlayerController|ClientSwitchInteractionIMC _output_get_3))))))))

(fn OffUI
  (bind _inventorywidget (Variables|Default|GetInventoryWidget))
  (if (Math|Boolean|ORBoolean (Variables|OnWidget|GetOnInventory) (Variables|OnWidget|GetOnQuest) (Variables|OnWidget|GetOnCraft) (Variables|OnWidget|GetOnEnhanced) (Variables|OnWidget|GetOnCustomizing) (Variables|OnWidget|GetOnShop))
    (Utilities|FlowControl|Sequence
      (:then_0
        (if (Variables|OnWidget|GetOnInventory)
          (Utilities|IsValid _inventorywidget
            (:Is%20Valid
              (Widget|RemovefromParent _inventorywidget)
              (Variables|OnWidget|SetOnInventory false)))))
      (:then_1
        (if (Variables|OnWidget|GetOnQuest)
          (bind _asworld_hud (Utilities|Casting|CastToWorldHUD (HUD|GetHUD)))
          (bind _aswbp_player_world_hud (Utilities|Casting|CastToWBP_PlayerWorldHUD (Variables|/Script/GFantasy.WorldHUD|GetPlayerHUD _asworld_hud)))
          (Widget|SetVisibility (Variables|/Script/GFantasy.PlayerHUD|GetWBP_QuestList _aswbp_player_world_hud) "Hidden")
          (Variables|OnWidget|SetOnQuest false)))
      (:then_2
        (if (Variables|OnWidget|GetOnCraft)
          (CallFunction|OnCraftWidget false)))
      (:then_3
        (if (Variables|OnWidget|GetOnEnhanced)
          (CallFunction|OnEnhancedWidget false)))
      (:then_4
        (if (Variables|OnWidget|GetOnShop)
          (CallFunction|OnShopWidget false)
          (return false))))
    (else
      (return true))))