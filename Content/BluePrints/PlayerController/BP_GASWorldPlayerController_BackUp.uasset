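; Player controller Blueprint (named as a backup) that handles UI hotkeys for inventory, quest list, description and menu widgets, and closes craft and enhancement widgets.
; Number keys use the first quick-slot item or add random equipment, materials and recipes through the InventoryComponent.
; Per-widget flags feed CheckUIOn, which switches cursor and input mode, though it checks only inventory, quest and craft.
; A PlaySequence event also plays a given level sequence.
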(event Custom|PlaySequence
  (params (LevelSequence :type Level%20Sequence%20Object%20Reference))
  (bind _returnvalue (Sequencer|Player|CreateLevelSequencePlayer LevelSequence))
  (Sequencer|Player|Play _returnvalue :!class /Script/MovieScene.MovieSceneSequencePlayer))

(event EventSelectInputModewhenUIOnly
  (CallFunction|CheckUIon))

(event Input|KeyboardEvents|1
  (params (Key :type Key%20Structure :default "None"))
  (:Pressed
    (bind _returnvalue (Class|InventoryComponent|GetInventoryEntries (Variables|Default|GetInventoryComponent)))
    (for _array_element _returnvalue
      (if (GameplayTags|MatchesTag (Utilities|Struct|BreakGFInventoryEntry _array_element) (Variables|Default|GetQuikSlot1) true)
        (Class|InventoryComponent|UseItem (Variables|Default|GetInventoryComponent) _array_element 1)))))

(event Input|KeyboardEvents|U
  (params (Key :type Key%20Structure :default "None"))
  (:Pressed
    (bind _asworld_hud (Utilities|Casting|CastToWorldHUD (HUD|GetHUD)))
    (bind _aswbp_player_world_hud (Utilities|Casting|CastToWBP_PlayerWorldHUD (Variables|/Script/GFantasy.WorldHUD|GetPlayerHUD _asworld_hud)))
    (Utilities|FlowControl|FlipFlop
      (:A
        (Widget|SetVisibility (Variables|/Script/GFantasy.PlayerHUD|GetWBP_QuestList _aswbp_player_world_hud) "Visible")
        (CallFunction|SetUIandGameMode)
        (Variables|Default|SetOnQuest true))
      (:B
        (Widget|SetVisibility (Variables|/Script/GFantasy.PlayerHUD|GetWBP_QuestList _aswbp_player_world_hud) "Hidden")
        (Variables|Default|SetOnQuest false)
        (CallFunction|CheckUIon)))))

(event Input|KeyboardEvents|B
  (params (Key :type Key%20Structure :default "None"))
  ;[1 1 1] 강화
  (:Pressed
    (CallFunction|OnEnhancedWidget false)))

(event Input|KeyboardEvents|I
  (params (Key :type Key%20Structure :default "None"))
  (bind _inventorywidget (Variables|Default|GetInventoryWidget))
  (:Pressed
    (if (not (Variables|Default|GetOnEnhanced))
      (if (Variables|Default|GetOnInventory)
        (Utilities|IsValid _inventorywidget
          (:Is%20Valid
            (Widget|RemovefromParent _inventorywidget)
            (Variables|Default|SetOnInventory false)
            (CallFunction|CheckUIon)))
        (else
          (Class|GASWorldPlayerController|CreateInventoryWidget)
          (Variables|Default|SetbShowMouseCursor true)
          (Input|SetInputModeGameandUI self 0 "DoNotLock" true false)
          (Variables|Default|SetOnInventory true))))))

(event Input|KeyboardEvents|Escape
  (params (Key :type Key%20Structure :default "None"))
  ;[1 1 1] 옵션
  (:Pressed
    (if (Variables|Default|GetAllUIOff)
      (Utilities|FlowControl|FlipFlop
        (:A
          (bind _returnvalue (UserInterface|CreateWidget "/Game/UI/World/WBP_Menu.WBP_Menu_C" self))
          (bind _output_get (Variables|Default|SetWBP_MenuWidget _returnvalue))
          (UserInterface|Viewport|AddtoViewport _output_get 0)
          (CallFunction|SetUIandGameMode)
          (Variables|Default|SetOnMenu true))
        (:B
          (Utilities|IsValid (Variables|Default|GetWBP_MenuWidget)
            (:Is%20Valid
              (Widget|RemovefromParent (Variables|Default|GetWBP_MenuWidget))
              (Variables|Default|SetOnMenu false)
              (CallFunction|CheckUIon)))))
      (else
        (CallFunction|OnCraftWidget false)
        (CallFunction|OnEnhancedWidget false)))))

(event Input|KeyboardEvents|H
  (params (Key :type Key%20Structure :default "None"))
  ;[1 1 1] 설명서
  (:Pressed
    (Utilities|FlowControl|FlipFlop
      (:A
        (bind _returnvalue (UserInterface|CreateWidget "/Game/UI/Title/WBP_Description.WBP_Description_C" self))
        (bind _output_get (Variables|Default|SetWBP_DescriptionWidget _returnvalue))
        (UserInterface|Viewport|AddtoViewport _output_get 0)
        (CallFunction|SetUIOnlyMode)
        (Variables|Default|SetOnDescription true))
      (:B
        (Utilities|IsValid (Variables|Default|GetWBP_DescriptionWidget)
          (:Is%20Valid
            (Widget|RemovefromParent (Variables|Default|GetWBP_DescriptionWidget))
            (Variables|Default|SetOnDescription false)
            (CallFunction|CheckUIon)))))))

(event Input|KeyboardEvents|C
  (params (Key :type Key%20Structure :default "None"))
  ;[1 1 1] 제작
  (:Pressed
    (CallFunction|OnCraftWidget false)))

(event Input|KeyboardEvents|0
  (params (Key :type Key%20Structure :default "None"))
  ;[1 1 1] 옵션
  (:Pressed
    (if (Variables|Default|GetAllUIOff)
      (Utilities|FlowControl|FlipFlop
        (:A
          (bind _returnvalue (UserInterface|CreateWidget "/Game/UI/World/WBP_Menu.WBP_Menu_C" self))
          (bind _output_get (Variables|Default|SetWBP_MenuWidget _returnvalue))
          (UserInterface|Viewport|AddtoViewport _output_get 0)
          (CallFunction|SetUIandGameMode)
          (Variables|Default|SetOnMenu true))
        (:B
          (Utilities|IsValid (Variables|Default|GetWBP_MenuWidget)
            (:Is%20Valid
              (Widget|RemovefromParent (Variables|Default|GetWBP_MenuWidget))
              (Variables|Default|SetOnMenu false)
              (CallFunction|CheckUIon)))))
      (else
        (CallFunction|OnCraftWidget false)
        (CallFunction|OnEnhancedWidget false)))))

(event Input|KeyboardEvents|7
  (params (Key :type Key%20Structure :default "None"))
  (:Pressed
    (Class|InventoryComponent|AddItem (Variables|Default|GetInventoryComponent) (.OutItem (Utilities|Array|Random (Variables|Default|GetEquipmentItems))) 1)))

(event Input|KeyboardEvents|8
  (params (Key :type Key%20Structure :default "None"))
  (:Pressed
    (Class|InventoryComponent|AddItem (Variables|Default|GetInventoryComponent) (.OutItem (Utilities|Array|Random (Variables|Default|GetCraftRecipe))) 1)))

(event Input|KeyboardEvents|9
  (params (Key :type Key%20Structure :default "None"))
  (:Pressed
    (Class|InventoryComponent|AddItem (Variables|Default|GetInventoryComponent) (.OutItem (Utilities|Array|Random (Variables|Default|GetTestMaterials))) 1)))

(fn ConstructionScript)

(fn CheckUIon
  (if (Math|Boolean|ORBoolean (Variables|Default|GetOnInventory) (Variables|Default|GetOnQuest) (Variables|Default|GetOnCraft))
    (Variables|Default|SetAllUIOff false)
    (else
      (Variables|Default|SetAllUIOff true)))
  (CallFunction|SelectGameMode))

(fn SetUIandGameMode
  (bind _self self)
  (Input|SetInputModeGameandUI _self 0 "DoNotLock" true false)
  (Variables|Default|SetbShowMouseCursor _self true))

(fn SetUIOnlyMode
  (bind _self self)
  (Input|SetInputModeUIOnly _self 0 "DoNotLock" false)
  (Variables|Default|SetbShowMouseCursor _self true))

(fn SelectGameMode
  (if (Variables|Default|GetAllUIOff)
    (CallFunction|SetGameOnlyMode)
    (else
      (CallFunction|SetUIandGameMode))))

(fn SetGameOnlyMode
  (bind _self self)
  (Input|SetInputModeGameOnly _self false)
  (Variables|Default|SetbShowMouseCursor _self false))

(fn OnCraftWidget
  (params (OnWidget :type Boolean))
  (bind _craftwidget (Variables|Default|GetCraftWidget))
  (if OnWidget
    (Class|GASWorldPlayerController|CreateCraftWidget)
    (Variables|Default|SetbShowMouseCursor false)
    (Input|SetInputModeGameandUI self 0 "DoNotLock" true false)
    (Variables|Default|SetOnCraft true)
    (else
      (Utilities|IsValid _craftwidget
        (:Is%20Valid
          (Widget|RemovefromParent _craftwidget)
          (Variables|Default|SetOnCraft false)
          (CallFunction|CheckUIon))))))

(fn OnEnhancedWidget
  (params (OnWidget :type Boolean))
  (if OnWidget
    (if (Variables|Default|GetOnInventory)
      (Class|GASWorldPlayerController|CreateEnhancedWidget)
      (Variables|Default|SetOnEnhanced true)
      (else
        (Class|GASWorldPlayerController|CreateInventoryWidget)
        (Class|GASWorldPlayerController|CreateEnhancedWidget)
        (Variables|Default|SetbShowMouseCursor true)
        (Input|SetInputModeGameandUI self 0 "DoNotLock" true false)
        (Variables|Default|SetOnEnhanced true)
        (Variables|Default|SetOnInventory true)))
    (elif (Variables|Default|GetOnInventory)
      (Widget|RemovefromParent (Variables|Default|GetEnhancedWidget))
      (Widget|RemovefromParent (Variables|Default|GetInventoryWidget))
      (Variables|Default|SetOnEnhanced false)
      (Variables|Default|SetOnInventory false)
      (CallFunction|CheckUIon)
      (else
        (Widget|RemovefromParent (Variables|Default|GetEnhancedWidget))
        (Variables|Default|SetOnEnhanced false)
        (CallFunction|CheckUIon)))))