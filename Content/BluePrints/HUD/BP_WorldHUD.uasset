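; BP_WorldHUD is a Blueprint that opens and closes the options and description UI screens.
; OpenOption and OpenDescription each create a widget for player controller 0, store it and add it to the viewport.
; CloseOption and CloseDescription remove the stored widget from its parent after a validity check.
; The event graph holds no logic, so these functions run only when called from elsewhere.
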(event EventBeginPlay)

(event Collision|EventActorBeginOverlap
  (params (OtherActor :type Actor%20Object%20Reference)))

(event EventTick
  (params (DeltaSeconds :type Float%20%28single-precision%29)))

(fn ConstructionScript)

(fn OpenOption
  (bind _returnvalue (UserInterface|CreateWidget "/Game/UI/World/WBP_Option.WBP_Option_C" (Game|GetPlayerController 0)))
  (bind _output_get (Variables|Default|SetWBP_Option _returnvalue))
  (UserInterface|Viewport|AddtoViewport _output_get 0))

(fn CloseOption
  (bind _wbp_option (Variables|Default|GetWBP_Option))
  (Utilities|IsValid _wbp_option
    (:Is%20Valid
      (Widget|RemovefromParent _wbp_option))))

(fn OpenDescription
  (bind _returnvalue (UserInterface|CreateWidget "/Game/UI/Title/WBP_Description.WBP_Description_C" (Game|GetPlayerController 0)))
  (bind _output_get (Variables|Default|SetWBP_Desc _returnvalue))
  (UserInterface|Viewport|AddtoViewport _output_get 0))

(fn CloseDescription
  (bind _wbp_desc (Variables|Default|GetWBP_Desc))
  (Utilities|IsValid _wbp_desc
    (:Is%20Valid
      (Widget|RemovefromParent _wbp_desc))))