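; Succubus AI weapon actor that handles hit detection and a dissolve effect on its scythe mesh.
; HitCollision overlaps pass the other actor to OnBeginOverlap only on the network authority.
; WeaponVisible plays a timeline that drives DissolveAmount on a dynamic material instance, while HideWeapon sets that parameter straight to fully dissolved.
; Both events create and cache the material instance when none is valid.
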(event OnComponentBeginOverlap(HitCollision)
  (params (OverlappedComponent :type Primitive%20Component%20Object%20Reference) (OtherActor :type Actor%20Object%20Reference) (OtherComp :type Primitive%20Component%20Object%20Reference) (OtherBodyIndex :type Integer) (bFromSweep :type Boolean) (SweepResult :type Hit%20Result%20Structure%20%28by%20ref%29))
  (Networking|SwitchHasAuthority
    (:Authority
      (Class|BaseWeapon|OnBeginOverlap OtherActor))))

(event Custom|WeaponVisible
  (Utilities|IsValid (Variables|Default|GetWeaponDynamicInstance)
    (:Is%20Valid
      (bind _dissolvetime (Timeline|WeaponDissolveTimeline PlayFromStart)
        (:Update
          (Rendering|Material|SetScalarParameterValue (Variables|Default|GetWeaponDynamicInstance) "DissolveAmount" _dissolvetime :!class /Script/Engine.MaterialInstanceDynamic))))
    (:Is%20Not%20Valid
      (bind _returnvalue (Rendering|Material|CreateDynamicMaterialInstance (Variables|Default|GetWeaponMesh) 0 "/Game/Asset/Character/Cosmo_Succubus/Materials/Clothes/Scythe/MI_CSG_Scythe_05.MI_CSG_Scythe_05" "None" :!class /Script/Engine.PrimitiveComponent))
      (Variables|Default|SetWeaponDynamicInstance _returnvalue)
      (Timeline|WeaponDissolveTimeline PlayFromStart))))

(event Custom|HideWeapon
  (Utilities|IsValid (Variables|Default|GetWeaponDynamicInstance)
    (:Is%20Valid
      _)
    (:Is%20Not%20Valid
      (bind _returnvalue (Rendering|Material|CreateDynamicMaterialInstance (Variables|Default|GetWeaponMesh) 0 "/Game/Asset/Character/Cosmo_Succubus/Materials/Clothes/Scythe/MI_CSG_Scythe_05.MI_CSG_Scythe_05" "None" :!class /Script/Engine.PrimitiveComponent))
      (Variables|Default|SetWeaponDynamicInstance _returnvalue)))
  (Rendering|Material|SetScalarParameterValue (Variables|Default|GetWeaponDynamicInstance) "DissolveAmount" 1.0 :!class /Script/Engine.MaterialInstanceDynamic))

(event EventBeginPlay)

(event Collision|EventActorBeginOverlap
  (params (OtherActor :type Actor%20Object%20Reference)))

(event EventTick
  (params (DeltaSeconds :type Float%20%28single-precision%29)))

(fn ConstructionScript)