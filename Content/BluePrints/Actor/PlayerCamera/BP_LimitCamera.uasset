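; Camera actor that plays a scripted camera move, apparently for a Limit Break sequence.
; InitializeCameraPosition turns it to face TargetActor.
; StartTimeLine chains three timelines with delays: a yaw sweep from CachedRotation, which this graph never sets, then two world-space position offsets lerped from cached locations.
; A Limit Break camera shake plays on player controller 0 before the final move.
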(event EventBeginPlay)

(event Collision|EventActorBeginOverlap
  (params (OtherActor :type Actor%20Object%20Reference)))

(event EventTick
  (params (DeltaSeconds :type Float%20%28single-precision%29)))

(event EventInitializeCameraPosition
  (bind _targetactor (Variables|Default|GetTargetActor)
    (:then
      (Transformation|SetActorRotation (Math|Rotator|FindLookatRotation (Transformation|GetActorLocation) (Transformation|GetActorLocation _targetactor))))
    (:else)))

(event EventStartTimeLine
  (bind _cachedrotation (Variables|Default|GetCachedRotation))
  (bind _newtrack_0 (Timeline|LimitBreakTL_01 Play)
    (:Update
      (Transformation|SetActorRotation (Math|Rotator|Lerp(Rotator) (Variables|Default|GetCachedRotation) (Math|Rotator|MakeRotator (.roll _cachedrotation) (.pitch _cachedrotation) (+ (.yaw _cachedrotation) -3e+02)) _newtrack_0)))
    (:Finished
      (Variables|Default|SetCachedRotation_02 (Transformation|GetActorRotation))
      (Utilities|FlowControl|Delay 0.15)
      (Variables|Default|SetCachedLocation_01 (Transformation|GetActorLocation))
      (bind _newtrack_0_2 (Timeline|Timeline Play)
        (:Update
          (Transformation|SetActorLocation (Math|Vector|Lerp(Vector) (Variables|Default|GetCachedLocation_01) (- (Variables|Default|GetCachedLocation_01) "30.000000,200.000000,-80.000000") _newtrack_0_2) false false))
        (:Finished
          (Utilities|FlowControl|Delay 2.4)
          (Class|LimitBreakCamera|StartCameraShake)
          (Variables|Default|SetNewVar (Transformation|GetActorLocation))
          (Utilities|FlowControl|Delay 0.6)
          (bind _newtrack_0_3 (Timeline|Timeline_0 Play)
            (:Update
              (Transformation|SetActorLocation (Math|Vector|Lerp(Vector) (Variables|Default|GetNewVar) (- (Variables|Default|GetNewVar) "50.000000,50.000000,0.000000") _newtrack_0_3) false false))))))))

(event EventStartCameraShake
  (bind _returnvalue (Game|GetPlayerController 0))
  (Utilities|IsValid _returnvalue
    (:Is%20Valid
      (Game|Feedback|ClientStartCameraShake _returnvalue "/Game/BluePrints/Combat/PlayerSkill/Camera/BP_CS_LimitBreak.BP_CS_LimitBreak_C" 0.8 "CameraLocal" "0, 0, 0"))))

(fn ConstructionScript)

(fn NewFunction)