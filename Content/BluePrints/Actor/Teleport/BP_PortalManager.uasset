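; BP_PortalManager is a two-way portal actor that moves player characters between Tp1 and Tp2 if they carry the required item.
; Each collision's overlap calls TpPlayer with the other end's location, which acts only on authority for BP_GASPlayerCharacter.
; Players not in TpUsePlayerArr go through AddPlayer before FindItem searches their controller's inventory for the PortalRequireItem tag, and a match moves them without sweep.
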(event OnComponentBeginOverlap(Tp1Collision)
  (params (OverlappedComponent :type Primitive%20Component%20Object%20Reference) (OtherActor :type Actor%20Object%20Reference) (OtherComp :type Primitive%20Component%20Object%20Reference) (OtherBodyIndex :type Integer) (bFromSweep :type Boolean) (SweepResult :type Hit%20Result%20Structure%20%28by%20ref%29))
  (CallFunction|TpPlayer OtherActor (Transformation|GetWorldLocation (Variables|Default|GetTp2))))

(event OnComponentBeginOverlap(Tp2Collision)
  (params (OverlappedComponent :type Primitive%20Component%20Object%20Reference) (OtherActor :type Actor%20Object%20Reference) (OtherComp :type Primitive%20Component%20Object%20Reference) (OtherBodyIndex :type Integer) (bFromSweep :type Boolean) (SweepResult :type Hit%20Result%20Structure%20%28by%20ref%29))
  (CallFunction|TpPlayer OtherActor (Transformation|GetWorldLocation (Variables|Default|GetTp1))))

(event EventBeginPlay)

(event Collision|EventActorBeginOverlap
  (params (OtherActor :type Actor%20Object%20Reference)))

(event EventTick
  (params (DeltaSeconds :type Float%20%28single-precision%29)))

(fn ConstructionScript)

(fn FindItem
  (params (ItemTag :type Gameplay%20Tag%20Structure) (타깃 :type Inventory%20Component%20Object%20Reference))
  (bind _returnvalue (Class|InventoryComponent|GetInventoryEntries 타깃))
  (bind _array_element (Utilities|Array|ForEachLoopwithBreak _returnvalue :!label _label)
    (:LoopBody
      (if (== (.ItemTag (Utilities|Struct|BreakGFInventoryEntry _array_element)) ItemTag)
        (LocalVariables|SetbIsFindItem true)
        (goto _label Break)))
    (:Completed
      (return (LocalVariables|GetbIsFindItem)))))

(fn TpPlayer
  (params (Actor :type Actor%20Object%20Reference) (TpLocation :type Vector))
  (Networking|SwitchHasAuthority
    (:Authority
      (bind _asbp_gasplayer_character (Utilities|Casting|CastToBP_GASPlayerCharacter Actor))
      (if (not (Utilities|Array|ContainsItem (Variables|Default|GetTpUsePlayerArr) _asbp_gasplayer_character))
        (Class|PortalBase|AddPlayer _asbp_gasplayer_character)
        (bind _returnvalue (Class|InventoryInterface|GetInventoryComponent(Message) (Pawn|GetController _asbp_gasplayer_character)))
        (Utilities|IsValid _returnvalue
          (:Is%20Valid
            (bind _bfinditem (CallFunction|FindItem (Variables|Default|GetPortalRequireItem) _returnvalue))
            (if _bfinditem
              (Transformation|SetActorLocation _asbp_gasplayer_character TpLocation false false))))))))