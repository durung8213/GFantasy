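; BP_CustomizeTeleportStart is a teleport trigger that sends a player into character customization.
; On BeginPlay it caches the BP_CustomizeTeleportEnd actor found in the level.
; When a BP_GASPlayerCharacter overlaps its box, the server calls ServerCustomizingStart on that player's world controller, then teleports the character to the end actor's location and rotation.
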(event OnComponentBeginOverlap(Box)
  (params (OverlappedComponent :type Primitive%20Component%20Object%20Reference) (OtherActor :type Actor%20Object%20Reference) (OtherComp :type Primitive%20Component%20Object%20Reference) (OtherBodyIndex :type Integer) (bFromSweep :type Boolean) (SweepResult :type Hit%20Result%20Structure%20%28by%20ref%29))
  (bind _bpend (Variables|Default|GetBPEnd))
  (Networking|SwitchHasAuthority
    (:Authority
      (bind _asbp_gasplayer_character (Utilities|Casting|CastToBP_GASPlayerCharacter OtherActor))
      (bind _asbp_gasworld_player_controller (Utilities|Casting|CastToBP_GASWorldPlayerController (Pawn|GetController _asbp_gasplayer_character)))
      (Default|ServerCustomizingStart _asbp_gasworld_player_controller)
      (Transformation|Teleport _asbp_gasplayer_character (Transformation|GetActorLocation _bpend) (Transformation|GetActorRotation _bpend)))))

(event EventBeginPlay
  (bind _returnvalue (Actor|GetActorOfClass "/Game/BluePrints/Actor/Teleport/BP_CustomizeTeleportEnd.BP_CustomizeTeleportEnd_C"))
  (Variables|Default|SetBPEnd _returnvalue))

(event Collision|EventActorBeginOverlap
  (params (OtherActor :type Actor%20Object%20Reference)))

(event EventTick
  (params (DeltaSeconds :type Float%20%28single-precision%29)))

(fn ConstructionScript)