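; BP_TP is a teleporter actor that moves the player to a destination actor referenced by TPActorLocation.
; On BeginPlay it writes TPText to its TextRender label.
; When a GASPlayerCharacter overlaps the Box, it places the character slightly above the destination without sweeping.
; If no valid destination is set, it prints a Korean warning asking for one.
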(event OnComponentBeginOverlap(Box)
  (params (OverlappedComponent :type Primitive%20Component%20Object%20Reference) (OtherActor :type Actor%20Object%20Reference) (OtherComp :type Primitive%20Component%20Object%20Reference) (OtherBodyIndex :type Integer) (bFromSweep :type Boolean) (SweepResult :type Hit%20Result%20Structure%20%28by%20ref%29))
  (bind _tpactorlocation (Variables|Default|GetTPActorLocation))
  (bind _asgasplayer_character (Utilities|Casting|CastToGASPlayerCharacter OtherActor))
  (Utilities|IsValid _tpactorlocation
    (:Is%20Valid
      (Transformation|SetActorLocation _asgasplayer_character (+ (Transformation|GetActorLocation _tpactorlocation) "0.000000,0.000000,20.000000") false false))
    (:Is%20Not%20Valid
      (Development|PrintString "도착점 액터를 설정해 주세요" true true "(R=1.000000,G=0.033746,B=0.000000,A=1.000000)"))))

(event EventBeginPlay
  (Rendering|Components|TextRender|SetText (Variables|Default|GetTextRender) (Variables|Default|GetTPText)))

(event Collision|EventActorBeginOverlap
  (params (OtherActor :type Actor%20Object%20Reference)))

(event EventTick
  (params (DeltaSeconds :type Float%20%28single-precision%29)))

(fn ConstructionScript)