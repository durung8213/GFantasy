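; Enemy projectile actor for a normal attack that explodes into area damage when it hits something other than a GASCombatNPC.
; On overlap it stops its movement, swaps the flight particles for the impact particle and destroys itself after a short timer.
; A sphere trace around the impact finds targets, and the shooter's ability system component applies the Succubus phase 1 attack GameplayEffect to each hit actor.
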(event OnComponentBeginOverlap(HitCollision)
  (params (OverlappedComponent :type Primitive%20Component%20Object%20Reference) (OtherActor :type Actor%20Object%20Reference) (OtherComp :type Primitive%20Component%20Object%20Reference) (OtherBodyIndex :type Integer) (bFromSweep :type Boolean) (SweepResult :type Hit%20Result%20Structure%20%28by%20ref%29))
  (bind _returnvalue (Transformation|GetActorLocation))
  (bind _shooterasc (Variables|Default|GetShooterASC))
  (bind _shooterasc_2 (Variables|Default|GetShooterASC))
  (if (!= OtherActor self)
    (Utilities|Casting|CastToGASCombatNPC OtherActor
      (:CastFailed
        (Components|Activation|Activate (Variables|Default|GetImpactPartical) false)
        (Variables|/Script/Engine.MovementComponent|SetVelocity (Variables|Default|GetProjectileMovement) "0, 0, 0")
        (Components|Activation|Deactivate (Variables|Default|GetProjectilePartical))
        (Components|Activation|Deactivate (Variables|Default|GetProjectilePartical1))
        (Utilities|Time|SetTimerbyEvent (delegate Custom|DestoryActor) 0.5)
        (bind _outhits (Collision|MultiSphereTraceForObjects _returnvalue _returnvalue 1.5e+02 (Variables|Default|GetObject%20Types) false (Variables|Default|GetActors%20to%20Ignore) "None"))
        (for _array_element _outhits
          (Utilities|IsValid _shooterasc
            (:Is%20Valid
              (GameplayEffects|ApplyGameplayEffectSpecToTarget _shooterasc (GameplayEffects|MakeOutgoingSpec _shooterasc_2 "/Game/Characters/Enemy/EnemySuccubus/GAS/Effect/Attack/GE_SuccubusPhase1Attack1.GE_SuccubusPhase1Attack1_C" 1.0 (GameplayEffects|MakeEffectContext _shooterasc_2)) (Ability|GetAbilitySystemComponent (.HitActor (Collision|BreakHitResult _array_element)))))))))))

(event Custom|DestoryActor
  (Actor|DestroyActor)
  (Development|PrintString "공격 삭제"))

(event EventBeginPlay
  (Components|Activation|Deactivate (Variables|Default|GetImpactPartical)))

(event Collision|EventActorBeginOverlap
  (params (OtherActor :type Actor%20Object%20Reference)))

(event EventTick
  (params (DeltaSeconds :type Float%20%28single-precision%29)))

(fn ConstructionScript)