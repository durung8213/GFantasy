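; BP_SuccubusSlash1 is a slash projectile actor for the Succubus boss that damages the player through the Gameplay Ability System.
; When its Box overlaps a BP_GASPlayerCharacter with a valid ability system component, it applies GE_DummyAttack from the shooter's ASC to the player's.
; It is not destroyed on hit; a timer set at BeginPlay destroys it after a fixed lifetime.
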(event OnComponentBeginOverlap(Box)
  (params (OverlappedComponent :type Primitive%20Component%20Object%20Reference) (OtherActor :type Actor%20Object%20Reference) (OtherComp :type Primitive%20Component%20Object%20Reference) (OtherBodyIndex :type Integer) (bFromSweep :type Boolean) (SweepResult :type Hit%20Result%20Structure%20%28by%20ref%29))
  (bind _asbp_gasplayer_character (Utilities|Casting|CastToBP_GASPlayerCharacter OtherActor))
  (Utilities|IsValid (Ability|GetAbilitySystemComponent _asbp_gasplayer_character)
    (:Is%20Valid
      (Class|GASAbilitySystemLibrary|ApplyGASEffecttoTargettoASC (Variables|Default|GetShooterASC) (Ability|GetAbilitySystemComponent _asbp_gasplayer_character) "/Game/BluePrints/GAS/GameplayEffect/Enemy/Enemy1/GE_DummyAttack.GE_DummyAttack_C" 1.0))))

(event Custom|DestorActor
  (Utilities|Time|ClearandInvalidateTimerbyHandle (Variables|Default|GetDestoryTimer))
  (Actor|DestroyActor))

(event EventBeginPlay
  (bind _returnvalue (Utilities|Time|SetTimerbyEvent (delegate Custom|DestorActor) 6.0))
  (Variables|Default|SetDestoryTimer _returnvalue))

(event Collision|EventActorBeginOverlap
  (params (OtherActor :type Actor%20Object%20Reference)))

(event EventTick
  (params (DeltaSeconds :type Float%20%28single-precision%29)))

(fn ConstructionScript)