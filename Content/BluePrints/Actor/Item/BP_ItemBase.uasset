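; Base world item pickup that shows a rarity-based Niagara effect and adds itself to a player's inventory on touch.
; BeginPlay looks up the ItemTag's definition through player controller 0 and picks the Normal, Epic or Legendary effect for Common, Rair or Epic rarity.
; Box overlap runs on authority only, adding one item, or a fixed bulk amount for Item.Cash, to the overlapping player's InventoryComponent, then destroys the actor.
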(event OnComponentBeginOverlap(BoxCollision)
  (params (OverlappedComponent :type Primitive%20Component%20Object%20Reference) (OtherActor :type Actor%20Object%20Reference) (OtherComp :type Primitive%20Component%20Object%20Reference) (OtherBodyIndex :type Integer) (bFromSweep :type Boolean) (SweepResult :type Hit%20Result%20Structure%20%28by%20ref%29))
  (bind _itemtag (Variables|Default|GetItemTag))
  (Networking|SwitchHasAuthority
    (:Authority
      (bind _asbp_gasplayer_character (Utilities|Casting|CastToBP_GASPlayerCharacter OtherActor))
      (bind _asbp_gasworld_player_controller (Utilities|Casting|CastToBP_GASWorldPlayerController (Pawn|GetController _asbp_gasplayer_character)))
      (if (!= _itemtag "(TagName=\"Item.Cash\")")
        (Class|InventoryComponent|AddItem (Variables|/Script/GFantasy.GASWorldPlayerController|GetInventoryComponent _asbp_gasworld_player_controller) _itemtag 1)
        (Actor|DestroyActor)
        (else
          (Class|InventoryComponent|AddItem (Variables|/Script/GFantasy.GASWorldPlayerController|GetInventoryComponent _asbp_gasworld_player_controller) _itemtag 1000)
          (Actor|DestroyActor))))))

(event EventBeginPlay
  (bind _asbp_gasworld_player_controller (Utilities|Casting|CastToBP_GASWorldPlayerController (Game|GetPlayerController 0)))
  (bind _returnvalue (Class|InventoryInterface|GetInventoryComponent(Message) _asbp_gasworld_player_controller))
  (if (GameplayTags|MatchesTag (Utilities|Struct|BreakMasterItemDefinition (Class|InventoryComponent|GetItemDefinitionbyTag _returnvalue (Variables|Default|GetItemTag))) "(TagName=\"Item.Rarity.Common\")" true)
    (Class|NiagaraComponent|SetAsset (Variables|Default|GetItemSpawnNiagaraComponent) "/Game/Asset/VFX/sA_ItemDropFx/Fx/NS_Normal_System.NS_Normal_System" true)
    (elif (GameplayTags|MatchesTag (Utilities|Struct|BreakMasterItemDefinition (Class|InventoryComponent|GetItemDefinitionbyTag _returnvalue (Variables|Default|GetItemTag))) "(TagName=\"Item.Rarity.Rair\")" true)
      (Class|NiagaraComponent|SetAsset (Variables|Default|GetItemSpawnNiagaraComponent) "/Game/Asset/VFX/sA_ItemDropFx/Fx/NS_Epic_System.NS_Epic_System" true)
      (elif (GameplayTags|MatchesTag (Utilities|Struct|BreakMasterItemDefinition (Class|InventoryComponent|GetItemDefinitionbyTag _returnvalue (Variables|Default|GetItemTag))) "(TagName=\"Item.Rarity.Epic\")" true)
        (Class|NiagaraComponent|SetAsset (Variables|Default|GetItemSpawnNiagaraComponent) "/Game/Asset/VFX/sA_ItemDropFx/Fx/NS_Legendary_System.NS_Legendary_System" true)))))

(fn ConstructionScript)