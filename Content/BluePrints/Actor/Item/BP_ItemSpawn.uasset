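; BP_ItemSpawn is an item drop actor that shows a rarity ribbon effect and becomes an item where it hits.
; On BeginPlay it looks up its ItemTag's rarity through the player controller's inventory component and picks the Niagara ribbon, with Rair using the Epic asset and Epic the Legendary.
; On authority, sphere hits ignore combat NPCs, player characters and rain attack AOEs; any other hit spawns BP_ItemBase with that tag and destroys this actor.
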(event OnComponentHit(SphereComponent)
  (params (HitComponent :type Primitive%20Component%20Object%20Reference) (OtherActor :type Actor%20Object%20Reference) (OtherComp :type Primitive%20Component%20Object%20Reference) (NormalImpulse :type Vector :default "0, 0, 0") (Hit :type Hit%20Result%20Structure%20%28by%20ref%29))
  (bind (_bblockinghit _binitialoverlap _time _distance _location _impactpoint _normal _impactnormal _physmat _hitactor) (Collision|BreakHitResult Hit))
  (Networking|SwitchHasAuthority
    (:Authority
      (Utilities|Casting|CastToGASCombatNPC _hitactor
        (:CastFailed
          (Utilities|Casting|CastToGASPlayerCharacter _hitactor
            (:CastFailed
              (Utilities|Casting|CastToBP_RainAttackAOE _hitactor
                (:CastFailed
                  (Game|SpawnActorfromClass "/Game/BluePrints/Actor/Item/BP_ItemBase.BP_ItemBase_C" (Math|Transform|MakeTransform _location "0, 0, 0" "1.000000,1.000000,1.000000") "Undefined" "MultiplyWithRoot" 0 (Variables|Default|GetItemTag) 0)
                  (Actor|DestroyActor))))))))))

(event EventBeginPlay
  (bind _asbp_gasworld_player_controller (Utilities|Casting|CastToBP_GASWorldPlayerController (Game|GetPlayerController 0)))
  (bind _returnvalue (Class|InventoryInterface|GetInventoryComponent(Message) _asbp_gasworld_player_controller))
  (if (GameplayTags|MatchesTag (Utilities|Struct|BreakMasterItemDefinition (Class|InventoryComponent|GetItemDefinitionbyTag _returnvalue (Variables|Default|GetItemTag))) "(TagName=\"Item.Rarity.Common\")" true)
    (Class|NiagaraComponent|SetAsset (Variables|Default|GetItemSpawnNiagaraComponent) "/Game/Asset/VFX/sA_ItemDropFx/Fx/NS_Normal_Ribbon.NS_Normal_Ribbon" true)
    (elif (GameplayTags|MatchesTag (Utilities|Struct|BreakMasterItemDefinition (Class|InventoryComponent|GetItemDefinitionbyTag _returnvalue (Variables|Default|GetItemTag))) "(TagName=\"Item.Rarity.Rair\")" true)
      (Class|NiagaraComponent|SetAsset (Variables|Default|GetItemSpawnNiagaraComponent) "/Game/Asset/VFX/sA_ItemDropFx/Fx/NS_Epic_Ribbon.NS_Epic_Ribbon" true)
      (elif (GameplayTags|MatchesTag (Utilities|Struct|BreakMasterItemDefinition (Class|InventoryComponent|GetItemDefinitionbyTag _returnvalue (Variables|Default|GetItemTag))) "(TagName=\"Item.Rarity.Epic\")" true)
        (Class|NiagaraComponent|SetAsset (Variables|Default|GetItemSpawnNiagaraComponent) "/Game/Asset/VFX/sA_ItemDropFx/Fx/NS_Legendary_Ribbon.NS_Legendary_Ribbon" true)))))

(fn ConstructionScript)