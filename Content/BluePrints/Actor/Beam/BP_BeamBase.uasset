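; Base beam attack actor that draws a particle beam from a socket on its StartActor to a target.
; Each Tick it updates the endpoints, using the Arm component for BP_BossSuccubus and Mesh otherwise, then repositions the body and explosion effects.
; The end follows either TargetActor or a point swept along BeamSplineActor's spline over Duration.
; On authority, a per-tick capsule trace applies GE_DummyAttack through GAS to hit actors.
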(event EventBeginPlay
  (Effects|Components|ParticleSystem|SetTemplate (Variables|Default|GetBeamBody) (Variables|Default|GetBodyPartical))
  (Effects|Components|ParticleSystem|SetTemplate (Variables|Default|GetBeamExplosion) (Variables|Default|GetExplosionPartical)))

(event Collision|EventActorBeginOverlap
  (params (OtherActor :type Actor%20Object%20Reference)))

(event EventTick
  (params (DeltaSeconds :type Float%20%28single-precision%29))
  (bind _startactor (Variables|Default|GetStartActor))
  (bind _returnvalue (Ability|GetAbilitySystemComponent _startactor))
  (Utilities|FlowControl|Sequence
    (:then_0
      (Variables|Default|SetElapsedTime (+ (Variables|Default|GetElapsedTime) DeltaSeconds)))
    (:then_1
      (bind _asbp_boss_succubus (Utilities|Casting|CastToBP_BossSuccubus (Variables|Default|GetStartActor))
        (:then
          (CallFunction|SuccubusSetStartandEndPoint _asbp_boss_succubus))
        (:CastFailed
          (CallFunction|SetStartandEndPoint))))
    (:then_2
      ;[1 1 1] 빔 이팩트 설정
      (bind _index (Utilities|FlowControl|ForLoopwithBreak 0 10)
        (:LoopBody
          (Class|ParticleSystemComponent|SetBeamSourcePoint (Variables|Default|GetBeamBody) _index (Variables|Default|GetStartLocation))
          (Class|ParticleSystemComponent|SetBeamTargetPoint (Variables|Default|GetBeamBody) _index (Variables|Default|GetEndLocation))
          (Transformation|SetWorldLocation (Variables|Default|GetBeamExplosion) (Variables|Default|GetEndLocation) false false))))
    (:then_3
      (Networking|SwitchHasAuthority
        (:Authority
          (bind _outhits (Class|KismetSystemLibrary|CapsuleTraceMultiforObjects (Variables|Default|GetStartLocation) (Variables|Default|GetEndLocation) (Variables|Default|GetRadius) (Variables|Default|GetHalf%20Height) (Variables|Default|GetObject%20Types) false 0 "ForDuration" true "(R=1.000000,G=0.000000,B=0.000000,A=1.000000)" "(R=0.000000,G=1.000000,B=0.000000,A=1.000000)" DeltaSeconds))
          (for _array_element _outhits
            (Utilities|IsValid _returnvalue
              (:Is%20Valid
                (Utilities|IsValid (Ability|GetAbilitySystemComponent (.HitActor (Collision|BreakHitResult _array_element)))
                  (:Is%20Valid
                    (GameplayEffects|ApplyGameplayEffectSpecToTarget _returnvalue (GameplayEffects|MakeOutgoingSpec _returnvalue "/Game/BluePrints/GAS/GameplayEffect/Enemy/Enemy1/GE_DummyAttack.GE_DummyAttack_C" 1.0 (GameplayEffects|MakeEffectContext _returnvalue)) (Ability|GetAbilitySystemComponent (.HitActor (Collision|BreakHitResult _array_element))))))))))))))

(fn ConstructionScript)

(fn BeamEnd
  (Actor|DestroyActor))

(fn ChangeTargetActor
  (params (TargetActor :type Actor%20Object%20Reference))
  (Variables|Default|SetTargetActor TargetActor))

(fn SetStartandEndPoint
  (bind _startactor (Variables|Default|GetStartActor))
  (bind _beamsplineactor (Variables|Default|GetBeamSplineActor))
  (bind _beamspline (Variables|/Game/BluePrints/Actor/Beam/BP_BeamSplineBase.BP_BeamSplineBase_C|GetBeamSpline _beamsplineactor))
  (Utilities|IsValid _startactor
    (:Is%20Valid
      (Variables|Default|SetStartLocation (+ (Transformation|GetSocketLocation (Variables|/Script/Engine.Character|GetMesh _startactor) (Variables|Default|GetSocketName)) (* (Transformation|GetActorForwardVector _startactor) "20.000000,20.000000,20.000000")))
      (if (Variables|Default|GetbTargetIsActor)
        (Utilities|IsValid (Variables|Default|GetTargetActor) :!label _label
          (:Is%20Valid
            (Variables|Default|SetEndLocation (Transformation|GetActorLocation (Variables|Default|GetTargetActor))))
          (:Is%20Not%20Valid
            (Development|PrintString "빔의 타겟을 액터로 하였으나 타겟 액터가 설정되어 있지 않음 " true true "(R=1.000000,G=0.000000,B=0.022914,A=1.000000)")))
        (else
          (Utilities|IsValid (Variables|Default|GetBeamSplineActor)
            (:Is%20Valid
              (Variables|Default|SetEndLocation (Spline|GetLocationatDistanceAlongSpline _beamspline (* (Spline|GetSplineLength _beamspline) (Math|Float|Clamp(Float) (/ (Variables|Default|GetElapsedTime) (Variables|Default|GetDuration)))) "World")))
            (:Is%20Not%20Valid
              (Development|PrintString "빔의 타겟을 스플라인으로 하였으나 타겟 액터가 설정되어 있지 않음 " true true "(R=1.000000,G=0.000000,B=0.022914,A=1.000000)"))))))
    (:Is%20Not%20Valid
      (goto _label))))

(fn SuccubusSetStartandEndPoint
  (params (NewParam :type BP%20Boss%20Succubus%20Object%20Reference))
  (bind _beamsplineactor (Variables|Default|GetBeamSplineActor))
  (bind _beamspline (Variables|/Game/BluePrints/Actor/Beam/BP_BeamSplineBase.BP_BeamSplineBase_C|GetBeamSpline _beamsplineactor))
  (Utilities|IsValid NewParam
    (:Is%20Valid
      (Variables|Default|SetStartLocation (+ (Transformation|GetSocketLocation (Variables|/Game/Characters/Enemy/EnemySuccubus/BP_BossSuccubus.BP_BossSuccubus_C|GetArm NewParam) (Variables|Default|GetSocketName)) (* (Transformation|GetActorForwardVector (Variables|Default|GetStartActor)) "20.000000,20.000000,20.000000")))
      (if (Variables|Default|GetbTargetIsActor)
        (Utilities|IsValid (Variables|Default|GetTargetActor) :!label _label
          (:Is%20Valid
            (Variables|Default|SetEndLocation (Transformation|GetActorLocation (Variables|Default|GetTargetActor))))
          (:Is%20Not%20Valid
            (Development|PrintString "빔의 타겟을 액터로 하였으나 타겟 액터가 설정되어 있지 않음 " true true "(R=1.000000,G=0.000000,B=0.022914,A=1.000000)")))
        (else
          (Utilities|IsValid (Variables|Default|GetBeamSplineActor)
            (:Is%20Valid
              (Variables|Default|SetEndLocation (Spline|GetLocationatDistanceAlongSpline _beamspline (* (Spline|GetSplineLength _beamspline) (Math|Float|Clamp(Float) (/ (Variables|Default|GetElapsedTime) (Variables|Default|GetDuration)))) "World")))
            (:Is%20Not%20Valid
              (Development|PrintString "빔의 타겟을 스플라인으로 하였으나 타겟 액터가 설정되어 있지 않음 " true true "(R=1.000000,G=0.000000,B=0.022914,A=1.000000)"))))))
    (:Is%20Not%20Valid
      (goto _label))))