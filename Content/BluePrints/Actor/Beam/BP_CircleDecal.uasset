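; BP_CircleDecal is an actor that shows a colored circle on a surface using two decals, a circumference and an area.
; BeginPlay creates dynamic materials for both, using one scalar to select ring or fill, then applies color and radius.
; A timeline animates the area's fill value.
; Color changes replicate through a server event and OnRep, with a multicast event that also applies color directly.
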(event Custom|MultiSetDecalColor
  (params (Value :type Linear%20Color%20Structure))
  (CallFunction|SetDecalColor Value))

(event Custom|ServerSetDecalColor
  (params (Value :type Linear%20Color%20Structure))
  (Variables|Default|SetColor Value))

(event EventBeginPlay
  (Utilities|FlowControl|Sequence
    (:then_0
      (bind _returnvalue (Rendering|Material|CreateDynamicMaterialInstance (Variables|Default|GetCircum) :!class /Script/Engine.DecalComponent))
      (bind _output_get (Variables|Default|SetCircumRef _returnvalue))
      (Rendering|Material|SetScalarParameterValue _output_get "Circum1Area0" 1.0 :!class /Script/Engine.MaterialInstanceDynamic))
    (:then_1
      (bind _returnvalue_2 (Rendering|Material|CreateDynamicMaterialInstance (Variables|Default|GetArea) :!class /Script/Engine.DecalComponent))
      (bind _output_get_2 (Variables|Default|SetAreaRef _returnvalue_2))
      (Rendering|Material|SetScalarParameterValue _output_get_2 "Circum1Area0" 0.0 :!class /Script/Engine.MaterialInstanceDynamic))
    (:then_2
      (CallFunction|SetDecalColor (Variables|Default|GetColor)))
    (:then_3
      (CallFunction|SetDecalRadius (Variables|Default|GetRadius)))
    (:then_4
      (bind _areavaluealpha (Timeline|AreaValueTimeline Play)
        (:Update
          (Utilities|IsValid (Variables|Default|GetAreaRef)
            (:Is%20Valid
              (Rendering|Material|SetScalarParameterValue (Variables|Default|GetAreaRef) "AreaValue" _areavaluealpha :!class /Script/Engine.MaterialInstanceDynamic))))))))

(fn ConstructionScript)

(fn OnRepValue0)

(fn SetDecalColor
  (params (Value :type Linear%20Color%20Structure))
  (bind _circumref (Variables|Default|GetCircumRef))
  (if (and (Utilities|IsValid _circumref) (Utilities|IsValid (Variables|Default|GetAreaRef)))
    (Rendering|Material|SetVectorParameterValue _circumref "DecalColor" Value :!class /Script/Engine.MaterialInstanceDynamic)))

(fn SetDecalRadius
  (params (Value :type Float%20%28single-precision%29))
  (Rendering|Material|SetScalarParameterValue (Variables|Default|GetCircumRef) "RadianValue" Value :!class /Script/Engine.MaterialInstanceDynamic))

(fn OnRepColor
  (CallFunction|SetDecalColor (Variables|Default|GetColor)))