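; BP_RidingHorse is a rideable horse character that adjusts its speed and turn state from how sharply it changes direction.
; Each Tick compares the forward vector with the velocity direction while moving; at 30 degrees or more it lowers MaxWalkSpeed, otherwise it restores the faster speed.
; The sign of the cross product's Z picks RotateR or RotateL, flags that reset every frame.
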(event EventBeginPlay)

(event Collision|EventActorBeginOverlap
  (params (OtherActor :type Actor%20Object%20Reference)))

(event EventTick
  (params (DeltaSeconds :type Float%20%28single-precision%29))
  (bind _self self)
  (bind _returnvalue (Transformation|GetVelocity _self))
  (Utilities|IsValid _self
    (:Is%20Valid
      (Variables|Default|SetbRotateR false)
      (Variables|Default|SetbRotateL false)
      (Variables|Default|SetActorLocation (Transformation|GetActorLocation _self))
      (Variables|Default|SetForwardVector (Transformation|GetActorForwardVector _self))
      (Variables|Default|SetVelocityDir (Math|Vector|Normalize _returnvalue))
      (if (not (Math|Vector|VectorIsNearlyZero _returnvalue))
        (if (>= (Math|Trig|RadiansToDegrees (Math|Trig|Acos(Degrees) (Math|Float|Clamp(Float) (Math|Vector|DotProduct (Variables|Default|GetForwardVector) (Variables|Default|GetVelocityDir)) -1.0))) 3e+01)
          (if (> (.z (Math|Vector|CrossProduct (Variables|Default|GetForwardVector) (Variables|Default|GetVelocityDir))) 0.0)
            (Variables|Default|SetbRotateR true)
            (else
              (Variables|Default|SetbRotateL true)))
          (Variables|/Script/Engine.CharacterMovementComponent|SetMaxWalkSpeed (Variables|Character|GetCharacterMovement) 7e+02)
          (else
            (Variables|/Script/Engine.CharacterMovementComponent|SetMaxWalkSpeed (Variables|Character|GetCharacterMovement) 1.2e+03)))))))

(fn ConstructionScript)