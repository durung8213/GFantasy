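; Construction-script tool that builds a straight fence along local X, sized by the length of its InterSpline rather than following the curve.
; It derives the piece count from spline length and mesh bounds, spaces pieces by Calculator, and scales the last to fill the remainder.
; Chained chance rolls pick each other piece's variant, re-rolling on every reconstruction, though all four variants are currently set to the same mesh.
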(event EventBeginPlay)

(event Collision|EventActorBeginOverlap
  (params (OtherActor :type Actor%20Object%20Reference)))

(event EventTick
  (params (DeltaSeconds :type Float%20%28single-precision%29)))

(fn ConstructionScript
  (bind _interspline (Variables|Default|GetInterSpline))
  (bind _returnvalue (Spline|GetSplineLength _interspline))
  (Variables|Default|SetFence_01 "/Game/MapAsset/NativeAmericanVillage/StaticMesh/Building_Kit/WoodenFences/SM_Fence_02a.SM_Fence_02a")
  (Variables|Default|SetFence_02 "/Game/MapAsset/NativeAmericanVillage/StaticMesh/Building_Kit/WoodenFences/SM_Fence_02a.SM_Fence_02a")
  (Variables|Default|SetFence%2003 "/Game/MapAsset/NativeAmericanVillage/StaticMesh/Building_Kit/WoodenFences/SM_Fence_02a.SM_Fence_02a")
  (Variables|Default|SetFence%2004 "/Game/MapAsset/NativeAmericanVillage/StaticMesh/Building_Kit/WoodenFences/SM_Fence_02a.SM_Fence_02a")
  (Variables|Default|SetCalculator (Variables|Default|GetCalculator))
  (bind _output_get (Variables|Default|Setlength (.x (+ (Math|Vector|VectorGetAbs (.min (StaticMesh|GetBoundingBox (Variables|Default|GetFence_02)))) (Math|Vector|VectorGetAbs (.max (StaticMesh|GetBoundingBox (Variables|Default|GetFence_02))))))))
  (bind _returnvalue_2 (AddComponent|AddStaticMeshComponent false (Math|Transform|MakeTransform (Math|Vector|MakeVector (Math|Conversions|ToFloat(Integer) (* (- (Math|Float|Floor (/ (+ _returnvalue (/ (Variables|Default|GetCalculator) 2.0)) (+ _output_get 0.0))) 1) (Variables|Default|GetCalculator))) 0.0 0.0) "0, 0, 0" (Math|Vector|MakeVector (/ (- _returnvalue (* (- (Math|Float|Floor (/ (+ _returnvalue (/ (Variables|Default|GetCalculator) 2.0)) (+ _output_get 0.0))) 1) (Variables|Default|GetCalculator))) (Variables|Default|GetCalculator)) 1.0 1.0))))
  (Components|StaticMesh|SetStaticMesh _returnvalue_2 (Variables|Default|GetFence_02))
  (for _index (range 0 (- (Math|Float|Floor (/ (+ _returnvalue (/ (Variables|Default|GetCalculator) 2.0)) (+ _output_get 0.0))) 2))
    (bind _returnvalue_3 (AddComponent|AddStaticMeshComponent false (Math|Transform|MakeTransform (Math|Vector|MakeVector (Math|Conversions|ToFloat(Integer) (* _index (Variables|Default|GetCalculator))) 0.0 0.0) "0, 0, 0" (Math|Vector|MakeVector 1.0 1.0 1.0))))
    (if (<= (Math|Random|RandomInteger 100) (Variables|Default|GetVariation_01%20Spawn%20Chance))
      (Components|StaticMesh|SetStaticMesh _returnvalue_3 (Variables|Default|GetFence_01))
      (elif (<= (Math|Random|RandomInteger 100) (Variables|Default|GetVariation_02%20Spawn%20Chance))
        (Components|StaticMesh|SetStaticMesh _returnvalue_3 (Variables|Default|GetFence%2003))
        (elif (<= (Math|Random|RandomInteger 100) (Variables|Default|GetVariation_03%20Spawn%20Chance))
          (Components|StaticMesh|SetStaticMesh _returnvalue_3 (Variables|Default|GetFence%2004))
          (else
            (Components|StaticMesh|SetStaticMesh _returnvalue_3 (Variables|Default|GetFence_02))))))))